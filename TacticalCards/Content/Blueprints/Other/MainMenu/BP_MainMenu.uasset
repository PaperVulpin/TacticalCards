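; Main menu actor that creates the menu widget on BeginPlay and cycles streamed levels behind it.
; An endless latent loop alternates L_Hexagon_01 and L_Hexagon_02, using non-blocking loads and unloading each before the next loads.
; The widget's show and hide background events run on fixed delays between each load and unload.
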(event EventBeginPlay
  (bind _returnvalue (UserInterface|CreateWidget "/Game/Blueprints/Other/MainMenu/W_MainMenu.W_MainMenu_C"))
  (bind _output_get (Variables|Default|SetW_MainMenu _returnvalue))
  (UserInterface|Viewport|AddtoViewport _output_get 0)
  (Game|LoadStreamLevel(byName) "L_Hexagon_01" true :!label _label)
  (Default|EventShowBackground (Variables|Default|GetW_MainMenu))
  (Utilities|FlowControl|Delay 5.0)
  (Default|EventHideBackground (Variables|Default|GetW_MainMenu))
  (Utilities|FlowControl|Delay 5.0)
  (Game|UnloadStreamLevel(byName) "L_Hexagon_01" false)
  (Game|LoadStreamLevel(byName) "L_Hexagon_02" true)
  (Default|EventShowBackground (Variables|Default|GetW_MainMenu))
  (Utilities|FlowControl|Delay 5.0)
  (Default|EventHideBackground (Variables|Default|GetW_MainMenu))
  (Utilities|FlowControl|Delay 5.0)
  (Game|UnloadStreamLevel(byName) "L_Hexagon_02" false)
  (goto _label))

(event Collision|EventActorBeginOverlap
  (params (OtherActor :type Actor%20Object%20Reference)))

(event EventTick
  (params (DeltaSeconds :type Float%20%28single-precision%29)))

(fn ConstructionScript)