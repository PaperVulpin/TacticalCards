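; Overworld scenario actor that sets up the level's units as groups, some flagged as encounters.
; BuildUnitGroupsBasedOnUnitsNames fills the UnitGroups map from all BP_Unit actors, parsing group ID and encounter flag ("_AI") from display names.
; On BeginPlay, it sets each mapped unit's context and registers units and encounter flags with OverworldUnitGroupManager.
; A short startup delay works around CharacterMovement not being initialized on the first frame.
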(event EventBeginPlay
  (Utilities|FlowControl|Delay 0.01) ; Delay is a workaround as CharacterMovement does not seem to be initialized on first frame.
  (bind _values (Utilities|Map|Values (Variables|Default|GetUnitGroups)))
  (for _array_element _values
    (for _array_element_2 (.Units (Utilities|Struct|BreakS_OverworldUnitGroup _array_element))
      (Default|SetUnitContext _array_element_2 "NewEnumerator1")
      (Default|AddUnittoGroup (Variables|Default|GetOverworldUnitGroupManager) _array_element_2 (.GroupID (Utilities|Struct|BreakS_OverworldUnitGroup _array_element))))
    (Default|SetGroupIsEncounter (Variables|Default|GetOverworldUnitGroupManager) (.IsEncounter (Utilities|Struct|BreakS_OverworldUnitGroup _array_element)) (.GroupID (Utilities|Struct|BreakS_OverworldUnitGroup _array_element)))))

(event Collision|EventActorBeginOverlap
  (params (OtherActor :type Actor%20Object%20Reference)))

(event EventTick
  (params (DeltaSeconds :type Float%20%28single-precision%29)))

(fn ConstructionScript)

(fn BuildUnitGroupsBasedonUnitsNames
  (Utilities|Map|Clear (Variables|Default|GetUnitGroups))
  (bind _outactors (Actor|GetAllActorsOfClass "/Game/Blueprints/Core/Units/BP_Unit.BP_Unit_C"))
  (for _array_element _outactors
    (bind _output_get (LocalVariables|SetUnit _array_element))
    (LocalVariables|SetGroupID (Math|Conversions|ToInteger(Byte) (.LeftS (Utilities|String|Split (.RightS (Utilities|String|Split (Utilities|GetDisplayName _output_get) "Group")) "_"))))
    (LocalVariables|SetIsEncounter (Utilities|String|Contains (Utilities|GetDisplayName (LocalVariables|GetUnit)) "_AI"))
    (bind _output_get_2 (LocalVariables|SetGroup (.Value (Utilities|Map|Find (Variables|Default|GetUnitGroups) (LocalVariables|GetGroupID)))))
    (Utilities|Struct|SetmembersinS_OverworldUnitGroup _output_get_2 (LocalVariables|GetGroupID) (LocalVariables|GetIsEncounter))
    (Utilities|Array|AddUnique (Utilities|Struct|BreakS_OverworldUnitGroup (LocalVariables|GetGroup)) (LocalVariables|GetUnit))
    (Utilities|Map|Add (Variables|Default|GetUnitGroups) (LocalVariables|GetGroupID) (LocalVariables|GetGroup))))