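; BP_PlayerActions is the player's input controller for grid-based turn combat, handling tile and unit hover, selection and mouse actions.
; Tick traces the cursor to update the hovered tile and unit, feeding action actors spawned per mouse button, which repeat while held on hover change.
; Grid and CombatSystem events update selection, swap move or cast-ability actions, and manage the combat and end-screen widgets.
; Number keys select abilities during combat.
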(event Custom|OnHoveredTileChanged
  (bind _hoveredtile (Variables|Default|GetHoveredTile))
  (bind _selectedaction_rightclick (Variables|Actions|GetSelectedAction_RightClick))
  (bind _selectedaction_leftclick (Variables|Actions|GetSelectedAction_LeftClick))
  (Utilities|FlowControl|Sequence
    (:then_0
      (Utilities|IsValid _selectedaction_leftclick
        (:Is%20Valid
          (Default|ExecuteHoveredAction _selectedaction_leftclick (Variables|Default|GetHoveredTile))
          (if (Variables|Actions|GetIsLeftClickDown)
            (Default|ExecuteAction (Variables|Actions|GetSelectedAction_LeftClick) _hoveredtile)))))
    (:then_1
      (Utilities|IsValid _selectedaction_rightclick
        (:Is%20Valid
          (Default|ExecuteHoveredAction _selectedaction_rightclick (Variables|Default|GetHoveredTile))
          (if (Variables|Actions|GetIsRightClickDown)
            (Default|ExecuteAction (Variables|Actions|GetSelectedAction_RightClick) _hoveredtile)))))))

(event EventBeginPlay
  (bind _returnvalue (Actor|GetActorOfClass "/Game/Blueprints/Core/Grid/BP_Grid.BP_Grid_C"))
  (Variables|Components|SetGrid _returnvalue)
  (EventDispatchers|BindEventtoOnGridGenerated (Variables|Components|GetGrid) (EventDispatchers|CreateEvent :!event OnGridGenerated))
  (EventDispatchers|BindEventtoOnTileDataUpdated (Variables|Components|GetGrid) (EventDispatchers|CreateEvent :!event OnTileDataUpdated))
  (bind _returnvalue_2 (Actor|GetActorOfClass "/Game/Blueprints/Core/Combat/BP_CombatSystem.BP_CombatSystem_C"))
  (bind _output_get (Variables|Components|SetCombatSystem _returnvalue_2))
  (EventDispatchers|BindEventtoOnUnitGridIndexChanged _output_get (EventDispatchers|CreateEvent :!event OnUnitGridIndexChanged))
  (EventDispatchers|BindEventtoOnCombatStarted _output_get (EventDispatchers|CreateEvent :!event OnCombatStarted))
  (EventDispatchers|BindEventtoOnCombatEnded _output_get (EventDispatchers|CreateEvent :!event OnCombatEnded))
  (EventDispatchers|BindEventtoOnUnitTurnStarted _output_get (EventDispatchers|CreateEvent :!event OnUnitTurnStarted))
  (EventDispatchers|BindEventtoOnUnitTurnEnded _output_get (EventDispatchers|CreateEvent :!event OnUnitTurnEnded))
  (EventDispatchers|BindEventtoOnCombatFinishing _output_get (EventDispatchers|CreateEvent :!event OnCombatFinishing))
  (Input|EnableInput (Game|GetPlayerController 0)))

(event EventTick
  (params (DeltaSeconds :type Float%20%28single-precision%29))
  (CallFunction|UpdateHoveredTileandUnit))

(event Input|MouseEvents|LeftMouseButton
  (params (Key :type Key%20Structure :default "None"))
  (bind _selectedaction_leftclick (Variables|Actions|GetSelectedAction_LeftClick))
  (:Pressed
    (CallFunction|UpdateHoveredTileandUnit)
    (Variables|Actions|SetIsLeftClickDown true)
    (Utilities|IsValid _selectedaction_leftclick
      (:Is%20Valid
        (Default|ExecuteAction _selectedaction_leftclick (Variables|Default|GetHoveredTile)))))
  (:Released
    (Variables|Actions|SetIsLeftClickDown false)))

(event Input|MouseEvents|RightMouseButton
  (params (Key :type Key%20Structure :default "None"))
  (bind _selectedaction_rightclick (Variables|Actions|GetSelectedAction_RightClick))
  (:Pressed
    (CallFunction|UpdateHoveredTileandUnit)
    (Variables|Actions|SetIsRightClickDown true)
    (Utilities|IsValid _selectedaction_rightclick
      (:Is%20Valid
        (Default|ExecuteAction _selectedaction_rightclick (Variables|Default|GetHoveredTile)))))
  (:Released
    (Variables|Actions|SetIsRightClickDown false)))

(event Input|KeyboardEvents|AnyKey
  (params (Key :type Key%20Structure :default "None"))
  (bind _returnvalue (Class|KismetInputLibrary|KeyGetDisplayName Key true))
  (bind _combatsystem (Variables|Components|GetCombatSystem))
  (bind _returnvalue_2 (Utilities|String|ToString(Text) _returnvalue))
  (:Pressed
    (if (and (Variables|/Game/Blueprints/Core/Combat/BP_CombatSystem.BP_CombatSystem_C|GetIsInCombat _combatsystem) (not (Variables|/Game/Blueprints/Core/Combat/BP_CombatSystem.BP_CombatSystem_C|GetIsFinishingCombat _combatsystem)))
      (if (Class|KismetStringLibrary|IsNumeric _returnvalue_2)
        (Default|SetSelectedAbilityfromIndex (Variables|/Game/Blueprints/Core/Combat/Widgets/W_Combat.W_Combat_C|GetButtonList_Abilities (Variables|Default|GetW_Combat)) (Math|Conversions|ToInteger(Byte) _returnvalue_2))))))

(fn ConstructionScript)

(fn UpdateHoveredTileandUnit
  (bind _grid (Variables|Components|GetGrid))
  (Utilities|FlowControl|Sequence
    (:then_0
      (bind _unit (CallFunction|GetUnitUnderCursor))
      (if (!= _unit (Variables|Default|GetHoveredUnit))
        (Utilities|FlowControl|Sequence
          (:then_0
            (Utilities|IsValid (Variables|Default|GetHoveredUnit)
              (:Is%20Valid
                (Default|SetIsHovered (Variables|Default|GetHoveredUnit) false))))
          (:then_1
            (Variables|Default|SetHoveredUnit _unit)
            (Utilities|IsValid _unit
              (:Is%20Valid
                (Default|SetIsHovered _unit true)))))))
    (:then_1
      (Utilities|IsValid (Variables|Default|GetHoveredUnit)
        (:Is%20Valid
          (LocalVariables|SetNewIndex (Variables|/Game/Blueprints/Core/Units/BP_Unit.BP_Unit_C|GetIndex (Variables|Default|GetHoveredUnit))))
        (:Is%20Not%20Valid
          (bind _index (Default|GetTileIndexUnderCursor _grid))
          (bind _output_get (LocalVariables|SetNewIndex _index))))
      (if (!= _output_get (Variables|Default|GetHoveredTile))
        (Default|RemoveStatefromTile _grid (Variables|Default|GetHoveredTile) "NewEnumerator1")
        (bind _output_get_2 (Variables|Default|SetHoveredTile _output_get))
        (Default|AddStatetoTile _grid _output_get_2 "NewEnumerator1")
        (CallFunction|OnHoveredTileChanged)))))

(fn SetSelectedActions
  (params (LeftAction :type BP%20Action%20Class%20Reference) (RightAction :type BP%20Action%20Class%20Reference))
  (Utilities|FlowControl|Sequence
    (:then_0
      (Utilities|IsValid (Variables|Actions|GetSelectedAction_LeftClick)
        (:Is%20Valid
          (Actor|DestroyActor (Variables|Actions|GetSelectedAction_LeftClick))
          (Variables|Actions|SetSelectedAction_LeftClick 0))
        (:Is%20Not%20Valid
          _))
      (if (Utilities|IsValidClass LeftAction)
        (bind _returnvalue (Game|SpawnActorfromClass LeftAction (Math|Transform|MakeTransform "0, 0, 0" "0, 0, 0" "1.000000,1.000000,1.000000") "AlwaysSpawn" "MultiplyWithRoot" 0 self 0))
        (Variables|Actions|SetSelectedAction_LeftClick _returnvalue)))
    (:then_1
      (Utilities|IsValid (Variables|Actions|GetSelectedAction_RightClick)
        (:Is%20Valid
          (Actor|DestroyActor (Variables|Actions|GetSelectedAction_RightClick))
          (Variables|Actions|SetSelectedAction_RightClick 0))
        (:Is%20Not%20Valid
          _))
      (if (Utilities|IsValidClass RightAction)
        (bind _returnvalue_2 (Game|SpawnActorfromClass RightAction (Math|Transform|MakeTransform "0, 0, 0" "0, 0, 0" "1.000000,1.000000,1.000000") "AlwaysSpawn" "MultiplyWithRoot" 0 self 0))
        (Variables|Actions|SetSelectedAction_RightClick _returnvalue_2)))
    (:then_2
      (Default|CallOnSelectedActionsChanged (Variables|Actions|GetSelectedAction_LeftClick) (Variables|Actions|GetSelectedAction_RightClick)))))

(fn GetUnitUnderCursor
  (params (PlayerIndex :type Integer))
  (bind _returnvalue (Game|GetPlayerController PlayerIndex))
  (bind (_hitresult _returnvalue_2) (Game|Player|GetHitResultUnderCursorbyChannel _returnvalue "TraceTypeQuery5" false))
  (if _returnvalue_2
    (return (.AsBP%20Unit (Utilities|Casting|CastToBP_Unit (.HitActor (Collision|BreakHitResult _hitresult)))))
    (else
      (bind _index (Default|GetTileIndexUnderCursor (Variables|Components|GetGrid) PlayerIndex))
      (return (Utilities|Struct|BreakS_TileData (.Value (Utilities|Map|Find (Variables|/Game/Blueprints/Core/Grid/BP_Grid.BP_Grid_C|GetGridTiles (Variables|Components|GetGrid)) _index)))))))

(fn SetSelectedTileandUnit
  (params (Index :type Int%20Point%20Structure) (Force :type Boolean))
  (bind _grid (Variables|Components|GetGrid))
  (Utilities|FlowControl|Sequence
    (:then_0
      (if (or (!= Index (Variables|Default|GetSelectedTile)) Force) ; Different Tile?
        (Default|RemoveStatefromTile _grid (Variables|Default|GetSelectedTile) "NewEnumerator2")
        (bind _output_get (Variables|Default|SetSelectedTile Index))
        (Default|AddStatetoTile _grid _output_get "NewEnumerator2")
        (else
          (Default|RemoveStatefromTile _grid (Variables|Default|GetSelectedTile) "NewEnumerator2")
          (Variables|Default|SetSelectedTile (Utilities|Struct|MakeIntPoint -999 -999))))
      (Default|CallOnSelectedTileChanged (Variables|Default|GetSelectedTile)))
    (:then_1
      (LocalVariables|SetNewUnit (Utilities|Struct|BreakS_TileData (.Value (Utilities|Map|Find (Variables|/Game/Blueprints/Core/Grid/BP_Grid.BP_Grid_C|GetGridTiles (Variables|Components|GetGrid)) (Variables|Default|GetSelectedTile)))))
      (if (or Force (!= (Variables|Default|GetSelectedUnit) (LocalVariables|GetNewUnit)))
        (Utilities|FlowControl|Sequence
          (:then_0
            (Utilities|IsValid (Variables|Default|GetSelectedUnit)
              (:Is%20Valid
                (Default|SetIsSelected (Variables|Default|GetSelectedUnit) false))))
          (:then_1
            (bind _output_get_2 (Variables|Default|SetSelectedUnit (LocalVariables|GetNewUnit)))
            (Utilities|IsValid _output_get_2
              (:Is%20Valid
                (Default|SetIsSelected _output_get_2 true)))))))))

(fn OnGridGenerated
  (if (Default|IsIndexValid (Variables|Components|GetGrid) (Variables|Default|GetSelectedTile))
    (CallFunction|SetSelectedTileandUnit (Variables|Default|GetSelectedTile) true)
    (else
      (CallFunction|SetSelectedTileandUnit (Utilities|Struct|MakeIntPoint -999 -999) false))))

(fn OnTileDataUpdated
  (params (Index :type Int%20Point%20Structure))
  (if (Class|KismetMathLibrary|EqualIntPointIntPoint Index (Variables|Default|GetSelectedTile))
    (CallFunction|OnGridGenerated)))

(fn OnUnitGridIndexChanged
  (params (Unit :type BP%20Unit%20Object%20Reference))
  (if (== Unit (Variables|Default|GetSelectedUnit))
    (CallFunction|SetSelectedTileandUnit (Variables|/Game/Blueprints/Core/Units/BP_Unit.BP_Unit_C|GetIndex Unit) false)))

(fn OnCombatStarted
  (CallFunction|SetSelectedActions)
  (CallFunction|SetSelectedTileandUnit (Utilities|Struct|MakeIntPoint -999 -999) false)
  (bind _returnvalue (UserInterface|CreateWidget "/Game/Blueprints/Core/Combat/Widgets/W_Combat.W_Combat_C" 0 self))
  (bind _output_get (Variables|Default|SetW_Combat _returnvalue))
  (UserInterface|Viewport|AddtoPlayerScreen _output_get)
  (EventDispatchers|BindEventtoOnSelectedAbilityButtonChanged (Variables|/Game/Blueprints/Core/Combat/Widgets/W_Combat.W_Combat_C|GetButtonList_Abilities (Variables|Default|GetW_Combat)) (EventDispatchers|CreateEvent :!event OnSelectedAbilityChanged)))

(fn OnCombatEnded
  (Widget|RemovefromParent (Variables|Default|GetW_CombatEndScreen))
  (Variables|Default|SetW_CombatEndScreen 0))

(fn OnUnitTurnStarted
  (params (Unit :type BP%20Unit%20Object%20Reference))
  (CallFunction|SetSelectedTileandUnit (Variables|/Game/Blueprints/Core/Units/BP_Unit.BP_Unit_C|GetIndex Unit) false)
  (CallFunction|SetSelectedActions "/Game/Blueprints/Core/Player/Actions/Combat/Action_Combat_Move.Action_Combat_Move_C")
  (Default|LinkUnittoAbilitiesList (Variables|/Game/Blueprints/Core/Combat/Widgets/W_Combat.W_Combat_C|GetButtonList_Abilities (Variables|Default|GetW_Combat)) (Variables|Default|GetSelectedUnit)))

(fn OnUnitTurnEnded
  (params (Unit :type BP%20Unit%20Object%20Reference))
  (CallFunction|SetSelectedTileandUnit (Utilities|Struct|MakeIntPoint -999 -999) false)
  (CallFunction|SetSelectedActions)
  (Default|LinkUnittoAbilitiesList (Variables|/Game/Blueprints/Core/Combat/Widgets/W_Combat.W_Combat_C|GetButtonList_Abilities (Variables|Default|GetW_Combat))))

(fn OnSelectedAbilityChanged
  (params (Button :type Button%20Ability%20Object%20Reference))
  (Utilities|IsValid Button
    (:Is%20Valid
      (CallFunction|SetSelectedActions "/Game/Blueprints/Core/Player/Actions/Combat/Action_Combat_CastAbility.Action_Combat_CastAbility_C") ; Set mouse action to cast
      (bind _asaction_combat_cast_ability (Utilities|Casting|CastToAction_Combat_CastAbility (Variables|Actions|GetSelectedAction_LeftClick)))
      (Default|SetAbility _asaction_combat_cast_ability (Variables|/Game/Blueprints/Core/Combat/Abilities/Widgets/Button_Ability.Button_Ability_C|GetAbility Button)))
    (:Is%20Not%20Valid
      (if (!= (Utilities|GetClass (Variables|Actions|GetSelectedAction_LeftClick)) "/Game/Blueprints/Core/Player/Actions/Combat/Action_Combat_Move.Action_Combat_Move_C")
        (CallFunction|SetSelectedActions "/Game/Blueprints/Core/Player/Actions/Combat/Action_Combat_Move.Action_Combat_Move_C") ; Set mouse action to move
      ))))

(fn OnCombatFinishing
  (params (WinningTeamIndex :type Integer))
  (CallFunction|SetSelectedActions)
  (CallFunction|SetSelectedTileandUnit (Utilities|Struct|MakeIntPoint -999 -999) false)
  (Widget|RemovefromParent (Variables|Default|GetW_Combat))
  (Variables|Default|SetW_Combat 0)
  (bind _returnvalue (UserInterface|CreateWidget "/Game/Blueprints/Core/Combat/Widgets/W_CombatEndScreen.W_CombatEndScreen_C" 0 self WinningTeamIndex))
  (bind _output_get (Variables|Default|SetW_CombatEndScreen _returnvalue))
  (UserInterface|Viewport|AddtoPlayerScreen _output_get))