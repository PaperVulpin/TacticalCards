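; Player pawn that acts as a movable camera with pan, zoom and stepped yaw rotation.
; BeginPlay adds the IMC_Player Enhanced Input context and seeds desired location, rotation and zoom from the current state.
; Input events only change those targets: panning follows the actor's axes, zoom is clamped, and rotation steps on action completion.
; Tick smoothly interpolates the actor transform and spring arm length toward the targets.
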(event Input|EnhancedActionEvents|EnhancedInputActionIA_ZoomCamera
  (params (ActionValue :type Float%20%28double-precision%29) (ElapsedSeconds :type Float%20%28double-precision%29) (TriggeredSeconds :type Float%20%28double-precision%29) (InputAction :type Input%20Action%20Object%20Reference :default "/Game/Blueprints/Core/Player/IA_ZoomCamera.IA_ZoomCamera"))
  (:Triggered
    (Variables|Default|SetZoom_Desired (Math|Float|Clamp(Float) (+ (* ActionValue (Variables|Default|GetZoomSpeed)) (Variables|Default|GetZoom_Desired)) (Variables|Default|GetZoomMin) (Variables|Default|GetZoomMax)))))

(event Input|EnhancedActionEvents|EnhancedInputActionIA_MoveCameraRight
  (params (ActionValue :type Float%20%28double-precision%29) (ElapsedSeconds :type Float%20%28double-precision%29) (TriggeredSeconds :type Float%20%28double-precision%29) (InputAction :type Input%20Action%20Object%20Reference :default "/Game/Blueprints/Core/Player/IA_MoveCameraRight.IA_MoveCameraRight"))
  (:Triggered
    (Variables|Default|SetLocation_Desired (+ (Variables|Default|GetLocation_Desired) (* (* ActionValue (Variables|Default|GetLocationSpeed)) (Transformation|GetActorRightVector))))))

(event Input|EnhancedActionEvents|EnhancedInputActionIA_MoveCameraForward
  (params (ActionValue :type Float%20%28double-precision%29) (ElapsedSeconds :type Float%20%28double-precision%29) (TriggeredSeconds :type Float%20%28double-precision%29) (InputAction :type Input%20Action%20Object%20Reference :default "/Game/Blueprints/Core/Player/IA_MoveCameraForward.IA_MoveCameraForward"))
  (:Triggered
    (Variables|Default|SetLocation_Desired (+ (Variables|Default|GetLocation_Desired) (* (* ActionValue (Variables|Default|GetLocationSpeed)) (Transformation|GetActorForwardVector))))))

(event Input|EnhancedActionEvents|EnhancedInputActionIA_RotateCameraRight
  (params (ActionValue :type Boolean) (ElapsedSeconds :type Float%20%28double-precision%29) (TriggeredSeconds :type Float%20%28double-precision%29) (InputAction :type Input%20Action%20Object%20Reference :default "/Game/Blueprints/Core/Player/IA_RotateCameraRight.IA_RotateCameraRight"))
  (:Completed
    (Variables|Default|SetRotation_Desired (Math|Rotator|CombineRotators (Variables|Default|GetRotation_Desired) (Math|Rotator|MakeRotator 0.0 0.0 (* (Variables|Default|GetRotationSpeed) -1.0))))))

(event Input|EnhancedActionEvents|EnhancedInputActionIA_RotateCameraLeft
  (params (ActionValue :type Boolean) (ElapsedSeconds :type Float%20%28double-precision%29) (TriggeredSeconds :type Float%20%28double-precision%29) (InputAction :type Input%20Action%20Object%20Reference :default "/Game/Blueprints/Core/Player/IA_RotateCameraLeft.IA_RotateCameraLeft"))
  (:Completed
    (Variables|Default|SetRotation_Desired (Math|Rotator|CombineRotators (Variables|Default|GetRotation_Desired) (Math|Rotator|MakeRotator 0.0 0.0 (Variables|Default|GetRotationSpeed))))))

(event EventBeginPlay
  (bind _asbp_player_controller (Utilities|Casting|CastToBP_PlayerController (Pawn|GetController)))
  (Input|AddMappingContext (PlayerController|LocalPlayerSubsystems|GetEnhancedInputLocalPlayerSubsystem _asbp_player_controller) "/Game/Blueprints/Core/Player/IMC_Player.IMC_Player" 0 "(bIgnoreAllPressedKeysUntilRelease=True,bForceImmediately=False)")
  (Variables|Default|SetLocation_Desired (Transformation|GetActorLocation))
  (Variables|Default|SetZoom_Desired (Variables|/Script/Engine.SpringArmComponent|GetTargetArmLength (Variables|Default|GetSpringArm)))
  (Variables|Default|SetRotation_Desired (Transformation|GetActorRotation)))

(event EventTick
  (params (DeltaSeconds :type Float%20%28single-precision%29))
  (bind _springarm (Variables|Default|GetSpringArm))
  (Variables|/Script/Engine.SpringArmComponent|SetTargetArmLength _springarm (Math|Interpolation|FInterpTo (Variables|/Script/Engine.SpringArmComponent|GetTargetArmLength _springarm) (Variables|Default|GetZoom_Desired) DeltaSeconds (Variables|Default|GetZoomInterpSpeed)))
  (Transformation|SetActorLocation (Math|Interpolation|VInterpTo (Transformation|GetActorLocation) (Variables|Default|GetLocation_Desired) DeltaSeconds (Variables|Default|GetLocationInterpSpeed)) false false)
  (Transformation|SetActorRotation (Math|Interpolation|RInterpTo (Transformation|GetActorRotation) (Variables|Default|GetRotation_Desired) DeltaSeconds (Variables|Default|GetRotationInterpSpeed))))

(fn ConstructionScript)