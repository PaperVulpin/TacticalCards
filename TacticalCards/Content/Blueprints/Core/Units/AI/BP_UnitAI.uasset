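; Actor that plays an AI unit's turn in grid-based tactical combat: move, cast the best ability, reposition and end the turn.
; It brute-force scores ability, origin and target combinations by cost-weighted impact, kill chance and travel distance.
; End-turn movement picks a reachable tile toward or away from allies or enemies.
; Event-driven async pathfinding and time-sliced manual loops spread the work across frames, with delayed state changes broadcast between phases.
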(event EventBeginPlay)

(event Collision|EventActorBeginOverlap
  (params (OtherActor :type Actor%20Object%20Reference)))

(event EventTick
  (params (DeltaSeconds :type Float%20%28single-precision%29)))

(event Custom|Event_RunAILogic
  (Utilities|SetAIStatewithDelay "NewEnumerator1")
  (CallFunction|DecideWhichAbilitytoCast))

(event Custom|MoveToEndTurnLocation_Done
  (Utilities|SetAIStatewithDelay "NewEnumerator7")
  (CallFunction|AIEndTurn))

(event Custom|DecideWhichAbilityToCast_Done
  (if (Utilities|Struct|BreakS_UnitAIAbilityCastingData (Variables|Default|GetAIAbilityCasting)) ; Able to cast an ability?
    (CallFunction|MovetoAbilityCastingLocation)
    (else
      (CallFunction|DecideWheretoEndTurn))))

(event Custom|MoveToAbilityCastingLocation_Done
  (CallFunction|CastAbility))

(event Custom|CastAbility_Done
  (CallFunction|DecideWheretoEndTurn))

(event Custom|OnCompleted_EndTurnReachables
  (params (Path :type Array%20of%20Int%20Point%20Structures))
  (bind _unit (Variables|Default|GetUnit))
  (bind _unitdata (Variables|/Game/Blueprints/Core/Units/BP_Unit.BP_Unit_C|GetUnitData _unit))
  (bind _stats (Utilities|Struct|BreakS_UnitData _unitdata))
  (bind (_validtiletypes _canmovediagonally _movement_current) (Utilities|Struct|BreakS_UnitData_Stats _stats))
  (EventDispatchers|UnbindEventfromOnPathfindingCompleted (CallFunction|GetAIPathfinding) (delegate Custom|OnCompleted_EndTurnReachables))
  (bind _index (CallFunction|FindBestIndexinReachables Path))
  (EventDispatchers|BindEventtoOnPathfindingCompleted (CallFunction|GetAIPathfinding) (delegate Custom|OnCompleted_EndTurnPath))
  (Default|FindPath (CallFunction|GetAIPathfinding) (Variables|/Game/Blueprints/Core/Units/BP_Unit.BP_Unit_C|GetIndex _unit) _index _canmovediagonally _validtiletypes 0.1 15.0 false _movement_current))

(event Custom|OnCompleted_EndTurnPath
  (params (Path :type Array%20of%20Int%20Point%20Structures))
  (EventDispatchers|UnbindEventfromOnPathfindingCompleted (CallFunction|GetAIPathfinding) (delegate Custom|OnCompleted_EndTurnPath))
  (CallFunction|DecideWheretoEndTurnDone Path))

(event Custom|DecideWhereToEndTurn_Done
  (params (Path :type Array%20of%20Int%20Point%20Structures))
  (CallFunction|MovetoEndTurnLocation Path))

(event Custom|MoveToEndTurnLocation
  (params (Path :type Array%20of%20Int%20Point%20Structures))
  (if (> (Utilities|Array|Length Path) 0) ; Need to move?
    (Utilities|SetAIStatewithDelay "NewEnumerator6")
    (EventDispatchers|BindEventtoOnUnitFinishedWalking (Variables|Default|GetUnit) (delegate Custom|OnCompleted_EndTurnUnitWalking))
    (Default|MoveUnit (Variables|Default|GetCombatSystem) (Variables|Default|GetUnit) Path)
    (else
      (CallFunction|MovetoEndTurnLocationDone))))

(event Custom|OnCompleted_EndTurnUnitWalking
  (params (Unit :type BP%20Unit%20Object%20Reference))
  (EventDispatchers|UnbindEventfromOnUnitFinishedWalking Unit (delegate Custom|OnCompleted_EndTurnUnitWalking))
  (CallFunction|MovetoEndTurnLocationDone))

(event Custom|DecideWhereToEndTurn
  (bind _unit (Variables|Default|GetUnit))
  (bind _unitdata (Variables|/Game/Blueprints/Core/Units/BP_Unit.BP_Unit_C|GetUnitData _unit))
  (bind _stats (Utilities|Struct|BreakS_UnitData _unitdata))
  (bind (_validtiletypes _canmovediagonally _movement_current) (Utilities|Struct|BreakS_UnitData_Stats _stats))
  (Utilities|SetAIStatewithDelay "NewEnumerator5")
  (if (> (Utilities|Struct|BreakS_UnitData_Stats (Utilities|Struct|BreakS_UnitData (Variables|/Game/Blueprints/Core/Units/BP_Unit.BP_Unit_C|GetUnitData (Variables|Default|GetUnit)))) 0) ; Can unit move?
    (EventDispatchers|BindEventtoOnPathfindingCompleted (CallFunction|GetAIPathfinding) (delegate Custom|OnCompleted_EndTurnReachables))
    (Default|FindPath (CallFunction|GetAIPathfinding) (Variables|/Game/Blueprints/Core/Units/BP_Unit.BP_Unit_C|GetIndex _unit) (Utilities|Struct|MakeIntPoint -999 -999) _canmovediagonally _validtiletypes 0.1 15.0 true _movement_current)
    (else
      (CallFunction|DecideWheretoEndTurnDone (Utilities|Array|MakeArray)))))

(event Custom|OnCompleted_AbilityPath
  (params (Path :type Array%20of%20Int%20Point%20Structures))
  (bind _unit (Variables|Default|GetUnit))
  (EventDispatchers|UnbindEventfromOnPathfindingCompleted (CallFunction|GetAIPathfinding) (delegate Custom|OnCompleted_AbilityPath))
  (EventDispatchers|BindEventtoOnUnitFinishedWalking _unit (delegate Custom|OnCompleted_AbilityUnitWalking))
  (Default|MoveUnit (Variables|Default|GetCombatSystem) _unit Path))

(event Custom|OnCompleted_AbilityReachables
  (params (Path :type Array%20of%20Int%20Point%20Structures))
  (EventDispatchers|UnbindEventfromOnPathfindingCompleted (CallFunction|GetAIPathfinding) (delegate Custom|OnCompleted_AbilityReachables))
  (Variables|Default|SetTimeOfLastDelay (Math|DateTime|Now))
  (bind _abilities (CallFunction|GetCastableAbilities))
  (bind _array_element (Utilities|ManualforEachLoop _abilities :!label _label) ; Loop through abilities
    (:LoopBody
      (bind _array_element_2 (Utilities|ManualforEachLoop Path :!label _label_2) ; Loop through all origin indexes
        (:LoopBody
          (bind _rangeindexes (Default|GetAbilityRange (Variables|Default|GetCombatSystem) _array_element_2 (Utilities|Struct|BreakS_AbilityData _array_element)))
          (bind _array_element_3 (Utilities|ManualforEachLoop _rangeindexes :!label _label_3) ; Loop through all target indexes
            (:LoopBody
              (CallFunction|CalculateAbilityScoreandUpdateAbilityCasting _array_element_3 _array_element_2 _array_element)
              (Utilities|DelayifTakingTooLong)
              (goto _label_3 NextLoop))
            (:Completed
              (Utilities|DelayifTakingTooLong)
              (goto _label_2 NextLoop))))
        (:Completed
          (Utilities|DelayifTakingTooLong)
          (goto _label NextLoop))))
    (:Completed
      (CallFunction|DecideWhichAbilitytoCastDone))))

(event Custom|DecideWhichAbilityToCast
  (bind _unit (Variables|Default|GetUnit))
  (bind _unitdata (Variables|/Game/Blueprints/Core/Units/BP_Unit.BP_Unit_C|GetUnitData _unit))
  (bind _stats (Utilities|Struct|BreakS_UnitData _unitdata))
  (bind (_validtiletypes _canmovediagonally _movement_current) (Utilities|Struct|BreakS_UnitData_Stats _stats))
  (Utilities|SetAIStatewithDelay "NewEnumerator2")
  (Variables|Default|SetAIAbilityCasting "")
  (EventDispatchers|BindEventtoOnPathfindingCompleted (CallFunction|GetAIPathfinding) (delegate Custom|OnCompleted_AbilityReachables))
  (Default|FindPath (CallFunction|GetAIPathfinding) (Variables|/Game/Blueprints/Core/Units/BP_Unit.BP_Unit_C|GetIndex _unit) (Utilities|Struct|MakeIntPoint -999 -999) _canmovediagonally _validtiletypes 0.1 15.0 true _movement_current))

(event Custom|OnCompleted_AbilityUnitWalking
  (params (Unit :type BP%20Unit%20Object%20Reference))
  (EventDispatchers|UnbindEventfromOnUnitFinishedWalking (Variables|Default|GetUnit) (delegate Custom|OnCompleted_AbilityUnitWalking))
  (CallFunction|MovetoAbilityCastingLocationDone))

(event Custom|MoveToAbilityCastingLocation
  (bind _unit (Variables|Default|GetUnit))
  (bind _unitdata (Variables|/Game/Blueprints/Core/Units/BP_Unit.BP_Unit_C|GetUnitData _unit))
  (bind _stats (Utilities|Struct|BreakS_UnitData _unitdata))
  (bind (_validtiletypes _canmovediagonally _movement_current) (Utilities|Struct|BreakS_UnitData_Stats _stats))
  (if (!= (Variables|/Game/Blueprints/Core/Units/BP_Unit.BP_Unit_C|GetIndex (Variables|Default|GetUnit)) (Utilities|Struct|BreakS_UnitAIAbilityCastingData (Variables|Default|GetAIAbilityCasting))) ; Need to move?
    (Utilities|SetAIStatewithDelay "NewEnumerator3")
    (EventDispatchers|BindEventtoOnPathfindingCompleted (CallFunction|GetAIPathfinding) (delegate Custom|OnCompleted_AbilityPath))
    (Default|FindPath (CallFunction|GetAIPathfinding) (Variables|/Game/Blueprints/Core/Units/BP_Unit.BP_Unit_C|GetIndex (Variables|Default|GetUnit)) (Utilities|Struct|BreakS_UnitAIAbilityCastingData (Variables|Default|GetAIAbilityCasting)) _canmovediagonally _validtiletypes 0.1 15.0 false _movement_current)
    (else
      (CallFunction|MovetoAbilityCastingLocationDone))))

(event Custom|CastAbility
  (bind _aiabilitycasting (Variables|Default|GetAIAbilityCasting))
  (bind (_ability _originindex _targetindex) (Utilities|Struct|BreakS_UnitAIAbilityCastingData _aiabilitycasting))
  (Utilities|SetAIStatewithDelay "NewEnumerator4")
  (Default|CastAbility (Variables|Default|GetCombatSystem) _ability _originindex _targetindex)
  (Utilities|FlowControl|Delay 0.5)
  (CallFunction|CastAbilityDone))

(fn ConstructionScript)

(fn AIPlayTurn
  (CallFunction|EventRunAILogic))

(fn AIEndTurn
  (Default|NextUnit (Variables|Default|GetCombatSystem)))

(fn GetAIPathfinding
  (return (Variables|/Game/Blueprints/Core/Grid/BP_Grid.BP_Grid_C|GetGridPathfinding_AI (Variables|/Game/Blueprints/Core/Combat/BP_CombatSystem.BP_CombatSystem_C|GetGrid (Variables|Default|GetCombatSystem)))))

(fn FindBestIndexinReachables
  (params (Reachables :type Array%20of%20Int%20Point%20Structures))
  (bind _unit (Variables|Default|GetUnit))
  (bind _unitdata (Variables|/Game/Blueprints/Core/Units/BP_Unit.BP_Unit_C|GetUnitData _unit))
  (bind _ai (Utilities|Struct|BreakS_UnitData _unitdata))
  (bind _movementlogic (Utilities|Struct|BreakS_UnitData_AI _ai))
  (Utilities|FlowControl|Sequence
    (:then_0
      (switch Utilities|FlowControl|Switch|SwitchonE_UnitAIMovementLogic _movementlogic
        (:NewEnumerator0
          (bind _units (CallFunction|GetEnemyUnits (Utilities|Array|MakeArray) :!label _label))
          (bind _keys (Utilities|Map|Keys _units))
          (LocalVariables|SetEnemiesOrAllies _keys))
        (:NewEnumerator1
          (bind _units_2 (CallFunction|GetAllyUnits false :!label _label_2))
          (bind _keys_2 (Utilities|Map|Keys _units_2))
          (bind _output_get (LocalVariables|SetEnemiesOrAllies _keys_2))
          (if (== (Utilities|Array|Length _output_get) 0) ; No allies left in team?
            (goto _label)))
        (:NewEnumerator2
          (goto _label))
        (:NewEnumerator3
          (goto _label_2))))
    (:then_1
      (switch Utilities|FlowControl|Switch|SwitchonE_UnitAIMovementLogic _movementlogic
        (:NewEnumerator0
          _)
        (:NewEnumerator1
          _)
        (:NewEnumerator2
          (bind _index (CallFunction|FindFarthestIndex Reachables (LocalVariables|GetEnemiesOrAllies) :!label _label_3))
          (return _index))
        (:NewEnumerator3
          (goto _label_3)))
      (bind _index_2 (CallFunction|FindClosestIndex Reachables (LocalVariables|GetEnemiesOrAllies)))
      (return _index_2))))

(fn GetAllyUnits
  (params (IncludeSelf :type Boolean))
  (bind _result (Utilities|Set|ToArray (Utilities|Struct|BreakS_UnitSet (.Value (Utilities|Map|Find (Variables|/Game/Blueprints/Core/Combat/BP_CombatSystem.BP_CombatSystem_C|GetUnitTeams (Variables|Default|GetCombatSystem)) (Variables|/Game/Blueprints/Core/Units/BP_Unit.BP_Unit_C|GetTeamIndex (Variables|Default|GetUnit)))))))
  (for _array_element _result
    (bind _output_get (LocalVariables|SetU _array_element))
    (if (Default|IsAlive _output_get) ; Is unit alive?
      (if (or (!= _output_get (Variables|Default|GetUnit)) IncludeSelf) ; Include self?
        (Utilities|Map|Add (LocalVariables|GetRet) (Variables|/Game/Blueprints/Core/Units/BP_Unit.BP_Unit_C|GetIndex (LocalVariables|GetU)) (LocalVariables|GetU)))))
  (return (LocalVariables|GetRet)))

(fn GetEnemyUnits
  (params (SpecificTeamIndexes :type Array%20of%20Integers))
  (if (> (Utilities|Array|Length SpecificTeamIndexes) 0) ; Any requested indexes?
    (LocalVariables|SetTeams SpecificTeamIndexes)
    (else
      (bind _keys (Utilities|Map|Keys (Variables|/Game/Blueprints/Core/Combat/BP_CombatSystem.BP_CombatSystem_C|GetUnitTeams (Variables|Default|GetCombatSystem))))
      (LocalVariables|SetTeams _keys)))
  (Utilities|Array|RemoveItem (LocalVariables|GetTeams) (Variables|/Game/Blueprints/Core/Units/BP_Unit.BP_Unit_C|GetTeamIndex (Variables|Default|GetUnit)))
  (for _array_element (LocalVariables|GetTeams)
    (bind _result (Utilities|Set|ToArray (Utilities|Struct|BreakS_UnitSet (.Value (Utilities|Map|Find (Variables|/Game/Blueprints/Core/Combat/BP_CombatSystem.BP_CombatSystem_C|GetUnitTeams (Variables|Default|GetCombatSystem)) _array_element)))))
    (for _array_element_2 _result
      (bind _output_get (LocalVariables|SetU _array_element_2))
      (if (Default|IsAlive _output_get)
        (Utilities|Map|Add (LocalVariables|GetRet) (Variables|/Game/Blueprints/Core/Units/BP_Unit.BP_Unit_C|GetIndex (LocalVariables|GetU)) (LocalVariables|GetU)))))
  (return (LocalVariables|GetRet)))

(fn FindClosestIndex
  (params (Reachables :type Array%20of%20Int%20Point%20Structures) (PossibleTargets :type Array%20of%20Int%20Point%20Structures))
  (LocalVariables|SetSmallestDistance 999999999)
  (for _array_element Reachables
    (LocalVariables|SetReachable _array_element)
    (for _array_element_2 PossibleTargets
      (LocalVariables|SetTarget _array_element_2)
      (bind _output_get (LocalVariables|SetNewDistance (Default|GetMinimumCostBetweenTwoTiles (Variables|/Game/Blueprints/Core/Grid/BP_Grid.BP_Grid_C|GetGridPathfinding_AI (Variables|/Game/Blueprints/Core/Combat/BP_CombatSystem.BP_CombatSystem_C|GetGrid (Variables|Default|GetCombatSystem))) (LocalVariables|GetReachable) (LocalVariables|GetTarget) (Utilities|Struct|BreakS_UnitData_Stats (Utilities|Struct|BreakS_UnitData (Variables|/Game/Blueprints/Core/Units/BP_Unit.BP_Unit_C|GetUnitData (Variables|Default|GetUnit)))))))
      (if (< _output_get (LocalVariables|GetSmallestDistance))
        (LocalVariables|SetRet (LocalVariables|GetReachable))
        (LocalVariables|SetSmallestDistance (LocalVariables|GetNewDistance)))))
  (return (LocalVariables|GetRet)))

(fn FindFarthestIndex
  (params (Reachables :type Array%20of%20Int%20Point%20Structures) (IndexesToAvoid :type Array%20of%20Int%20Point%20Structures))
  (LocalVariables|SetBiggestDistance -999)
  (for _array_element Reachables
    (LocalVariables|SetReachable _array_element)
    (LocalVariables|SetNewDistance 999999999)
    (for _array_element_2 IndexesToAvoid
      (LocalVariables|SetToAvoid _array_element_2)
      (LocalVariables|SetNewDistance (Math|Integer|Min(Integer) (LocalVariables|GetNewDistance) (Default|GetMinimumCostBetweenTwoTiles (Variables|/Game/Blueprints/Core/Grid/BP_Grid.BP_Grid_C|GetGridPathfinding_AI (Variables|/Game/Blueprints/Core/Combat/BP_CombatSystem.BP_CombatSystem_C|GetGrid (Variables|Default|GetCombatSystem))) (LocalVariables|GetReachable) (LocalVariables|GetToAvoid) (Utilities|Struct|BreakS_UnitData_Stats (Utilities|Struct|BreakS_UnitData (Variables|/Game/Blueprints/Core/Units/BP_Unit.BP_Unit_C|GetUnitData (Variables|Default|GetUnit))))))))
    (if (> (LocalVariables|GetNewDistance) (LocalVariables|GetBiggestDistance))
      (LocalVariables|SetRet (LocalVariables|GetReachable))
      (LocalVariables|SetBiggestDistance (LocalVariables|GetNewDistance))))
  (return (LocalVariables|GetRet)))

(fn GetCastableAbilities
  (for _array_element (Utilities|Struct|BreakS_UnitData_Stats (Utilities|Struct|BreakS_UnitData (Variables|/Game/Blueprints/Core/Units/BP_Unit.BP_Unit_C|GetUnitData (Variables|Default|GetUnit))))
    (bind _abilitydata (CallFunction|GetAbilityDatafromAbility _array_element))
    (bind _cancast (Default|CanCastAbility (Variables|Default|GetUnit) _abilitydata))
    (if _cancast
      (Utilities|Array|Add (LocalVariables|GetRet) _abilitydata)))
  (return (LocalVariables|GetRet)))

(fn CalculateAbilityScoreandUpdateAbilityCasting
  (params (Target :type Int%20Point%20Structure) (Origin :type Int%20Point%20Structure) (Ability :type S%20Ability%20Data%20Structure))
  (bind _allunits (CallFunction|GetAllUnits false))
  (LocalVariables|SetAllUnitsExceptSelf _allunits)
  (bind _attackedindexes (Default|GetAttackedIndexes (Variables|Default|GetCombatSystem) Ability Target))
  (LocalVariables|SetAttackedIndexes _attackedindexes)
  (LocalVariables|SetTotalAbilityScore (* (Math|Vector|Distance2D(Vector) (Math|Conversions|ToVector2D(IntPoint) (Variables|/Game/Blueprints/Core/Units/BP_Unit.BP_Unit_C|GetIndex (Variables|Default|GetUnit))) (Math|Conversions|ToVector2D(IntPoint) Origin)) -0.1))
  (for _array_element (LocalVariables|GetAttackedIndexes)
    (bind _output_get (LocalVariables|SetAttackedIndex _array_element))
    (if (Class|KismetMathLibrary|EqualIntPointIntPoint _output_get Origin) ; Hit self?
      (LocalVariables|SetAttackedUnit (Variables|Default|GetUnit))
      (else
        (LocalVariables|SetAttackedUnit (.Value (Utilities|Map|Find (LocalVariables|GetAllUnitsExceptSelf) (LocalVariables|GetAttackedIndex))))))
    (Utilities|IsValid (LocalVariables|GetAttackedUnit)
      (:Is%20Valid
        (bind _impactscore (CallFunction|CalculateImpactScore Ability (LocalVariables|GetAttackedUnit)))
        (LocalVariables|SetTotalAbilityScore (+ _impactscore (LocalVariables|GetTotalAbilityScore))))))
  (if (> (LocalVariables|GetTotalAbilityScore) (Utilities|Struct|BreakS_UnitAIAbilityCastingData (Variables|Default|GetAIAbilityCasting))) ; Is this ability better?
    (Variables|Default|SetAIAbilityCasting (Utilities|Struct|MakeS_UnitAIAbilityCastingData true (Utilities|Struct|BreakS_AbilityData Ability) Origin Target (LocalVariables|GetTotalAbilityScore)))))

(fn GetAllUnits
  (params (IncludeSelf :type Boolean))
  (for _array_element (Variables|/Game/Blueprints/Core/Combat/BP_CombatSystem.BP_CombatSystem_C|GetUnitsInCombat (Variables|Default|GetCombatSystem))
    (bind _output_get (LocalVariables|SetU _array_element))
    (if (Default|IsAlive _output_get)
      (if (or (!= _output_get (Variables|Default|GetUnit)) IncludeSelf)
        (Utilities|Map|Add (LocalVariables|GetRet) (Variables|/Game/Blueprints/Core/Units/BP_Unit.BP_Unit_C|GetIndex (LocalVariables|GetU)) (LocalVariables|GetU)))))
  (return (LocalVariables|GetRet)))

(fn CalculateImpactScore
  (params (Ability :type S%20Ability%20Data%20Structure) (AttackedUnit :type BP%20Unit%20Object%20Reference))
  (bind _requirements (Utilities|Struct|BreakS_AbilityData Ability))
  (bind _impact (Utilities|Struct|BreakS_AbilityData Ability))
  (bind _impact_2 (Utilities|Struct|BreakS_AbilityData Ability))
  (bind _impact_3 (Utilities|Struct|BreakS_AbilityData Ability))
  (bind _unitdata (Variables|/Game/Blueprints/Core/Units/BP_Unit.BP_Unit_C|GetUnitData AttackedUnit))
  (bind (_cost_hp _cost_ap _cost_movement) (Utilities|Struct|BreakS_AbilityData_Requirements _requirements))
  (bind _minmaxmodifier_hp (Utilities|Struct|BreakS_AbilityData_Impact _impact))
  (bind (_minmaxmodifier_ap _minmaxmodifier_movement) (Utilities|Struct|BreakS_AbilityData_Impact _impact_2))
  (bind _stats (Utilities|Struct|BreakS_UnitData _unitdata))
  (bind _minmaxmodifier_hp_2 (Utilities|Struct|BreakS_AbilityData_Impact _impact_3))
  (bind (_x _y) (Utilities|Struct|BreakIntPoint _minmaxmodifier_hp))
  (bind (_x_2 _y_2) (Utilities|Struct|BreakIntPoint _minmaxmodifier_hp_2))
  (bind (_validtiletypes _canmovediagonally _availableabilities _hp_current _hp_max) (Utilities|Struct|BreakS_UnitData_Stats _stats))
  (bind _returnvalue (Math|Integer|Absolute(Integer) _x))
  (bind _returnvalue_2 (- _hp_max _hp_current))
  (bind _returnvalue_3 (Math|Conversions|ToFloat(Integer) _returnvalue))
  (LocalVariables|SetHPValue 1.0)
  (LocalVariables|SetMovementValue 1.5)
  (LocalVariables|SetAPValue 1.5)
  (LocalVariables|SetKillingBlowValue 1e+02)
  (Utilities|FlowControl|Sequence
    (:then_0
      (LocalVariables|SetCost (+ (* _cost_hp (LocalVariables|GetHPValue)) (* _cost_ap (LocalVariables|GetAPValue)) (* _cost_movement (LocalVariables|GetMovementValue))))
      (LocalVariables|SetIsAlly (== (Variables|/Game/Blueprints/Core/Units/BP_Unit.BP_Unit_C|GetTeamIndex (Variables|Default|GetUnit)) (Variables|/Game/Blueprints/Core/Units/BP_Unit.BP_Unit_C|GetTeamIndex AttackedUnit)))
      (LocalVariables|SetHPScore (CallFunction|CalculateStatScore (select (> _x_2 0) (Utilities|Struct|MakeIntPoint (Math|Integer|Min(Integer) _x_2 _returnvalue_2) (Math|Integer|Min(Integer) _y_2 _returnvalue_2)) _minmaxmodifier_hp_2) (LocalVariables|GetHPValue) (LocalVariables|GetIsAlly)))
      (LocalVariables|SetAPScore (CallFunction|CalculateStatScore _minmaxmodifier_ap (LocalVariables|GetAPValue) (LocalVariables|GetIsAlly)))
      (LocalVariables|SetMovementScore (CallFunction|CalculateStatScore _minmaxmodifier_movement (LocalVariables|GetMovementValue) (LocalVariables|GetIsAlly)))
      (if (< (.X (Utilities|Struct|BreakIntPoint (Utilities|Struct|BreakS_AbilityData_Impact (Utilities|Struct|BreakS_AbilityData Ability)))) 0) ; Is damage?
        (LocalVariables|SetKillingBlowScore (* (Math|Float|Clamp(Float) (- 1.0 (/ (- (Math|Conversions|ToFloat(Integer) (Utilities|Struct|BreakS_UnitData_Stats (Utilities|Struct|BreakS_UnitData (Variables|/Game/Blueprints/Core/Units/BP_Unit.BP_Unit_C|GetUnitData AttackedUnit)))) _returnvalue_3) (- _returnvalue_3 (+ (Math|Conversions|ToFloat(Integer) (Math|Integer|Absolute(Integer) _y)) 1.0))))) (LocalVariables|GetKillingBlowValue) (select (LocalVariables|GetIsAlly) -1.0 1.0)))
        (else
          (LocalVariables|SetKillingBlowScore 0.0))))
    (:then_1
      (return (/ (+ (LocalVariables|GetHPScore) (LocalVariables|GetAPScore) (LocalVariables|GetMovementScore) (LocalVariables|GetKillingBlowScore)) (Math|Float|Max(Float) (LocalVariables|GetCost) 1.0))))))

(fn CalculateStatScore
  (params (ImpactMinMax :type Int%20Point%20Structure%20%28by%20ref%29) (StatValue :type Float%20%28double-precision%29) (IsAlly :type Boolean))
  (bind (_x _y) (Utilities|Struct|BreakIntPoint ImpactMinMax))
  (bind _returnvalue (+ _x _y))
  (bind _returnvalue_2 (/ _returnvalue 2))
  (return (* (Math|Float|Absolute(Float) (* _returnvalue_2 StatValue)) (select (== (> _returnvalue_2 0) IsAlly) 1.0 -1.0))))