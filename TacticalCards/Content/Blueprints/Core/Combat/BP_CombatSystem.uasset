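; BP_CombatSystem runs turn-based grid combat, tracking units, teams, tile occupancy and the combat lifecycle.
; It cycles turns through living units, charges movement by path cost, and revalidates units when the grid or tiles change.
; Abilities resolve range and AoE from patterns, walkability and offset line-of-sight traces, then spawn an animation actor and apply impacts.
; Deaths free tiles and finish combat when one team survives, stopping further impacts to prevent ties.
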(event EventBeginPlay
  (bind _grid (Variables|Default|GetGrid))
  (EventDispatchers|BindEventtoOnGridGenerated _grid (EventDispatchers|CreateEvent :!event OnGridGenerated))
  (EventDispatchers|BindEventtoOnTileDataUpdated _grid (EventDispatchers|CreateEvent :!event OnTileDataUpdated)))

(event Collision|EventActorBeginOverlap
  (params (OtherActor :type Actor%20Object%20Reference)))

(event EventTick
  (params (DeltaSeconds :type Float%20%28single-precision%29)))

(fn ConstructionScript)

(fn AddUnitinCombat
  (params (Unit :type BP%20Unit%20Object%20Reference) (Index :type Int%20Point%20Structure) (TeamIndex :type Integer))
  (Utilities|Array|Add (Variables|Default|GetUnitsInCombat) Unit)
  (Default|SetGrid Unit (Variables|Default|GetGrid))
  (Units|SetUnitIndexonGrid Unit Index false true)
  (EventDispatchers|BindEventtoOnUnitReachedNewTile Unit (EventDispatchers|CreateEvent :!event OnUnitReachedNewTile))
  (CallFunction|SetUnitTeamIndex Unit TeamIndex))

(fn RemoveUnitfromCombat
  (params (Unit :type BP%20Unit%20Object%20Reference) (DestroyUnit :type Boolean))
  (Utilities|Array|RemoveItem (Variables|Default|GetUnitsInCombat) Unit)
  (Units|SetUnitIndexonGrid Unit (Utilities|Struct|MakeIntPoint -999 -999) false true)
  (CallFunction|SetUnitTeamIndex Unit -1)
  (if DestroyUnit
    (Actor|DestroyActor Unit)))

(fn SetUnitIndexonGrid
  (params (Unit :type BP%20Unit%20Object%20Reference) (Index :type Int%20Point%20Structure) (Force :type Boolean) (SnapLocation :type Boolean))
  (bind _grid (Variables|Default|GetGrid))
  (bind _gridtiles (Variables|/Game/Blueprints/Core/Grid/BP_Grid.BP_Grid_C|GetGridTiles _grid))
  (bind (_value _returnvalue) (Utilities|Map|Find _gridtiles Index))
  (Utilities|FlowControl|Sequence
    (:then_0
      (if (or (!= (Variables|/Game/Blueprints/Core/Units/BP_Unit.BP_Unit_C|GetIndex Unit) Index) Force)
        (Utilities|FlowControl|Sequence
          (:then_0
            (bind _output_get (LocalVariables|SetPreviousTile (.Value (Utilities|Map|Find (Variables|/Game/Blueprints/Core/Grid/BP_Grid.BP_Grid_C|GetGridTiles (Variables|Default|GetGrid)) (Variables|/Game/Blueprints/Core/Units/BP_Unit.BP_Unit_C|GetIndex Unit)))))
            (if (== (Utilities|Struct|BreakS_TileData _output_get) Unit)
              (bind _structout (Utilities|Struct|SetmembersinS_TileData (LocalVariables|GetPreviousTile) 0))
              (Utilities|Map|Add (Variables|/Game/Blueprints/Core/Grid/BP_Grid.BP_Grid_C|GetGridTiles (Variables|Default|GetGrid)) (Utilities|Struct|BreakS_TileData _structout) _structout)))
          (:then_1
            (Default|SetGridIndex Unit Index)
            (if (!= Index (Utilities|Struct|MakeIntPoint -999 -999))
              (bind _structout_2 (Utilities|Struct|SetmembersinS_TileData (.Value (Utilities|Map|Find (Variables|/Game/Blueprints/Core/Grid/BP_Grid.BP_Grid_C|GetGridTiles (Variables|Default|GetGrid)) Index)) Unit))
              (Utilities|Map|Add (Variables|/Game/Blueprints/Core/Grid/BP_Grid.BP_Grid_C|GetGridTiles (Variables|Default|GetGrid)) (Utilities|Struct|BreakS_TileData _structout_2) _structout_2)))
          (:then_2
            (Default|CallOnUnitGridIndexChanged Unit)))))
    (:then_1
      (if SnapLocation
        (Transformation|SetActorLocation Unit (select _returnvalue (.location (Utilities|Struct|BreakS_TileData _value)) "-99999.000000,-99999.000000,-99999.000000") false false)))))

(fn OnGridGenerated
  (bind _output_get (LocalVariables|SetCopyOfUnitsInCombat (Variables|Default|GetUnitsInCombat)))
  (for _array_element _output_get
    (if (Utilities|Array|ContainsItem (.ValidTileTypes (Utilities|Struct|BreakS_UnitData_Stats (.stats (Variables|/Game/Blueprints/Core/Units/BP_Unit.BP_Unit_C|GetUnitData _array_element)))) (.type (.Value (Utilities|Map|Find (Variables|/Game/Blueprints/Core/Grid/BP_Grid.BP_Grid_C|GetGridTiles (Variables|Default|GetGrid)) (Variables|/Game/Blueprints/Core/Units/BP_Unit.BP_Unit_C|GetIndex _array_element)))))
      (Units|SetUnitIndexonGrid _array_element (Variables|/Game/Blueprints/Core/Units/BP_Unit.BP_Unit_C|GetIndex _array_element) true true)
      (else
        (Units|RemoveUnitfromCombat _array_element true)))))

(fn OnTileDataUpdated
  (params (Index :type Int%20Point%20Structure))
  (bind _output_get (LocalVariables|SetCopyOfUnitsInCombat (Variables|Default|GetUnitsInCombat)))
  (bind _array_element (Utilities|Array|ForEachLoopwithBreak _output_get :!label _label)
    (:LoopBody
      (if (Class|KismetMathLibrary|EqualIntPointIntPoint Index (Variables|/Game/Blueprints/Core/Units/BP_Unit.BP_Unit_C|GetIndex _array_element))
        (if (Utilities|Array|ContainsItem (.ValidTileTypes (Utilities|Struct|BreakS_UnitData_Stats (.stats (Variables|/Game/Blueprints/Core/Units/BP_Unit.BP_Unit_C|GetUnitData _array_element)))) (.type (.Value (Utilities|Map|Find (Variables|/Game/Blueprints/Core/Grid/BP_Grid.BP_Grid_C|GetGridTiles (Variables|Default|GetGrid)) (Variables|/Game/Blueprints/Core/Units/BP_Unit.BP_Unit_C|GetIndex _array_element)))))
          (Units|SetUnitIndexonGrid _array_element (Variables|/Game/Blueprints/Core/Units/BP_Unit.BP_Unit_C|GetIndex _array_element) false true)
          (goto _label Break)
          (else
            (Units|RemoveUnitfromCombat _array_element true)
            (goto _label Break)))))))

(fn OnUnitReachedNewTile
  (params (Unit :type BP%20Unit%20Object%20Reference) (Index :type Int%20Point%20Structure))
  (Game|SpawnActorfromClass "/Game/Blueprints/UI/Core/BP_AnimatedNumber.BP_AnimatedNumber_C" (Math|Transform|MakeTransform (Transformation|GetActorLocation Unit) "0, 0, 0" "1.000000,1.000000,1.000000") "Undefined" "MultiplyWithRoot" 0 (- 0 (CallFunction|GetTileTypeCost (.Type (Utilities|Struct|BreakS_TileData (.Value (Utilities|Map|Find (Variables|/Game/Blueprints/Core/Grid/BP_Grid.BP_Grid_C|GetGridTiles (Variables|Default|GetGrid)) Index)))))) "NewEnumerator1" 0))

(fn CastAbility
  (params (Ability :type E_Ability%20Enum :default "NewEnumerator0") (OriginIndex :type Int%20Point%20Structure) (TargetIndex :type Int%20Point%20Structure))
  (bind _grid (Variables|Default|GetGrid))
  (bind _grid_2 (Variables|Default|GetGrid))
  (bind _gridtiles (Variables|/Game/Blueprints/Core/Grid/BP_Grid.BP_Grid_C|GetGridTiles _grid_2))
  (bind _gridtiles_2 (Variables|/Game/Blueprints/Core/Grid/BP_Grid.BP_Grid_C|GetGridTiles _grid))
  (bind _value (Utilities|Map|Find _gridtiles OriginIndex))
  (bind _value_2 (Utilities|Map|Find _gridtiles_2 OriginIndex))
  (bind _unitontile (Utilities|Struct|BreakS_TileData _value))
  (bind _unitontile_2 (Utilities|Struct|BreakS_TileData _value_2))
  (bind _abilitydata (CallFunction|GetAbilityDatafromAbility Ability))
  (bind _output_get (LocalVariables|SetData _abilitydata))
  (Utilities|IsValid _unitontile
    (:Is%20Valid
      (bind _cancast (Default|CanCastAbility _unitontile _output_get))
      (if _cancast
        (bind _rangeindexes (CallFunction|GetAbilityRange OriginIndex (.Cast (Utilities|Struct|BreakS_AbilityData _output_get)) :!label _label))
        (if (Utilities|Array|ContainsItem _rangeindexes TargetIndex)
          (if (Utilities|Enum|Equal(Enum) (.RangePattern (Utilities|Struct|BreakS_AbilityData_Cast (.CastAoE (Utilities|Struct|BreakS_AbilityData _output_get)))) "NewEnumerator0")
            (LocalVariables|SetAttackedIndexes (Utilities|Array|MakeArray TargetIndex))
            (else
              (bind _rangeindexes_2 (CallFunction|GetAbilityRange TargetIndex (.CastAoE (Utilities|Struct|BreakS_AbilityData _output_get))))
              (LocalVariables|SetAttackedIndexes _rangeindexes_2)))
          (bind _returnvalue (Game|SpawnActorfromClass (.Animation (Utilities|Struct|BreakS_AbilityData_Assets (.Assets (Utilities|Struct|BreakS_AbilityData _output_get)))) (Math|Transform|MakeTransform "0, 0, 0" "0, 0, 0" "1.000000,1.000000,1.000000") "AlwaysSpawn" "MultiplyWithRoot" 0 (Variables|Default|GetGrid) OriginIndex TargetIndex (LocalVariables|GetAttackedIndexes) 0))
          (LocalVariables|SetAbilityAnimation _returnvalue)
          (Utilities|FlowControl|Sequence
            (:then_0
              (Utilities|IsValid _unitontile_2
                (:Is%20Valid
                  (Default|UnitCastAbility _unitontile_2 TargetIndex (LocalVariables|GetData)))))
            (:then_1
              (LocalVariables|SetAbilityImpactReal (Utilities|Struct|MakeS_AbilityData_Impact_Real (CallFunction|MinMaxRandom (Utilities|Struct|BreakS_AbilityData_Impact (.Impact (Utilities|Struct|BreakS_AbilityData (LocalVariables|GetData)))))))
              (for _array_element (LocalVariables|GetAttackedIndexes)
                (bind _output_get_2 (LocalVariables|SetUnit (Utilities|Struct|BreakS_TileData (.Value (Utilities|Map|Find (Variables|/Game/Blueprints/Core/Grid/BP_Grid.BP_Grid_C|GetGridTiles (Variables|Default|GetGrid)) _array_element)))))
                (Utilities|IsValid _output_get_2
                  (:Is%20Valid
                    (if (Default|IsAlive (LocalVariables|GetUnit)) ; Might remove later
                      (Default|UnitHitbyAbility (LocalVariables|GetUnit) (LocalVariables|GetAbilityImpactReal) (LocalVariables|GetAbilityAnimation))
                      (if (not (Default|IsAlive (LocalVariables|GetUnit))) ; Just Died?
                        (CallFunction|ProcessUnitDeath (LocalVariables|GetUnit))
                        (if (Variables|Default|GetIsFinishingCombat) ; Prevents application of damage after winner has been declared. This prevents draws/ties.
                          (return))))))))))))
    (:Is%20Not%20Valid
      (goto _label))))

(fn GetAbilityRange
  (params (OriginIndex :type Int%20Point%20Structure) (Cast :type S%20Ability%20Data%20Cast%20Structure))
  (bind (_rangepattern _rangeminmax _lineofsight) (Utilities|Struct|BreakS_AbilityData_Cast Cast))
  (bind _indexes (CallFunction|GetIndexesfromPatternandRange OriginIndex (Variables|/Game/Blueprints/Core/Grid/BP_Grid.BP_Grid_C|GetGridShape (Variables|Default|GetGrid)) _rangepattern _rangeminmax))
  (bind _indexeswithlineofsight (CallFunction|RemoveNotWalkableIndexes _indexes))
  (if (.RequireLineOfSight (Utilities|Struct|BreakS_AbilityData_LineOfSight _lineofsight))
    (bind _indexeswithlineofsight_2 (CallFunction|RemoveIndexesWithoutLineOfSight OriginIndex _indexeswithlineofsight Cast))
    (return _indexeswithlineofsight_2)
    (else
      (return _indexeswithlineofsight))))

(fn HasLineOfSight
  (params (OriginIndex :type Int%20Point%20Structure) (TargetIndex :type Int%20Point%20Structure) (Cast :type S%20Ability%20Data%20Cast%20Structure))
  (bind _grid (Variables|Default|GetGrid))
  (bind _grid_2 (Variables|Default|GetGrid))
  (bind _lineofsight (Utilities|Struct|BreakS_AbilityData_Cast Cast))
  (bind _lineofsight_2 (Utilities|Struct|BreakS_AbilityData_Cast Cast))
  (bind _gridtiles (Variables|/Game/Blueprints/Core/Grid/BP_Grid.BP_Grid_C|GetGridTiles _grid_2))
  (bind _gridtilesize (Variables|/Game/Blueprints/Core/Grid/BP_Grid.BP_Grid_C|GetGridTileSize _grid))
  (bind _offsetfromcenter (Utilities|Struct|BreakS_AbilityData_LineOfSight _lineofsight_2))
  (bind _heightfromground (Utilities|Struct|BreakS_AbilityData_LineOfSight _lineofsight))
  (bind _returnvalue (Math|Vector|MakeVector 0.0 0.0 _heightfromground))
  (bind _returnvalue_2 (* _gridtilesize _offsetfromcenter))
  (bind _output_get (LocalVariables|SetOriginTile (.Value (Utilities|Map|Find _gridtiles OriginIndex))))
  (LocalVariables|SetTargetTile (.Value (Utilities|Map|Find _gridtiles TargetIndex)))
  (LocalVariables|SetStart (+ (.location (Utilities|Struct|BreakS_TileData _output_get)) _returnvalue))
  (LocalVariables|SetEnd (+ _returnvalue (.location (Utilities|Struct|BreakS_TileData (LocalVariables|GetTargetTile)))))
  (for _array_element (Utilities|Array|MakeArray (Math|Vector2D|MakeVector2D (.x _returnvalue_2) 0.0) (Math|Vector2D|MakeVector2D (- 0.0 (.x _returnvalue_2)) 0.0) (Math|Vector2D|MakeVector2D 0.0 (.y _returnvalue_2)) (Math|Vector2D|MakeVector2D 0.0 (- 0.0 (.y _returnvalue_2))))
    (bind _returnvalue_3 (Collision|LineTraceByChannel (+ (LocalVariables|GetStart) (Math|Conversions|ToVector(Vector2D) _array_element)) (LocalVariables|GetEnd) "TraceTypeQuery6" false (Utilities|Array|MakeArray (Utilities|Struct|BreakS_TileData (LocalVariables|GetOriginTile)) (Utilities|Struct|BreakS_TileData (LocalVariables|GetTargetTile))) (select (.DrawDebugLine (Utilities|Struct|BreakS_AbilityData_LineOfSight (Utilities|Struct|BreakS_AbilityData_Cast Cast))) "ForDuration" "None") true "(R=1.000000,G=0.000000,B=0.000000,A=1.000000)" "(R=0.000000,G=1.000000,B=0.000000,A=1.000000)" 3.0))
    (if (not _returnvalue_3)
      (return true)))
  (return false))

(fn RemoveIndexesWithoutLineOfSight
  (params (OriginIndex :type Int%20Point%20Structure) (Indexes :type Array%20of%20Int%20Point%20Structures) (Cast :type S%20Ability%20Data%20Cast%20Structure))
  (for _array_element Indexes
    (if (CallFunction|HasLineOfSight OriginIndex _array_element Cast)
      (Utilities|Array|Add (LocalVariables|GetReturn) _array_element)))
  (return (LocalVariables|GetReturn)))

(fn RemoveNotWalkableIndexes
  (params (Indexes :type Array%20of%20Int%20Point%20Structures))
  (for _array_element Indexes
    (if (Default|IsTileWalkable (Variables|Default|GetGrid) _array_element)
      (Utilities|Array|Add (LocalVariables|GetReturn) _array_element)))
  (return (LocalVariables|GetReturn)))

(fn SetUnitTeamIndex
  (params (Unit :type BP%20Unit%20Object%20Reference) (TeamIndex :type Integer))
  (Utilities|FlowControl|Sequence
    (:then_0
      (if (!= (Variables|/Game/Blueprints/Core/Units/BP_Unit.BP_Unit_C|GetTeamIndex Unit) -1) ; Is in a team already?
        (bind _output_get (LocalVariables|SetUnitSet (.unitset (.Value (Utilities|Map|Find (Variables|Default|GetUnitTeams) (Variables|/Game/Blueprints/Core/Units/BP_Unit.BP_Unit_C|GetTeamIndex Unit))))))
        (Utilities|Set|Remove _output_get Unit)
        (if (> (Utilities|Set|Length (LocalVariables|GetUnitSet)) 0)
          (Utilities|Map|Add (Variables|Default|GetUnitTeams) (Variables|/Game/Blueprints/Core/Units/BP_Unit.BP_Unit_C|GetTeamIndex Unit) (Utilities|Struct|MakeS_UnitSet (LocalVariables|GetUnitSet)))
          (else
            (Utilities|Map|Remove (Variables|Default|GetUnitTeams) (Variables|/Game/Blueprints/Core/Units/BP_Unit.BP_Unit_C|GetTeamIndex Unit))))))
    (:then_1
      (if (!= TeamIndex -1) ; Is valid team?
        (bind _output_get_2 (LocalVariables|SetUnitSet (.unitset (.Value (Utilities|Map|Find (Variables|Default|GetUnitTeams) TeamIndex)))))
        (Utilities|Set|Add _output_get_2 Unit)
        (Utilities|Map|Add (Variables|Default|GetUnitTeams) TeamIndex (Utilities|Struct|MakeS_UnitSet (LocalVariables|GetUnitSet)))))
    (:then_2
      (Default|SetTeamIndex Unit TeamIndex)
      (Default|CallOnUnitTeamsChanged))))

(fn CanStartCombat
  (bind _unitsincombat (Variables|Default|GetUnitsInCombat))
  (bind _unitteams (Variables|Default|GetUnitTeams))
  (bind _isincombat (Variables|Default|GetIsInCombat))
  (bind _returnvalue (Utilities|Array|Length _unitsincombat))
  (bind _returnvalue_2 (Utilities|Map|Length _unitteams))
  (bind _returnvalue_3 (not _isincombat))
  (bind _returnvalue_4 (>= _returnvalue 2))
  (bind _returnvalue_5 (>= _returnvalue_2 2))
  (return (Math|Boolean|ANDBoolean _returnvalue_4 _returnvalue_5 _returnvalue_3) _returnvalue_4 _returnvalue_5 _returnvalue_3))

(fn StartCombat
  (Variables|Default|SetIsInCombat true)
  (for _array_element (Variables|Default|GetUnitsInCombat)
    (Default|CombatStarted _array_element))
  (Default|CallOnCombatStarted)
  (Variables|Default|SetCurrentUnit 0)
  (CombatFlow|NextUnit))

(fn EndCombat
  (Variables|Default|SetIsInCombat false)
  (Variables|Default|SetIsFinishingCombat false)
  (Variables|Default|SetCurrentUnit 0)
  (for _array_element (Variables|Default|GetUnitsInCombat)
    (Default|CombatEnded _array_element))
  (Default|CallOnCombatEnded))

(fn NextUnit
  (Utilities|FlowControl|Sequence
    (:then_0
      (Utilities|IsValid (Variables|Default|GetCurrentUnit)
        (:Is%20Valid
          (Default|TurnedEnded (Variables|Default|GetCurrentUnit))
          (Default|CallOnUnitTurnEnded (Variables|Default|GetCurrentUnit)))))
    (:then_1
      (bind _output_get (LocalVariables|SetCurrentIndex (Utilities|Array|FindItem (Variables|Default|GetUnitsInCombat) (Variables|Default|GetCurrentUnit))))
      (while (not (Utilities|IsValid (LocalVariables|GetNextLivingUnit)))
        (LocalVariables|SetCurrentIndex (Math|Integer|%(Integer) (+ _output_get 1) (Utilities|Array|Length (Variables|Default|GetUnitsInCombat))))
        (if (Default|IsAlive (Utilities|Array|Get(acopy) (Variables|Default|GetUnitsInCombat) (LocalVariables|GetCurrentIndex)))
          (LocalVariables|SetNextLivingUnit (Utilities|Array|Get(acopy) (Variables|Default|GetUnitsInCombat) (LocalVariables|GetCurrentIndex)))))
      (bind _output_get_2 (Variables|Default|SetCurrentUnit (LocalVariables|GetNextLivingUnit)))
      (Default|TurnStarted _output_get_2)
      (Default|CallOnUnitTurnStarted _output_get_2))))

(fn MoveUnit
  (params (Unit :type BP%20Unit%20Object%20Reference) (Path :type Array%20of%20Int%20Point%20Structures))
  (if (> (Utilities|Array|Length Path) 0)
    (Default|EventFollowPath Unit Path)
    (bind _cost (Default|GetPathCost (Variables|/Game/Blueprints/Core/Grid/BP_Grid.BP_Grid_C|GetGridPathfinding (Variables|Default|GetGrid)) Path))
    (Default|ModifyCurrentMovement Unit (- 0 _cost) false)
    (Units|SetUnitIndexonGrid Unit (Utilities|Array|Get(acopy) Path (Utilities|Array|LastIndex Path)) false false)))

(fn ProcessUnitDeath
  (params (Unit :type BP%20Unit%20Object%20Reference))
  (bind _teamswithatleastoneunitalive (LocalVariables|GetTeamsWithAtLeastOneUnitAlive))
  (if (Variables|Default|GetIsInCombat)
    (Variables|/Game/Blueprints/Core/Units/BP_Unit.BP_Unit_C|SetIndexToRememberForSpellImpact Unit (Variables|/Game/Blueprints/Core/Units/BP_Unit.BP_Unit_C|GetIndex Unit))
    (Units|SetUnitIndexonGrid Unit (Utilities|Struct|MakeIntPoint -999 -999) false false)
    (Default|EventHideUnitAfterFewSeconds Unit)
    (bind _keys (Utilities|Map|Keys (Variables|Default|GetUnitTeams)))
    (for _array_element _keys
      (bind _output_get (LocalVariables|SetTeamIndex _array_element))
      (bind _result (Utilities|Set|ToArray (Utilities|Struct|BreakS_UnitSet (.Value (Utilities|Map|Find (Variables|Default|GetUnitTeams) _output_get)))))
      (bind _array_element_2 (Utilities|Array|ForEachLoopwithBreak _result :!label _label)
        (:LoopBody
          (if (Default|IsAlive _array_element_2)
            (Utilities|Array|Add (LocalVariables|GetTeamsWithAtLeastOneUnitAlive) (LocalVariables|GetTeamIndex))
            (goto _label Break)))))
    (if (== (Utilities|Array|Length _teamswithatleastoneunitalive) 1) ; Only 1 team left alive?
      (CallFunction|FinishCombat (Utilities|Array|Get(acopy) _teamswithatleastoneunitalive)))
    (else
      (Default|DebugRespawnAfterFewSeconds Unit))))

(fn FinishCombat
  (params (WinningTeam :type Integer))
  (Variables|Default|SetIsFinishingCombat true)
  (Default|CallOnCombatFinishing WinningTeam))