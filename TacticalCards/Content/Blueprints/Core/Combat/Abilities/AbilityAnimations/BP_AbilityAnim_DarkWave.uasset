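; Ability animation actor that plays the Dark Wave visual effect on a target tile during combat.
; When triggered, it moves to the target tile, then a timeline scales the AnimScale component and drives the Opacity material parameter on three static meshes.
; When the timeline finishes, it calls the ability animation completed event.
; Construction script nodes that would set the mesh color to black are left unconnected.
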(event EventBeginPlay
  (|CallParentFunction) ; This node is disabled and will not be called.\nDrag off pins to build functionality.
)

(event Collision|EventActorBeginOverlap
  (params (OtherActor :type Actor%20Object%20Reference)))

(event EventTick
  (params (DeltaSeconds :type Float%20%28single-precision%29)))

(event EventEventPlayAbilityAnimation
  (Transformation|SetActorLocation (.location (CallFunction|GetTileTransform (Variables|Default|GetTargetIndex))) false false)
  (bind (_direction _opacity _scale) (Timeline|Timeline PlayFromStart)
    (:Update
      (Transformation|SetRelativeScale3D (Variables|Default|GetAnim_Scale) _scale)
      (Rendering|Material|SetScalarParameterValueonMaterials (Variables|Default|GetStaticMesh) "Opacity" _opacity))
    (:Finished
      (CallFunction|EventCompletedAbilityAnimation))))

(fn ConstructionScript
  (|CallParentFunction))