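; Ability animation actor for a long-range arrow that visually flies from an origin tile to a target tile.
; On the play event it moves to the origin and yaws toward the target using the two tile indices as 2D coordinates.
; A timeline lerps its location between the tile transforms with an added height curve, while animating pitch and scale on a child component.
; When the timeline finishes, it fires the ability animation completed event.
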(event EventBeginPlay
  (|CallParentFunction) ; This node is disabled and will not be called.\nDrag off pins to build functionality.
)

(event Collision|EventActorBeginOverlap
  (params (OtherActor :type Actor%20Object%20Reference)))

(event EventTick
  (params (DeltaSeconds :type Float%20%28single-precision%29)))

(event EventEventPlayAbilityAnimation
  (bind _originindex (Variables|Default|GetOriginIndex))
  (bind _anim_rotationscale (Variables|Default|GetAnim_RotationScale))
  (Transformation|SetActorLocationAndRotation (.location (CallFunction|GetTileTransform _originindex)) (Math|Rotator|FindLookatRotation (Math|Conversions|ToVector(Vector2D) (Math|Conversions|ToVector2D(IntPoint) _originindex)) (Math|Conversions|ToVector(Vector2D) (Math|Conversions|ToVector2D(IntPoint) (Variables|Default|GetTargetIndex)))))
  (bind (_direction _locationalpha _locationz _rotationy _scale) (Timeline|Timeline Play)
    (:Update
      (Transformation|SetActorLocation (+ (Math|Vector|Lerp(Vector) (.location (CallFunction|GetTileTransform (Variables|Default|GetOriginIndex))) (.location (CallFunction|GetTileTransform (Variables|Default|GetTargetIndex))) _locationalpha) (Math|Vector|MakeVector 0.0 0.0 _locationz)) false false)
      (Transformation|SetRelativeRotation _anim_rotationscale (Math|Rotator|MakeRotator 0.0 _rotationy 0.0) false false)
      (Transformation|SetRelativeScale3D _anim_rotationscale (Math|Conversions|ToVector(Float) _scale)))
    (:Finished
      (CallFunction|EventCompletedAbilityAnimation))))

(fn ConstructionScript
  (|CallParentFunction))