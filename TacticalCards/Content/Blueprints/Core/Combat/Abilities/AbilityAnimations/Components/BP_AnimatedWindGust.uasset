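; Animated wind gust visual for combat abilities, a short-lived actor that moves from an origin transform to a target transform.
; On BeginPlay a timeline, scaled by PlayRate, drives the transform lerp and material opacity.
; It fires OnShapeAnimationCompleted once partway through playback, then destroys itself shortly after the timeline finishes.
; The construction script gives both material slots translucent dynamic materials in randomly brightened or darkened greens.
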(event EventBeginPlay
  (Components|Timeline|SetPlayRate (Variables|Default|GetTimeline_PlayAnimation) (Variables|Default|GetPlayRate))
  (bind (_direction _transformalpha _opacity) (Timeline|Timeline_PlayAnimation PlayFromStart)
    (:Update
      (Transformation|SetActorTransform (Math|Transform|Lerp(Transform) (Variables|Default|GetOriginTransform) (Variables|Default|GetTargetTransform) _transformalpha))
      (Rendering|Material|SetScalarParameterValueonMaterials (Variables|Default|GetAnimatedWindGust) "Opacity" _opacity)
      (if (>= (Components|Timeline|GetPlaybackPosition (Variables|Default|GetTimeline_PlayAnimation)) 0.35)
        (Utilities|FlowControl|DoOnce false
          (:Completed
            (Default|CallOnShapeAnimationCompleted self)))))
    (:Finished
      (Utilities|FlowControl|Delay 0.5)
      (Actor|DestroyActor))))

(fn ConstructionScript
  (bind _returnvalue (Rendering|Material|CreateDynamicMaterialInstance (Variables|Default|GetAnimatedWindGust) 0 "/Game/Assets/Materials/M_TranslucentColor.M_TranslucentColor" "None" :!class /Script/Engine.PrimitiveComponent))
  (Rendering|Material|SetVectorParameterValue _returnvalue "Color" (* "(R=0.164317,G=0.539930,B=0.115298,A=1.000000)" (Math|Random|RandomFloatinRange 0.0 1.5)) :!class /Script/Engine.MaterialInstanceDynamic)
  (bind _returnvalue_2 (Rendering|Material|CreateDynamicMaterialInstance (Variables|Default|GetAnimatedWindGust) 1 "/Game/Assets/Materials/M_TranslucentColor.M_TranslucentColor" "None" :!class /Script/Engine.PrimitiveComponent))
  (Rendering|Material|SetVectorParameterValue _returnvalue_2 "Color" (* "(R=0.305016,G=0.689236,B=0.254874,A=1.000000)" (Math|Random|RandomFloatinRange 0.0 1.5)) :!class /Script/Engine.MaterialInstanceDynamic))