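; Ability animation actor for Run Chicken Run, showing the ability's icon on a widget component at the target tile.
; It moves to the target tile, then a timeline animates the widget's height, draw size and opacity.
; A DoOnce fires the tile-hit callback partway through playback, and the timeline's end completes the ability animation.
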(event EventEventPlayAbilityAnimation
  (bind _widget (Variables|Default|GetWidget))
  (Transformation|SetActorLocation (.location (CallFunction|GetTileTransform (Variables|Default|GetTargetIndex))) false false)
  (bind _asw_image (Utilities|Casting|CastToW_Image (UserInterface|GetUserWidgetObject (Variables|Default|GetWidget))))
  (bind _output_get (Variables|Default|SetW_Image _asw_image))
  (Appearance|SetBrushfromTexture (Variables|/Game/Blueprints/Core/Combat/Abilities/AbilityAnimations/Components/W_Image.W_Image_C|GetImage_Component _output_get) "/Game/Blueprints/Core/Combat/Abilities/AbilityAnimations/Assets/Icon_RunChickenRun_NoBackground.Icon_RunChickenRun_NoBackground" false)
  (bind (_direction _locationz _drawsize _opacity) (Timeline|Timeline_RunChickenRun PlayFromStart)
    (:Update
      (Transformation|SetRelativeLocation _widget (Math|Vector|MakeVector 0.0 0.0 _locationz) false false)
      (Class|WidgetComponent|SetDrawSize _widget (Math|Vector2D|MakeVector2D _drawsize _drawsize))
      (Widget|SetRenderOpacity (Variables|Default|GetW_Image) _opacity)
      (if (>= (Components|Timeline|GetPlaybackPosition (Variables|Default|GetTimeline_RunChickenRun)) 0.2)
        (Utilities|FlowControl|DoOnce false
          (:Completed
            (Default|CallOnAbilityAnimationHitTile self (Variables|Default|GetTargetIndex))))))
    (:Finished
      (CallFunction|EventCompletedAbilityAnimation))))

(fn ConstructionScript
  (|CallParentFunction))