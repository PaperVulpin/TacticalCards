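; Placed scenario actor that quick-starts a tactical combat on BeginPlay and opens the main menu when that combat ends.
; In the editor, its construction script centers and spawns the grid, then maps units to tiles from their locations.
; Separate helpers fill the unit data by parsing team numbers from unit display names and marking all but the first team as AI-controlled.
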(event Custom|OnCombatEnded
  (if (== self (Variables|/Game/TacticalCards/Blueprints/Core/Combat/BP_CombatSystem.BP_CombatSystem_C|GetObjectThatStartedCombat (Variables|Default|GetCombatSystem)))
    (Game|OpenLevel(byName) "L_MainMenu")))

(event EventBeginPlay
  (EventDispatchers|BindEventtoOnCombatEnded (Variables|Default|GetCombatSystem) (delegate Custom|OnCombatEnded))
  (Default|QuickStartCombat (Variables|Default|GetCombatSystem) (Variables|Default|GetGridData) (Variables|Default|GetUnitsData) self))

(fn ConstructionScript
  (if (not (CallFunction|IsinGame))
    (Utilities|Struct|SetmembersinS_QuickCombat_Grid (Variables|Default|GetGridData) (Transformation|GetActorLocation))
    (CallFunction|SpawnGrid)
    (CallFunction|BuildDesiredGridIndexesBasedonUnitLocations)))

(fn BuildsTeamsBasedonUnitNames
  (bind _outactors (Actor|GetAllActorsOfClass "/Game/TacticalCards/Blueprints/Core/Units/BP_Unit.BP_Unit_C"))
  (for _array_element _outactors
    (bind _output_get (LocalVariables|SetUnit _array_element))
    (LocalVariables|SetTeam%20Index (Math|Conversions|ToInteger(Byte) (.LeftS (Utilities|String|Split (.RightS (Utilities|String|Split (Utilities|GetDisplayName _output_get) "Team")) "_"))))
    (if (< (Utilities|Array|Length (LocalVariables|GetUnitsTeams)) (+ (LocalVariables|GetTeam%20Index) 1)) ; Is array too small?
      (Utilities|Array|Resize (LocalVariables|GetUnitsTeams) (+ (LocalVariables|GetTeam%20Index) 1)))
    (Utilities|Array|Add (Utilities|Struct|BreakS_UnitArray (Utilities|Array|Get(acopy) (LocalVariables|GetUnitsTeams) (LocalVariables|GetTeam%20Index))) (LocalVariables|GetUnit)))
  (Utilities|Array|RemoveItem :TargetArray (LocalVariables|GetUnitsTeams)) ; Remove empty groups
  (Utilities|Struct|SetmembersinS_QuickCombat_UnitTeams (Variables|Default|GetUnitsData) (LocalVariables|GetUnitsTeams)))

(fn BuildAIListBasedonTeamIndexes
  (for (_array_element _array_index) (Utilities|Struct|BreakS_QuickCombat_UnitTeams (Variables|Default|GetUnitsData))
    (if (!= _array_index 0)
      (Utilities|Array|AppendArray (LocalVariables|GetAIs) (Utilities|Struct|BreakS_UnitArray _array_element))))
  (Utilities|Struct|SetmembersinS_QuickCombat_UnitTeams (Variables|Default|GetUnitsData) (LocalVariables|GetAIs)))

(fn BuildDesiredGridIndexesBasedonUnitLocations
  (for _array_element (Utilities|Struct|BreakS_QuickCombat_UnitTeams (Variables|Default|GetUnitsData))
    (for _array_element_2 (Utilities|Struct|BreakS_UnitArray _array_element)
      (bind _index (Default|GetTileIndexfromWorldLocation (Variables|/Game/TacticalCards/Blueprints/Core/Combat/BP_CombatSystem.BP_CombatSystem_C|GetGrid (Variables|Default|GetCombatSystem)) (Transformation|GetActorLocation _array_element_2)))
      (Utilities|Map|Add (LocalVariables|GetDesiredIndexes) _array_element_2 _index)))
  (Utilities|Struct|SetmembersinS_QuickCombat_UnitTeams (Variables|Default|GetUnitsData) (LocalVariables|GetDesiredIndexes)))

(fn SpawnGrid
  (bind _combatsystem (Variables|Default|GetCombatSystem))
  (bind _griddata (Variables|Default|GetGridData))
  (bind (_centerlocation _tilesize _tilecount _shape _useenvironment) (Utilities|Struct|BreakS_QuickCombat_Grid _griddata))
  (bind _grid (Variables|/Game/TacticalCards/Blueprints/Core/Combat/BP_CombatSystem.BP_CombatSystem_C|GetGrid _combatsystem))
  (Utilities|IsValid _combatsystem
    (:Is%20Valid
      (Utilities|IsValid _grid
        (:Is%20Valid
          (Default|SpawnGrid _grid _centerlocation _tilesize _tilecount _shape _useenvironment))))))