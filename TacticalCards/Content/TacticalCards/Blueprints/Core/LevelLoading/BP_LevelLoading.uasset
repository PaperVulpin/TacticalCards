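; Level-loading Blueprint that keeps track of one active streaming sublevel and swaps it on request.
; LoadLevel unloads and hides the current sublevel, then loads and shows the named one, skipping repeat requests unless forced.
; BeginPlay force-loads whatever level name is already stored.
; An invalid name other than "None" prints an error.
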(event EventBeginPlay
  (CallFunction|LoadLevel (Variables|Default|GetLevelLoaded) true))

(event Collision|EventActorBeginOverlap
  (params (OtherActor :type Actor%20Object%20Reference)))

(event EventTick
  (params (DeltaSeconds :type Float%20%28single-precision%29)))

(fn ConstructionScript)

(fn LoadLevel
  (params (Level :type String) (Force :type Boolean))
  (bind _returnvalue (Utilities|String|StringToName Level))
  (bind _returnvalue_2 (Class|GameplayStatics|GetStreamingLevel _returnvalue))
  (if (or (Utilities|Enum|NotEqual(Enum) Level (Variables|Default|GetLevelLoaded)) Force)
    (Utilities|FlowControl|Sequence
      (:then_0
        (Utilities|IsValid (Class|GameplayStatics|GetStreamingLevel (Utilities|String|StringToName (Variables|Default|GetLevelLoaded)))
          (:Is%20Valid
            (Variables|/Script/Engine.LevelStreaming|SetbShouldBeLoaded (Class|GameplayStatics|GetStreamingLevel (Utilities|String|StringToName (Variables|Default|GetLevelLoaded))) false)
            (Variables|/Script/Engine.LevelStreaming|SetbShouldBeVisible (Class|GameplayStatics|GetStreamingLevel (Utilities|String|StringToName (Variables|Default|GetLevelLoaded))) false))))
      (:then_1
        (bind _output_get (Variables|Default|SetLevelLoaded Level))
        (Utilities|IsValid _returnvalue_2
          (:Is%20Valid
            (Variables|/Script/Engine.LevelStreaming|SetbShouldBeLoaded _returnvalue_2 true)
            (Variables|/Script/Engine.LevelStreaming|SetbShouldBeVisible _returnvalue_2 true))
          (:Is%20Not%20Valid
            (if (Utilities|Enum|NotEqual(Enum) _output_get "None")
              (Development|PrintString (Utilities|String|Append "Error: LoadLevel - Invalid Level Name: " _output_get)))))))))