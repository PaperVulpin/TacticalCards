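; Player action that adds or removes units on the overworld map, depending on the IsAddingUnit flag.
; Adding traces under the cursor, spawns a quarter-scale BP_Unit of the set type, and snaps it onto the navmesh with a capsule-height offset.
; The new unit gets its context set and joins the given group through the OverworldUnitGroupsManager.
; Removing simply destroys the currently hovered unit.
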(event EventBeginPlay
  (|CallParentFunction) ; This node is disabled and will not be called.\nDrag off pins to build functionality.
)

(event Collision|EventActorBeginOverlap
  (params (OtherActor :type Actor%20Object%20Reference))
  (|CallParentFunction OtherActor) ; This node is disabled and will not be called.\nDrag off pins to build functionality.
)

(event EventTick
  (params (DeltaSeconds :type Float%20%28single-precision%29))
  (|CallParentFunction DeltaSeconds) ; This node is disabled and will not be called.\nDrag off pins to build functionality.
)

(fn ConstructionScript
  (|CallParentFunction))

(fn ExecuteAction
  (params (Index :type Int%20Point%20Structure))
  (bind _returnvalue (Game|GetPlayerController 0))
  (bind _playeractions (Variables|Default|GetPlayerActions))
  (bind (_hitresult _returnvalue_2) (Game|Player|GetHitResultUnderCursorbyChannel _returnvalue "TraceTypeQuery3" false))
  (bind _hoveredunit (Variables|/Game/TacticalCards/Blueprints/Core/Player/BP_PlayerActions.BP_PlayerActions_C|GetHoveredUnit _playeractions))
  (if (Variables|Default|GetIsAddingUnit)
    (if _returnvalue_2
      (LocalVariables|SetHitLocation (.Location (Collision|BreakHitResult _hitresult)))
      (bind _returnvalue_3 (Game|SpawnActorfromClass "/Game/TacticalCards/Blueprints/Core/Units/BP_Unit.BP_Unit_C" (Math|Transform|MakeTransform "0, 0, 0" "0, 0, 0" "0.250000,0.250000,0.250000") "AlwaysSpawn" "MultiplyWithRoot" 0 (Variables|Default|GetUnitType) 0))
      (bind _output_get (LocalVariables|SetUnit _returnvalue_3))
      (Transformation|SetActorLocation _output_get (Default|AddCapsuleHeight _output_get (.ProjectedLocation (AI|Navigation|ProjectPointtoNavigation (LocalVariables|GetHitLocation) (Variables|/Game/TacticalCards/Blueprints/Core/Units/BP_Unit.BP_Unit_C|GetNavData _output_get) 0 "50.000000,50.000000,9999.000000"))) false false)
      (Default|SetUnitContext _output_get "NewEnumerator1")
      (Default|AddUnittoGroup (Variables|/Game/TacticalCards/Blueprints/Core/Player/BP_PlayerActions.BP_PlayerActions_C|GetOverworldUnitGroupsManager (Variables|Default|GetPlayerActions)) _output_get (Variables|Default|GetGroupID)))
    (else
      (Utilities|IsValid _hoveredunit
        (:Is%20Valid
          (Actor|DestroyActor _hoveredunit))))))