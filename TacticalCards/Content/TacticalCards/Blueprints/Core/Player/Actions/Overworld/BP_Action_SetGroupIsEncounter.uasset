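; Overworld player action that sets whether the hovered unit's group is an encounter.
; When executed, it checks that the PlayerActions hovered unit is valid, then passes that unit's OverworldGroupID and the action's IsEncounter value to SetGroupIsEncounter on the OverworldUnitGroupsManager.
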(event EventBeginPlay
  (|CallParentFunction) ; This node is disabled and will not be called.\nDrag off pins to build functionality.
)

(event Collision|EventActorBeginOverlap
  (params (OtherActor :type Actor%20Object%20Reference))
  (|CallParentFunction OtherActor) ; This node is disabled and will not be called.\nDrag off pins to build functionality.
)

(event EventTick
  (params (DeltaSeconds :type Float%20%28single-precision%29))
  (|CallParentFunction DeltaSeconds) ; This node is disabled and will not be called.\nDrag off pins to build functionality.
)

(fn ConstructionScript
  (|CallParentFunction))

(fn ExecuteAction
  (params (Index :type Int%20Point%20Structure))
  (bind _playeractions (Variables|Default|GetPlayerActions))
  (bind _hoveredunit (Variables|/Game/TacticalCards/Blueprints/Core/Player/BP_PlayerActions.BP_PlayerActions_C|GetHoveredUnit _playeractions))
  (Utilities|IsValid _hoveredunit
    (:Is%20Valid
      (Default|SetGroupIsEncounter (Variables|/Game/TacticalCards/Blueprints/Core/Player/BP_PlayerActions.BP_PlayerActions_C|GetOverworldUnitGroupsManager (Variables|Default|GetPlayerActions)) (Variables|Default|GetIsEncounter) (Variables|/Game/TacticalCards/Blueprints/Core/Units/BP_Unit.BP_Unit_C|GetOverworldGroupID _hoveredunit)))))