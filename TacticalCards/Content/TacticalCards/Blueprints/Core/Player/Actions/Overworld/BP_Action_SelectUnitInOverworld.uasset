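; Player action for the overworld that selects the unit currently under the cursor.
; On execute, it looks up the hovered unit's group in the overworld unit groups manager and selects the unit only if that group is not an encounter.
; With no hovered unit it clears the selection using a sentinel tile index, and it does the same when the action ends play.
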(event EventBeginPlay
  (|CallParentFunction) ; This node is disabled and will not be called.\nDrag off pins to build functionality.
)

(event Collision|EventActorBeginOverlap
  (params (OtherActor :type Actor%20Object%20Reference))
  (|CallParentFunction OtherActor) ; This node is disabled and will not be called.\nDrag off pins to build functionality.
)

(event EventTick
  (params (DeltaSeconds :type Float%20%28single-precision%29))
  (|CallParentFunction DeltaSeconds) ; This node is disabled and will not be called.\nDrag off pins to build functionality.
)

(event EventEndPlay
  (params (EndPlayReason :type EEndPlayReason%20Enum :default "Destroyed"))
  (|CallParentFunction EndPlayReason)
  (Default|SetSelectedTileandUnit (Variables|Default|GetPlayerActions) (Utilities|Struct|MakeIntPoint -999 -999) 0 false))

(fn ConstructionScript
  (|CallParentFunction))

(fn ExecuteAction
  (params (Index :type Int%20Point%20Structure))
  (bind _playeractions (Variables|Default|GetPlayerActions))
  (bind _playeractions_2 (Variables|Default|GetPlayerActions))
  (bind _playeractions_3 (Variables|Default|GetPlayerActions))
  (Utilities|IsValid (Variables|/Game/TacticalCards/Blueprints/Core/Player/BP_PlayerActions.BP_PlayerActions_C|GetHoveredUnit _playeractions_3)
    (:Is%20Valid
      (if (not (Utilities|Struct|BreakS_OverworldUnitGroup (.Value (Utilities|Map|Find (Variables|/Game/TacticalCards/Blueprints/Core/Units/OverworldUnitGroups/BP_OverworldUnitGroupsManager.BP_OverworldUnitGroupsManager_C|GetUnitGroups (Variables|/Game/TacticalCards/Blueprints/Core/Player/BP_PlayerActions.BP_PlayerActions_C|GetOverworldUnitGroupsManager _playeractions_2)) (Variables|/Game/TacticalCards/Blueprints/Core/Units/BP_Unit.BP_Unit_C|GetOverworldGroupID (Variables|/Game/TacticalCards/Blueprints/Core/Player/BP_PlayerActions.BP_PlayerActions_C|GetHoveredUnit _playeractions_2))))))
        (Default|SetSelectedTileandUnit :self _playeractions :Unit (Variables|/Game/TacticalCards/Blueprints/Core/Player/BP_PlayerActions.BP_PlayerActions_C|GetHoveredUnit _playeractions))))
    (:Is%20Not%20Valid
      (Default|SetSelectedTileandUnit _playeractions_3 (Utilities|Struct|MakeIntPoint -999 -999) 0 false))))