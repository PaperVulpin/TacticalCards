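; BP_Action_SetTileType is a player action that changes the type of a grid tile in a tactical grid game.
; On execution it checks that the index is valid, looks up that tile's data in the grid's tile map, and re-adds the tile with its TileType variable.
; The tile's index, transform, states and occupying unit are carried over unchanged.
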(fn ConstructionScript
  (|CallParentFunction))

(fn ExecuteAction
  (params (Index :type Int%20Point%20Structure))
  (bind _playeractions (Variables|Default|GetPlayerActions))
  (bind _grid (Variables|/Game/TacticalCards/Blueprints/Core/Player/BP_PlayerActions.BP_PlayerActions_C|GetGrid _playeractions))
  (if (Default|IsIndexValid _grid Index)
    (bind _output_get (LocalVariables|SetData (.Value (Utilities|Map|Find (Variables|/Game/TacticalCards/Blueprints/Core/Grid/BP_Grid.BP_Grid_C|GetGridTiles _grid) Index))))
    (Default|AddGridTile _grid (Utilities|Struct|MakeS_TileData (.index _output_get) (Variables|Default|GetTileType) (.transform _output_get) (.states _output_get) (.unitontile _output_get)))))