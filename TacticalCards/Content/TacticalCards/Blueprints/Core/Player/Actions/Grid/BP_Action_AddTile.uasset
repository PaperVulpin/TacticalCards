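; Player grid action that adds a tile to the tactical grid at a given index.
; ExecuteAction runs only when that index is not already valid on the grid.
; It traces for ground at the index's location, then registers a tile of a fixed type at the traced point, using the grid's rotation for that index and its tile scale.
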(fn ConstructionScript
  (|CallParentFunction))

(fn ExecuteAction
  (params (Index :type Int%20Point%20Structure))
  (bind _playeractions (Variables|Default|GetPlayerActions))
  (bind _grid (Variables|/Game/TacticalCards/Blueprints/Core/Player/BP_PlayerActions.BP_PlayerActions_C|GetGrid _playeractions))
  (if (not (Default|IsIndexValid _grid Index))
    (bind _outlocation (Default|TraceforGround _grid (Default|GetTileLocationfromGridIndex _grid Index)))
    (Default|AddGridTile _grid (Utilities|Struct|MakeS_TileData Index "NewEnumerator1" (Math|Transform|MakeTransform _outlocation (Default|GetTileRotationfromGridIndex _grid Index) (Default|GetTileScale _grid)) "NewEnumerator0" 0))))