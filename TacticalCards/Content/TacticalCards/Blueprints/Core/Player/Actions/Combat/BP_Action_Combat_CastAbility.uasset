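; Combat player action that previews and casts a selected ability on the tile grid.
; SetAbility loads the ability's cast and AoE data and highlights tiles in range of the selected tile via the CombatSystem.
; Hovering an in-range tile redraws the AoE pattern, or just that tile if none exists.
; Executing casts through the CombatSystem and resets the combat widget's selection; EndPlay clears both highlights.
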(event EventBeginPlay
  (|CallParentFunction) ; This node is disabled and will not be called.\nDrag off pins to build functionality.
)

(event Collision|EventActorBeginOverlap
  (params (OtherActor :type Actor%20Object%20Reference))
  (|CallParentFunction OtherActor) ; This node is disabled and will not be called.\nDrag off pins to build functionality.
)

(event EventTick
  (params (DeltaSeconds :type Float%20%28single-precision%29))
  (|CallParentFunction DeltaSeconds) ; This node is disabled and will not be called.\nDrag off pins to build functionality.
)

(event EventEndPlay
  (params (EndPlayReason :type EEndPlayReason%20Enum :default "Destroyed"))
  (bind _playeractions (Variables|Default|GetPlayerActions))
  (bind _grid (Variables|/Game/TacticalCards/Blueprints/Core/Player/BP_PlayerActions.BP_PlayerActions_C|GetGrid _playeractions))
  (|CallParentFunction EndPlayReason)
  (Default|ClearStatesfromTiles _grid "NewEnumerator8")
  (Default|ClearStatesfromTiles _grid "NewEnumerator9"))

(fn ConstructionScript
  (|CallParentFunction))

(fn SetAbility
  (params (Ability :type E_Ability%20Enum :default "NewEnumerator0"))
  (bind _playeractions (Variables|Default|GetPlayerActions))
  (bind _grid (Variables|/Game/TacticalCards/Blueprints/Core/Player/BP_PlayerActions.BP_PlayerActions_C|GetGrid _playeractions))
  (bind _output_get (Variables|Default|SetAbility Ability))
  (if (Utilities|Enum|NotEqual(Enum) _output_get "NewEnumerator0")
    (bind _abilitydata (CallFunction|GetAbilityDatafromAbility (Variables|Default|GetAbility)))
    (Variables|Default|SetCast (.cast _abilitydata))
    (Variables|Default|SetCastAOE (.castaoe _abilitydata))
    (CallFunction|ShowAbilityRangePattern)
    (else
      (Default|ClearStatesfromTiles _grid "NewEnumerator8")
      (Default|ClearStatesfromTiles _grid "NewEnumerator9"))))

(fn ShowAbilityRangePattern
  (bind _playeractions (Variables|Default|GetPlayerActions))
  (Utilities|FlowControl|Sequence
    (:then_0
      (Default|ClearStatesfromTiles (Variables|/Game/TacticalCards/Blueprints/Core/Player/BP_PlayerActions.BP_PlayerActions_C|GetGrid (Variables|Default|GetPlayerActions)) "NewEnumerator8")
      (bind _rangeindexes (Default|GetAbilityRange (Variables|/Game/TacticalCards/Blueprints/Core/Player/BP_PlayerActions.BP_PlayerActions_C|GetCombatSystem _playeractions) (Variables|/Game/TacticalCards/Blueprints/Core/Player/BP_PlayerActions.BP_PlayerActions_C|GetSelectedTile _playeractions) (Variables|Default|GetCast)))
      (for _array_element _rangeindexes
        (Default|AddStatetoTile (Variables|/Game/TacticalCards/Blueprints/Core/Player/BP_PlayerActions.BP_PlayerActions_C|GetGrid (Variables|Default|GetPlayerActions)) _array_element "NewEnumerator8")))
    (:then_1
      (CallFunction|ShowAbilityRangeAOEPattern))))

(fn ExecuteAction
  (params (Index :type Int%20Point%20Structure))
  (bind _playeractions (Variables|Default|GetPlayerActions))
  (bind _playeractions_2 (Variables|Default|GetPlayerActions))
  (bind _w_combat (Variables|/Game/TacticalCards/Blueprints/Core/Player/BP_PlayerActions.BP_PlayerActions_C|GetW_Combat _playeractions))
  (|CallParentFunction Index)
  (Default|CastAbility (Variables|/Game/TacticalCards/Blueprints/Core/Player/BP_PlayerActions.BP_PlayerActions_C|GetCombatSystem _playeractions_2) (Variables|Default|GetAbility) (Variables|/Game/TacticalCards/Blueprints/Core/Player/BP_PlayerActions.BP_PlayerActions_C|GetSelectedTile _playeractions_2) Index)
  (Utilities|IsValid _w_combat ; Widget is destroyed during FinishingCombat phase
    (:Is%20Valid
      (Default|SetSelectedAbilityfromIndex (Variables|/Game/TacticalCards/Blueprints/Core/Combat/Widgets/WBP_Combat.WBP_Combat_C|GetButtonList_Abilities _w_combat) -1))))

(fn ShowAbilityRangeAOEPattern
  (bind _playeractions (Variables|Default|GetPlayerActions))
  (bind _playeractions_2 (Variables|Default|GetPlayerActions))
  (bind _playeractions_3 (Variables|Default|GetPlayerActions))
  (bind _grid (Variables|/Game/TacticalCards/Blueprints/Core/Player/BP_PlayerActions.BP_PlayerActions_C|GetGrid _playeractions_3))
  (Default|ClearStatesfromTiles _grid "NewEnumerator9")
  (if (Utilities|Array|ContainsItem (Utilities|Struct|BreakS_IntPointArray (.Value (Utilities|Map|Find (Variables|/Game/TacticalCards/Blueprints/Core/Grid/BP_Grid.BP_Grid_C|GetTileStateToIndexes _grid) "NewEnumerator8"))) (Variables|/Game/TacticalCards/Blueprints/Core/Player/BP_PlayerActions.BP_PlayerActions_C|GetHoveredTile _playeractions_3))
    (if (Utilities|Enum|NotEqual(Enum) (.RangePattern (Utilities|Struct|BreakS_AbilityData_Cast (Variables|Default|GetCastAOE))) "NewEnumerator0")
      (bind _rangeindexes (Default|GetAbilityRange (Variables|/Game/TacticalCards/Blueprints/Core/Player/BP_PlayerActions.BP_PlayerActions_C|GetCombatSystem _playeractions) (Variables|/Game/TacticalCards/Blueprints/Core/Player/BP_PlayerActions.BP_PlayerActions_C|GetHoveredTile _playeractions) (Variables|Default|GetCastAOE)))
      (for _array_element _rangeindexes
        (Default|AddStatetoTile (Variables|/Game/TacticalCards/Blueprints/Core/Player/BP_PlayerActions.BP_PlayerActions_C|GetGrid (Variables|Default|GetPlayerActions)) _array_element "NewEnumerator9"))
      (else
        (Default|AddStatetoTile (Variables|/Game/TacticalCards/Blueprints/Core/Player/BP_PlayerActions.BP_PlayerActions_C|GetGrid _playeractions_2) (Variables|/Game/TacticalCards/Blueprints/Core/Player/BP_PlayerActions.BP_PlayerActions_C|GetHoveredTile _playeractions_2) "NewEnumerator9")))))

(fn ExecuteHoveredAction
  (params (Index :type Int%20Point%20Structure))
  (|CallParentFunction Index)
  (CallFunction|ShowAbilityRangeAOEPattern))