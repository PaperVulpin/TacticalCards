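; Player combat action, used while waiting for a turn, that highlights the movement range of the hovered unit, falling back to the selected unit.
; When that unit changes, it clears the tile highlight state and runs the grid's time-sliced reachables pathfinding with the unit's movement stats.
; The completion callback applies the state to each reachable tile, and EndPlay clears it.
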(event EventBeginPlay
  (|CallParentFunction)
  (EventDispatchers|BindEventtoOnPathfindingCompleted (Variables|/Game/TacticalCards/Blueprints/Core/Grid/BP_Grid.BP_Grid_C|GetGridPathfinding_Reachables (Variables|/Game/TacticalCards/Blueprints/Core/Player/BP_PlayerActions.BP_PlayerActions_C|GetGrid (Variables|Default|GetPlayerActions))) (EventDispatchers|CreateEvent :!event OnPathfindingCompletedReachables)))

(event EventEndPlay
  (params (EndPlayReason :type EEndPlayReason%20Enum :default "Destroyed"))
  (|CallParentFunction EndPlayReason)
  (Default|ClearStatesfromTiles (Variables|/Game/TacticalCards/Blueprints/Core/Player/BP_PlayerActions.BP_PlayerActions_C|GetGrid (Variables|Default|GetPlayerActions)) "NewEnumerator7"))

(fn ConstructionScript
  (|CallParentFunction))

(fn GenerateReachables
  (params (Unit :type BP%20Unit%20Object%20Reference))
  (if (!= Unit (Variables|Default|GetCurrentUnitForReachables))
    (Variables|Default|SetCurrentUnitForReachables Unit)
    (Default|ClearStatesfromTiles (Variables|/Game/TacticalCards/Blueprints/Core/Player/BP_PlayerActions.BP_PlayerActions_C|GetGrid (Variables|Default|GetPlayerActions)) "NewEnumerator7")
    (Utilities|IsValid (Variables|Default|GetCurrentUnitForReachables)
      (:Is%20Valid
        (Default|FindPath (Variables|/Game/TacticalCards/Blueprints/Core/Grid/BP_Grid.BP_Grid_C|GetGridPathfinding_Reachables (Variables|/Game/TacticalCards/Blueprints/Core/Player/BP_PlayerActions.BP_PlayerActions_C|GetGrid (Variables|Default|GetPlayerActions))) (Variables|/Game/TacticalCards/Blueprints/Core/Units/BP_Unit.BP_Unit_C|GetIndex (Variables|Default|GetCurrentUnitForReachables)) (Utilities|Struct|MakeIntPoint -999 -999) (.CanMoveDiagonally (Utilities|Struct|BreakS_UnitData_Stats (.Stats (Utilities|Struct|BreakS_UnitData (Variables|/Game/TacticalCards/Blueprints/Core/Units/BP_Unit.BP_Unit_C|GetUnitData (Variables|Default|GetCurrentUnitForReachables)))))) (.ValidTileTypes (Utilities|Struct|BreakS_UnitData_Stats (.Stats (Utilities|Struct|BreakS_UnitData (Variables|/Game/TacticalCards/Blueprints/Core/Units/BP_Unit.BP_Unit_C|GetUnitData (Variables|Default|GetCurrentUnitForReachables)))))) 0.1 15.0 true (.Movement_Current (Utilities|Struct|BreakS_UnitData_Stats (.Stats (Utilities|Struct|BreakS_UnitData (Variables|/Game/TacticalCards/Blueprints/Core/Units/BP_Unit.BP_Unit_C|GetUnitData (Variables|Default|GetCurrentUnitForReachables)))))))))))

(fn OnPathfindingCompletedReachables
  (params (Reachables :type Array%20of%20Int%20Point%20Structures))
  (for _array_element Reachables
    (Default|AddStatetoTile (Variables|/Game/TacticalCards/Blueprints/Core/Player/BP_PlayerActions.BP_PlayerActions_C|GetGrid (Variables|Default|GetPlayerActions)) _array_element "NewEnumerator7")))

(fn ExecuteHoveredAction
  (params (Index :type Int%20Point%20Structure))
  (bind _playeractions (Variables|Default|GetPlayerActions))
  (bind _hoveredunit (Variables|/Game/TacticalCards/Blueprints/Core/Player/BP_PlayerActions.BP_PlayerActions_C|GetHoveredUnit _playeractions))
  (|CallParentFunction Index)
  (Utilities|IsValid _hoveredunit
    (:Is%20Valid
      (Reachables|GenerateReachables _hoveredunit))
    (:Is%20Not%20Valid
      (Reachables|GenerateReachables (Variables|/Game/TacticalCards/Blueprints/Core/Player/BP_PlayerActions.BP_PlayerActions_C|GetSelectedUnit _playeractions)))))