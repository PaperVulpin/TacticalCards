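; Combat player action for moving the selected unit on the tactical grid, previewing reachable tiles and the path to the hovered tile.
; Two grid pathfinders run on the unit's movement stats, and their completion callbacks mark tile states for reachables and path.
; Hovering another unit shows its reachables instead, and executing sends the stored path to the CombatSystem.
; Reachables clear when walking starts, hover updates pause until it finishes, and both highlights clear on EndPlay.
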(event EventBeginPlay
  (bind _playeractions (Variables|Default|GetPlayerActions))
  (bind _selectedunit (Variables|/Game/TacticalCards/Blueprints/Core/Player/BP_PlayerActions.BP_PlayerActions_C|GetSelectedUnit _playeractions))
  (|CallParentFunction)
  (EventDispatchers|BindEventtoOnPathfindingCompleted (Variables|/Game/TacticalCards/Blueprints/Core/Grid/BP_Grid.BP_Grid_C|GetGridPathfinding_Reachables (Variables|/Game/TacticalCards/Blueprints/Core/Player/BP_PlayerActions.BP_PlayerActions_C|GetGrid (Variables|Default|GetPlayerActions))) (EventDispatchers|CreateEvent :!event OnPathfindingCompletedReachables))
  (EventDispatchers|BindEventtoOnPathfindingCompleted (Variables|/Game/TacticalCards/Blueprints/Core/Grid/BP_Grid.BP_Grid_C|GetGridPathfinding (Variables|/Game/TacticalCards/Blueprints/Core/Player/BP_PlayerActions.BP_PlayerActions_C|GetGrid (Variables|Default|GetPlayerActions))) (EventDispatchers|CreateEvent :!event OnPathfindingCompletedPath))
  (EventDispatchers|BindEventtoOnUnitStartedWalking _selectedunit (EventDispatchers|CreateEvent :!event OnUnitStartedWalking))
  (EventDispatchers|BindEventtoOnUnitFinishedWalking _selectedunit (EventDispatchers|CreateEvent :!event OnUnitFinishedWalking))
  (CallFunction|GenerateReachables (Variables|/Game/TacticalCards/Blueprints/Core/Player/BP_PlayerActions.BP_PlayerActions_C|GetSelectedUnit (Variables|Default|GetPlayerActions))))

(event Collision|EventActorBeginOverlap
  (params (OtherActor :type Actor%20Object%20Reference))
  (|CallParentFunction OtherActor) ; This node is disabled and will not be called.\nDrag off pins to build functionality.
)

(event EventTick
  (params (DeltaSeconds :type Float%20%28single-precision%29))
  (|CallParentFunction DeltaSeconds) ; This node is disabled and will not be called.\nDrag off pins to build functionality.
)

(event EventEndPlay
  (params (EndPlayReason :type EEndPlayReason%20Enum :default "Destroyed"))
  (bind _playeractions (Variables|Default|GetPlayerActions))
  (bind _grid (Variables|/Game/TacticalCards/Blueprints/Core/Player/BP_PlayerActions.BP_PlayerActions_C|GetGrid _playeractions))
  (|CallParentFunction EndPlayReason)
  (Default|ClearStatesfromTiles _grid "NewEnumerator7")
  (Default|ClearStatesfromTiles _grid "NewEnumerator4"))

(fn ConstructionScript
  (|CallParentFunction))

(fn GenerateReachables
  (params (Unit :type BP%20Unit%20Object%20Reference))
  (if (!= Unit (Variables|Default|GetCurrentUnitForReachables))
    (Variables|Default|SetCurrentUnitForReachables Unit)
    (Default|ClearStatesfromTiles (Variables|/Game/TacticalCards/Blueprints/Core/Player/BP_PlayerActions.BP_PlayerActions_C|GetGrid (Variables|Default|GetPlayerActions)) "NewEnumerator7")
    (Default|FindPath (Variables|/Game/TacticalCards/Blueprints/Core/Grid/BP_Grid.BP_Grid_C|GetGridPathfinding_Reachables (Variables|/Game/TacticalCards/Blueprints/Core/Player/BP_PlayerActions.BP_PlayerActions_C|GetGrid (Variables|Default|GetPlayerActions))) (Variables|/Game/TacticalCards/Blueprints/Core/Units/BP_Unit.BP_Unit_C|GetIndex (Variables|Default|GetCurrentUnitForReachables)) (Utilities|Struct|MakeIntPoint -999 -999) (.CanMoveDiagonally (Utilities|Struct|BreakS_UnitData_Stats (.Stats (Utilities|Struct|BreakS_UnitData (Variables|/Game/TacticalCards/Blueprints/Core/Units/BP_Unit.BP_Unit_C|GetUnitData (Variables|Default|GetCurrentUnitForReachables)))))) (.ValidTileTypes (Utilities|Struct|BreakS_UnitData_Stats (.Stats (Utilities|Struct|BreakS_UnitData (Variables|/Game/TacticalCards/Blueprints/Core/Units/BP_Unit.BP_Unit_C|GetUnitData (Variables|Default|GetCurrentUnitForReachables)))))) 0.1 15.0 true (.Movement_Current (Utilities|Struct|BreakS_UnitData_Stats (.Stats (Utilities|Struct|BreakS_UnitData (Variables|/Game/TacticalCards/Blueprints/Core/Units/BP_Unit.BP_Unit_C|GetUnitData (Variables|Default|GetCurrentUnitForReachables)))))))))

(fn OnPathfindingCompletedReachables
  (params (Reachables :type Array%20of%20Int%20Point%20Structures))
  (if (not (Variables|Default|GetIsUnitWalking))
    (for _array_element Reachables
      (Default|AddStatetoTile (Variables|/Game/TacticalCards/Blueprints/Core/Player/BP_PlayerActions.BP_PlayerActions_C|GetGrid (Variables|Default|GetPlayerActions)) _array_element "NewEnumerator7"))))

(fn ExecuteHoveredAction
  (params (Index :type Int%20Point%20Structure))
  (bind _playeractions (Variables|Default|GetPlayerActions))
  (bind _hoveredunit (Variables|/Game/TacticalCards/Blueprints/Core/Player/BP_PlayerActions.BP_PlayerActions_C|GetHoveredUnit _playeractions))
  (|CallParentFunction Index)
  (if (not (Variables|Default|GetIsUnitWalking))
    (Utilities|IsValid _hoveredunit
      (:Is%20Valid
        (CallFunction|GenerateReachables _hoveredunit))
      (:Is%20Not%20Valid
        (CallFunction|GenerateReachables (Variables|/Game/TacticalCards/Blueprints/Core/Player/BP_PlayerActions.BP_PlayerActions_C|GetSelectedUnit _playeractions))
        (CallFunction|GeneratePath)))))

(fn GeneratePath
  (bind _playeractions (Variables|Default|GetPlayerActions))
  (bind _playeractions_2 (Variables|Default|GetPlayerActions))
  (bind _selectedunit (Variables|/Game/TacticalCards/Blueprints/Core/Player/BP_PlayerActions.BP_PlayerActions_C|GetSelectedUnit _playeractions))
  (bind _unitdata (Variables|/Game/TacticalCards/Blueprints/Core/Units/BP_Unit.BP_Unit_C|GetUnitData _selectedunit))
  (bind _stats (Utilities|Struct|BreakS_UnitData _unitdata))
  (bind (_validtiletypes _canmovediagonally _movement_current) (Utilities|Struct|BreakS_UnitData_Stats _stats))
  (Default|ClearStatesfromTiles (Variables|/Game/TacticalCards/Blueprints/Core/Player/BP_PlayerActions.BP_PlayerActions_C|GetGrid (Variables|Default|GetPlayerActions)) "NewEnumerator4")
  (Utilities|Array|Clear (Variables|Default|GetGeneratedPath))
  (Default|FindPath (Variables|/Game/TacticalCards/Blueprints/Core/Grid/BP_Grid.BP_Grid_C|GetGridPathfinding (Variables|/Game/TacticalCards/Blueprints/Core/Player/BP_PlayerActions.BP_PlayerActions_C|GetGrid _playeractions_2)) (Variables|/Game/TacticalCards/Blueprints/Core/Units/BP_Unit.BP_Unit_C|GetIndex (Variables|/Game/TacticalCards/Blueprints/Core/Player/BP_PlayerActions.BP_PlayerActions_C|GetSelectedUnit _playeractions_2)) (Variables|/Game/TacticalCards/Blueprints/Core/Player/BP_PlayerActions.BP_PlayerActions_C|GetHoveredTile _playeractions_2) _canmovediagonally _validtiletypes 0.1 15.0 false _movement_current))

(fn OnPathfindingCompletedPath
  (params (Path :type Array%20of%20Int%20Point%20Structures))
  (bind _output_get (Variables|Default|SetGeneratedPath Path))
  (for _array_element _output_get
    (Default|AddStatetoTile (Variables|/Game/TacticalCards/Blueprints/Core/Player/BP_PlayerActions.BP_PlayerActions_C|GetGrid (Variables|Default|GetPlayerActions)) _array_element "NewEnumerator4")))

(fn ExecuteAction
  (params (Index :type Int%20Point%20Structure))
  (bind _playeractions (Variables|Default|GetPlayerActions))
  (|CallParentFunction Index)
  (if (> (Utilities|Array|Length (Variables|Default|GetGeneratedPath)) 0)
    (Default|MoveUnit (Variables|/Game/TacticalCards/Blueprints/Core/Player/BP_PlayerActions.BP_PlayerActions_C|GetCombatSystem _playeractions) (Variables|/Game/TacticalCards/Blueprints/Core/Player/BP_PlayerActions.BP_PlayerActions_C|GetSelectedUnit _playeractions) (Variables|Default|GetGeneratedPath))
    (Utilities|Array|Clear (Variables|Default|GetGeneratedPath))))

(fn OnUnitStartedWalking
  (params (Unit :type BP%20Unit%20Object%20Reference))
  (Variables|Default|SetIsUnitWalking true)
  (Default|ClearStatesfromTiles (Variables|/Game/TacticalCards/Blueprints/Core/Player/BP_PlayerActions.BP_PlayerActions_C|GetGrid (Variables|Default|GetPlayerActions)) "NewEnumerator7")
  (Variables|Default|SetCurrentUnitForReachables 0))

(fn OnUnitFinishedWalking
  (params (Unit :type BP%20Unit%20Object%20Reference))
  (Variables|Default|SetIsUnitWalking false)
  (CallFunction|ExecuteHoveredAction (Variables|/Game/TacticalCards/Blueprints/Core/Player/BP_PlayerActions.BP_PlayerActions_C|GetHoveredTile (Variables|Default|GetPlayerActions))))