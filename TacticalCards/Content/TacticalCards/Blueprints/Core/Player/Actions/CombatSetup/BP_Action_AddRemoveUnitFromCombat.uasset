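; Player action for combat setup that adds a unit to, or removes one from, a grid tile.
; When adding, it checks the tile type against the unit type's valid tiles, clears any occupant, then spawns a BP_Unit and registers it with the CombatSystem under a team and AI setting.
; When removing, it reuses the same clearing path, unregistering the tile's unit from combat and destroying it.
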(event EventBeginPlay
  (|CallParentFunction) ; This node is disabled and will not be called.\nDrag off pins to build functionality.
)

(event Collision|EventActorBeginOverlap
  (params (OtherActor :type Actor%20Object%20Reference))
  (|CallParentFunction OtherActor) ; This node is disabled and will not be called.\nDrag off pins to build functionality.
)

(event EventTick
  (params (DeltaSeconds :type Float%20%28single-precision%29))
  (|CallParentFunction DeltaSeconds) ; This node is disabled and will not be called.\nDrag off pins to build functionality.
)

(fn ConstructionScript
  (|CallParentFunction))

(fn ExecuteAction
  (params (Index :type Int%20Point%20Structure))
  (if (Variables|Default|GetIsAddingUnit)
    (bind _unitdata (CallFunction|GetDefaultUnitDatafromUnitType (Variables|Default|GetUnitType)))
    (if (Utilities|Array|ContainsItem (.ValidTileTypes (Utilities|Struct|BreakS_UnitData_Stats (.stats _unitdata))) (.type (.Value (Utilities|Map|Find (Variables|/Game/TacticalCards/Blueprints/Core/Grid/BP_Grid.BP_Grid_C|GetGridTiles (Variables|/Game/TacticalCards/Blueprints/Core/Player/BP_PlayerActions.BP_PlayerActions_C|GetGrid (Variables|Default|GetPlayerActions))) Index))))
      (Utilities|FlowControl|Sequence
        (:then_0
          (bind _output_get (LocalVariables|SetUnit (Utilities|Struct|BreakS_TileData (.Value (Utilities|Map|Find (Variables|/Game/TacticalCards/Blueprints/Core/Grid/BP_Grid.BP_Grid_C|GetGridTiles (Variables|/Game/TacticalCards/Blueprints/Core/Player/BP_PlayerActions.BP_PlayerActions_C|GetGrid (Variables|Default|GetPlayerActions))) Index))) :!label _label))
          (Utilities|IsValid _output_get
            (:Is%20Valid
              (Default|RemoveUnitfromCombat (Variables|/Game/TacticalCards/Blueprints/Core/Player/BP_PlayerActions.BP_PlayerActions_C|GetCombatSystem (Variables|Default|GetPlayerActions)) _output_get)
              (Actor|DestroyActor _output_get))))
        (:then_1
          (bind _returnvalue (Game|SpawnActorfromClass "/Game/TacticalCards/Blueprints/Core/Units/BP_Unit.BP_Unit_C" (Math|Transform|MakeTransform "0, 0, 0" "0, 0, 0" "0.250000,0.250000,0.250000") "AlwaysSpawn" "MultiplyWithRoot" 0 (Variables|Default|GetUnitType) 0))
          (Default|AddUnitinCombat (Variables|/Game/TacticalCards/Blueprints/Core/Player/BP_PlayerActions.BP_PlayerActions_C|GetCombatSystem (Variables|Default|GetPlayerActions)) _returnvalue Index (Variables|Default|GetTeamIndex) (Variables|Default|GetUseAI)))))
    (else
      (goto _label))))