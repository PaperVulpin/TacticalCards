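; Player action for the tactical combat setup that shows ability range and area-of-effect patterns as tile states on the grid.
; Executing it clears and re-marks the tiles the combat system returns for the cast range around the selected tile.
; It then, and again on hover, marks the AOE pattern around the hovered tile if that lies in range, or just that tile for one specific pattern value.
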(event EventBeginPlay
  (|CallParentFunction) ; This node is disabled and will not be called.\nDrag off pins to build functionality.
)

(event Collision|EventActorBeginOverlap
  (params (OtherActor :type Actor%20Object%20Reference))
  (|CallParentFunction OtherActor) ; This node is disabled and will not be called.\nDrag off pins to build functionality.
)

(event EventTick
  (params (DeltaSeconds :type Float%20%28single-precision%29))
  (|CallParentFunction DeltaSeconds) ; This node is disabled and will not be called.\nDrag off pins to build functionality.
)

(fn ConstructionScript
  (|CallParentFunction))

(fn ExecuteAction
  (params (Index :type Int%20Point%20Structure))
  (|CallParentFunction Index)
  (CallFunction|ShowAbilityRangePattern))

(fn ShowAbilityRangePattern
  (bind _playeractions (Variables|Default|GetPlayerActions))
  (bind _playeractions_2 (Variables|Default|GetPlayerActions))
  (bind _grid (Variables|/Game/TacticalCards/Blueprints/Core/Player/BP_PlayerActions.BP_PlayerActions_C|GetGrid _playeractions_2))
  (Utilities|FlowControl|Sequence
    (:then_0
      (Default|ClearStatesfromTiles _grid "NewEnumerator8")
      (if (Default|IsIndexValid _grid (Variables|/Game/TacticalCards/Blueprints/Core/Player/BP_PlayerActions.BP_PlayerActions_C|GetSelectedTile _playeractions_2))
        (bind _rangeindexes (Default|GetAbilityRange (Variables|/Game/TacticalCards/Blueprints/Core/Player/BP_PlayerActions.BP_PlayerActions_C|GetCombatSystem _playeractions) (Variables|/Game/TacticalCards/Blueprints/Core/Player/BP_PlayerActions.BP_PlayerActions_C|GetSelectedTile _playeractions) (Variables|Default|GetCast)))
        (for _array_element _rangeindexes
          (Default|AddStatetoTile (Variables|/Game/TacticalCards/Blueprints/Core/Player/BP_PlayerActions.BP_PlayerActions_C|GetGrid (Variables|Default|GetPlayerActions)) _array_element "NewEnumerator8"))))
    (:then_1
      (CallFunction|ShowAbilityRangePatternAOE))))

(fn ShowAbilityRangePatternAOE
  (bind _playeractions (Variables|Default|GetPlayerActions))
  (bind _playeractions_2 (Variables|Default|GetPlayerActions))
  (bind _playeractions_3 (Variables|Default|GetPlayerActions))
  (bind _grid (Variables|/Game/TacticalCards/Blueprints/Core/Player/BP_PlayerActions.BP_PlayerActions_C|GetGrid _playeractions_3))
  (Default|ClearStatesfromTiles _grid "NewEnumerator9")
  (if (Utilities|Array|ContainsItem (Utilities|Struct|BreakS_IntPointArray (.Value (Utilities|Map|Find (Variables|/Game/TacticalCards/Blueprints/Core/Grid/BP_Grid.BP_Grid_C|GetTileStateToIndexes _grid) "NewEnumerator8"))) (Variables|/Game/TacticalCards/Blueprints/Core/Player/BP_PlayerActions.BP_PlayerActions_C|GetHoveredTile _playeractions_3))
    (if (Utilities|Enum|NotEqual(Enum) (.RangePattern (Utilities|Struct|BreakS_AbilityData_Cast (Variables|Default|GetCastAOE))) "NewEnumerator0")
      (bind _rangeindexes (Default|GetAbilityRange (Variables|/Game/TacticalCards/Blueprints/Core/Player/BP_PlayerActions.BP_PlayerActions_C|GetCombatSystem _playeractions) (Variables|/Game/TacticalCards/Blueprints/Core/Player/BP_PlayerActions.BP_PlayerActions_C|GetHoveredTile _playeractions) (Variables|Default|GetCastAOE)))
      (for _array_element _rangeindexes
        (Default|AddStatetoTile (Variables|/Game/TacticalCards/Blueprints/Core/Player/BP_PlayerActions.BP_PlayerActions_C|GetGrid (Variables|Default|GetPlayerActions)) _array_element "NewEnumerator9"))
      (else
        (Default|AddStatetoTile (Variables|/Game/TacticalCards/Blueprints/Core/Player/BP_PlayerActions.BP_PlayerActions_C|GetGrid _playeractions_2) (Variables|/Game/TacticalCards/Blueprints/Core/Player/BP_PlayerActions.BP_PlayerActions_C|GetHoveredTile _playeractions_2) "NewEnumerator9")))))

(fn ExecuteHoveredAction
  (params (Index :type Int%20Point%20Structure))
  (|CallParentFunction Index)
  (CallFunction|ShowAbilityRangePatternAOE))