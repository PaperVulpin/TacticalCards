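; Player action that highlights the valid neighboring tiles of a given grid tile.
; ExecuteAction clears a tile state from the grid, asks the grid's pathfinding for valid neighbors filtered by tile types and optional diagonals, then adds that state to each one.
; EndPlay runs it with an out-of-range index, presumably to clear the highlight when the action is removed.
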(event EventBeginPlay
  (|CallParentFunction) ; This node is disabled and will not be called.\nDrag off pins to build functionality.
)

(event Collision|EventActorBeginOverlap
  (params (OtherActor :type Actor%20Object%20Reference))
  (|CallParentFunction OtherActor) ; This node is disabled and will not be called.\nDrag off pins to build functionality.
)

(event EventTick
  (params (DeltaSeconds :type Float%20%28single-precision%29))
  (|CallParentFunction DeltaSeconds) ; This node is disabled and will not be called.\nDrag off pins to build functionality.
)

(event EventEndPlay
  (params (EndPlayReason :type EEndPlayReason%20Enum :default "Destroyed"))
  (CallFunction|ExecuteAction (Utilities|Struct|MakeIntPoint -999 -999)))

(fn ConstructionScript
  (|CallParentFunction))

(fn ExecuteAction
  (params (Index :type Int%20Point%20Structure))
  (bind _playeractions (Variables|Default|GetPlayerActions))
  (bind _grid (Variables|/Game/TacticalCards/Blueprints/Core/Player/BP_PlayerActions.BP_PlayerActions_C|GetGrid _playeractions))
  (Default|ClearStatesfromTiles _grid "NewEnumerator3")
  (bind _neighbors (Default|GetValidTileNeighbors (Variables|/Game/TacticalCards/Blueprints/Core/Grid/BP_Grid.BP_Grid_C|GetGridPathfinding _grid) Index (Variables|Default|GetInclude%20Diagonals) (Utilities|Array|MakeArray "NewEnumerator1" "NewEnumerator3" "NewEnumerator4" "NewEnumerator5")))
  (for _array_element _neighbors
    (Default|AddStatetoTile _grid (.index _array_element) "NewEnumerator3")))