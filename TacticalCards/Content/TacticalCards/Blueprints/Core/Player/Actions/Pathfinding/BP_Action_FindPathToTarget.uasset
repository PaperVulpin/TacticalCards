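; Player action that pathfinds from the selected tile to a target tile on the tactical grid and marks the resulting path.
; It clears old path states, calls GridPathfinding with configurable diagonals, flying-only tiles, length limit, iteration delay and per-frame time budget.
; The completion callback applies the path state to each returned tile.
; Selection changes and EndPlay rerun the action with an out-of-range sentinel target, clearing the previous path.
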(event Custom|OnSelectedTileChanged
  (params (Index :type Int%20Point%20Structure))
  (CallFunction|ExecuteAction (Utilities|Struct|MakeIntPoint -999 -999)))

(event EventBeginPlay
  (EventDispatchers|BindEventtoOnSelectedTileChanged (Variables|Default|GetPlayerActions) (delegate Custom|OnSelectedTileChanged)))

(event EventEndPlay
  (params (EndPlayReason :type EEndPlayReason%20Enum :default "Destroyed"))
  (CallFunction|ExecuteAction (Utilities|Struct|MakeIntPoint -999 -999)))

(fn ConstructionScript
  (|CallParentFunction))

(fn ExecuteAction
  (params (Index :type Int%20Point%20Structure))
  (bind _playeractions (Variables|Default|GetPlayerActions))
  (bind _grid (Variables|/Game/TacticalCards/Blueprints/Core/Player/BP_PlayerActions.BP_PlayerActions_C|GetGrid _playeractions))
  (bind _gridpathfinding (Variables|/Game/TacticalCards/Blueprints/Core/Grid/BP_Grid.BP_Grid_C|GetGridPathfinding _grid))
  (Default|ClearStatesfromTiles _grid "NewEnumerator4")
  (EventDispatchers|BindEventtoOnPathfindingCompleted _gridpathfinding (EventDispatchers|CreateEvent :!event OnPathfindingCompleted))
  (Default|FindPath _gridpathfinding (Variables|/Game/TacticalCards/Blueprints/Core/Player/BP_PlayerActions.BP_PlayerActions_C|GetSelectedTile _playeractions) Index (Variables|Default|GetInclude%20Diagonals) (select (Variables|Default|GetIncludeFlyingOnly) (Utilities|Array|MakeArray "NewEnumerator1" "NewEnumerator3" "NewEnumerator4" "NewEnumerator5") (Utilities|Array|MakeArray "NewEnumerator1" "NewEnumerator3" "NewEnumerator4")) (Variables|Default|GetDelayBetweenIterations) (Variables|Default|GetMaxMsPerFrame) false (Variables|Default|GetMaxPathLength)))

(fn OnPathfindingCompleted
  (params (Path :type Array%20of%20Int%20Point%20Structures))
  (for _array_element Path
    (Default|AddStatetoTile (Variables|/Game/TacticalCards/Blueprints/Core/Player/BP_PlayerActions.BP_PlayerActions_C|GetGrid (Variables|Default|GetPlayerActions)) _array_element "NewEnumerator4")))