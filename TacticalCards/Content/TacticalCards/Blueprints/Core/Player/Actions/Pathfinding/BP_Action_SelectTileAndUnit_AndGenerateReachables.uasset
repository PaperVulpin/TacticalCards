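; Player action that, after selecting a tile and unit, highlights the tiles reachable from the selected tile on the grid.
; It runs the grid's reachables pathfinder using the unit's movement, diagonal and tile-type stats, or the action's own path settings when no unit is selected.
; Completed results become tile states, which clear when the unit starts walking and regenerate when it finishes.
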(event EventBeginPlay
  (|CallParentFunction) ; This node is disabled and will not be called.\nDrag off pins to build functionality.
)

(event Collision|EventActorBeginOverlap
  (params (OtherActor :type Actor%20Object%20Reference))
  (|CallParentFunction OtherActor) ; This node is disabled and will not be called.\nDrag off pins to build functionality.
)

(event EventTick
  (params (DeltaSeconds :type Float%20%28single-precision%29))
  (|CallParentFunction DeltaSeconds) ; This node is disabled and will not be called.\nDrag off pins to build functionality.
)

(fn ConstructionScript
  (|CallParentFunction))

(fn GenerateReachables
  (bind _playeractions (Variables|Default|GetPlayerActions))
  (bind _selectedtile (Variables|/Game/TacticalCards/Blueprints/Core/Player/BP_PlayerActions.BP_PlayerActions_C|GetSelectedTile _playeractions))
  (bind _selectedunit (Variables|/Game/TacticalCards/Blueprints/Core/Player/BP_PlayerActions.BP_PlayerActions_C|GetSelectedUnit _playeractions))
  (bind _grid (Variables|/Game/TacticalCards/Blueprints/Core/Player/BP_PlayerActions.BP_PlayerActions_C|GetGrid _playeractions))
  (bind _gridpathfinding_reachables (Variables|/Game/TacticalCards/Blueprints/Core/Grid/BP_Grid.BP_Grid_C|GetGridPathfinding_Reachables _grid))
  (bind _unitdata (Variables|/Game/TacticalCards/Blueprints/Core/Units/BP_Unit.BP_Unit_C|GetUnitData _selectedunit))
  (bind _stats (Utilities|Struct|BreakS_UnitData _unitdata))
  (bind (_validtiletypes _canmovediagonally _availableabilities _hp_current _hp_max _movement_current) (Utilities|Struct|BreakS_UnitData_Stats _stats))
  (Default|ClearStatesfromTiles _grid "NewEnumerator7")
  (EventDispatchers|BindEventtoOnPathfindingCompleted _gridpathfinding_reachables (EventDispatchers|CreateEvent :!event OnPathfindingCompleted))
  (Utilities|IsValid _selectedunit
    (:Is%20Valid
      (EventDispatchers|BindEventtoOnUnitStartedWalking _selectedunit (EventDispatchers|CreateEvent :!event OnUnitStartedWalking))
      (EventDispatchers|BindEventtoOnUnitFinishedWalking _selectedunit (EventDispatchers|CreateEvent :!event OnUnitFinishedWalking))
      (Default|FindPath _gridpathfinding_reachables _selectedtile (Utilities|Struct|MakeIntPoint -999 -999) _canmovediagonally _validtiletypes 0.0 0.0 true _movement_current))
    (:Is%20Not%20Valid
      (Default|FindPath _gridpathfinding_reachables _selectedtile (Utilities|Struct|MakeIntPoint -999 -999) (Variables|Default|GetIncludeDiagonals) (select (Variables|Default|GetIncludeFlyingOnly) (Utilities|Array|MakeArray "NewEnumerator1" "NewEnumerator3" "NewEnumerator4" "NewEnumerator5") (Utilities|Array|MakeArray "NewEnumerator1" "NewEnumerator3" "NewEnumerator4")) (Variables|Default|GetDelayBetweenIterations) (Variables|Default|GetMaxMsPerFrame) true (Variables|Default|GetMaxPathLength)))))

(fn ExecuteAction
  (params (Index :type Int%20Point%20Structure))
  (|CallParentFunction Index)
  (CallFunction|GenerateReachables))

(fn OnPathfindingCompleted
  (params (Path :type Array%20of%20Int%20Point%20Structures))
  (for _array_element Path
    (Default|AddStatetoTile (Variables|/Game/TacticalCards/Blueprints/Core/Player/BP_PlayerActions.BP_PlayerActions_C|GetGrid (Variables|Default|GetPlayerActions)) _array_element "NewEnumerator7")))

(fn OnUnitStartedWalking
  (params (Unit :type BP%20Unit%20Object%20Reference))
  (Default|ClearStatesfromTiles (Variables|/Game/TacticalCards/Blueprints/Core/Player/BP_PlayerActions.BP_PlayerActions_C|GetGrid (Variables|Default|GetPlayerActions)) "NewEnumerator7"))

(fn OnUnitFinishedWalking
  (params (Unit :type BP%20Unit%20Object%20Reference))
  (CallFunction|GenerateReachables))