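; Player action that moves the selected unit across the grid from the selected tile to a target tile.
; ExecuteAction clears path tile states and requests pathfinding using the unit's diagonal, tile-type and current-movement stats.
; The completion callback marks path tiles, moves the unit via the CombatSystem and resets its movement; highlights clear when walking finishes.
; EndPlay re-runs ExecuteAction with an out-of-range sentinel index.
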(event EventBeginPlay
  (|CallParentFunction) ; This node is disabled and will not be called.\nDrag off pins to build functionality.
)

(event Collision|EventActorBeginOverlap
  (params (OtherActor :type Actor%20Object%20Reference))
  (|CallParentFunction OtherActor) ; This node is disabled and will not be called.\nDrag off pins to build functionality.
)

(event EventTick
  (params (DeltaSeconds :type Float%20%28single-precision%29))
  (|CallParentFunction DeltaSeconds) ; This node is disabled and will not be called.\nDrag off pins to build functionality.
)

(event EventEndPlay
  (params (EndPlayReason :type EEndPlayReason%20Enum :default "Destroyed"))
  (CallFunction|ExecuteAction (Utilities|Struct|MakeIntPoint -999 -999)))

(fn ConstructionScript
  (|CallParentFunction))

(fn ExecuteAction
  (params (Index :type Int%20Point%20Structure))
  (bind _playeractions (Variables|Default|GetPlayerActions))
  (bind _grid (Variables|/Game/TacticalCards/Blueprints/Core/Player/BP_PlayerActions.BP_PlayerActions_C|GetGrid _playeractions))
  (bind _gridpathfinding (Variables|/Game/TacticalCards/Blueprints/Core/Grid/BP_Grid.BP_Grid_C|GetGridPathfinding _grid))
  (Default|ClearStatesfromTiles _grid "NewEnumerator4")
  (bind _output_get (Variables|Default|SetCurrentUnit (Variables|/Game/TacticalCards/Blueprints/Core/Player/BP_PlayerActions.BP_PlayerActions_C|GetSelectedUnit _playeractions)))
  (Utilities|IsValid _output_get
    (:Is%20Valid
      (EventDispatchers|BindEventtoOnUnitFinishedWalking _output_get (EventDispatchers|CreateEvent :!event OnUnitFinishedWalking))
      (EventDispatchers|BindEventtoOnPathfindingCompleted _gridpathfinding (EventDispatchers|CreateEvent :!event OnPathfindingCompleted))
      (Default|FindPath _gridpathfinding (Variables|/Game/TacticalCards/Blueprints/Core/Player/BP_PlayerActions.BP_PlayerActions_C|GetSelectedTile _playeractions) Index (.CanMoveDiagonally (Utilities|Struct|BreakS_UnitData_Stats (.Stats (Utilities|Struct|BreakS_UnitData (Variables|/Game/TacticalCards/Blueprints/Core/Units/BP_Unit.BP_Unit_C|GetUnitData (Variables|Default|GetCurrentUnit)))))) (.ValidTileTypes (Utilities|Struct|BreakS_UnitData_Stats (.Stats (Utilities|Struct|BreakS_UnitData (Variables|/Game/TacticalCards/Blueprints/Core/Units/BP_Unit.BP_Unit_C|GetUnitData (Variables|Default|GetCurrentUnit)))))) 0.0 0.0 false (.Movement_Current (Utilities|Struct|BreakS_UnitData_Stats (.Stats (Utilities|Struct|BreakS_UnitData (Variables|/Game/TacticalCards/Blueprints/Core/Units/BP_Unit.BP_Unit_C|GetUnitData (Variables|Default|GetCurrentUnit))))))))))

(fn OnPathfindingCompleted
  (params (Path :type Array%20of%20Int%20Point%20Structures))
  (bind _playeractions (Variables|Default|GetPlayerActions))
  (bind _currentunit (Variables|Default|GetCurrentUnit))
  (Utilities|IsValid _currentunit
    (:Is%20Valid
      (if (== _currentunit (Variables|/Game/TacticalCards/Blueprints/Core/Player/BP_PlayerActions.BP_PlayerActions_C|GetSelectedUnit _playeractions))
        (for _array_element Path
          (Default|AddStatetoTile (Variables|/Game/TacticalCards/Blueprints/Core/Player/BP_PlayerActions.BP_PlayerActions_C|GetGrid _playeractions) _array_element "NewEnumerator4"))
        (Variables|/Game/TacticalCards/Blueprints/Core/Units/BP_Unit.BP_Unit_C|SetMoveDurationPerTile _currentunit (Variables|Default|GetMoveDuration))
        (Default|MoveUnit (Variables|/Game/TacticalCards/Blueprints/Core/Player/BP_PlayerActions.BP_PlayerActions_C|GetCombatSystem (Variables|Default|GetPlayerActions)) _currentunit Path)
        (Default|ResetMovement _currentunit)))))

(fn OnUnitFinishedWalking
  (params (Unit :type BP%20Unit%20Object%20Reference))
  (if (== Unit (Variables|Default|GetCurrentUnit))
    (Default|ClearStatesfromTiles (Variables|/Game/TacticalCards/Blueprints/Core/Player/BP_PlayerActions.BP_PlayerActions_C|GetGrid (Variables|Default|GetPlayerActions)) "NewEnumerator4")))