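; Player grid action that extends tile selection to calculate the minimum pathfinding cost from every tile to the selected tile.
; After the parent action runs, it clears the grid pathfinding's generated data.
; If the selected tile is valid, it registers every grid tile as discovered, with zero cost from start and its estimated minimum cost to that tile, optionally counting diagonals.
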(event EventBeginPlay
  (|CallParentFunction) ; This node is disabled and will not be called.\nDrag off pins to build functionality.
)

(event Collision|EventActorBeginOverlap
  (params (OtherActor :type Actor%20Object%20Reference))
  (|CallParentFunction OtherActor) ; This node is disabled and will not be called.\nDrag off pins to build functionality.
)

(event EventTick
  (params (DeltaSeconds :type Float%20%28single-precision%29))
  (|CallParentFunction DeltaSeconds) ; This node is disabled and will not be called.\nDrag off pins to build functionality.
)

(fn ConstructionScript
  (|CallParentFunction))

(fn ExecuteAction
  (params (Index :type Int%20Point%20Structure))
  (bind _playeractions (Variables|Default|GetPlayerActions))
  (bind _grid (Variables|/Game/TacticalCards/Blueprints/Core/Player/BP_PlayerActions.BP_PlayerActions_C|GetGrid _playeractions))
  (bind _selectedtile (Variables|/Game/TacticalCards/Blueprints/Core/Player/BP_PlayerActions.BP_PlayerActions_C|GetSelectedTile _playeractions))
  (bind _gridpathfinding (Variables|/Game/TacticalCards/Blueprints/Core/Grid/BP_Grid.BP_Grid_C|GetGridPathfinding _grid))
  (|CallParentFunction Index)
  (Default|ClearGeneratedData _gridpathfinding)
  (if (Default|IsIndexValid _grid _selectedtile)
    (bind _keys (Utilities|Map|Keys (Variables|/Game/TacticalCards/Blueprints/Core/Grid/BP_Grid.BP_Grid_C|GetGridTiles _grid)))
    (for _array_element _keys
      (Default|DiscoverTile _gridpathfinding (Utilities|Struct|MakeS_PathfindingData _array_element 1 0 (Default|GetMinimumCostBetweenTwoTiles _gridpathfinding _array_element _selectedtile (Variables|Default|GetIncludeDiagonals)) "(X=-999,Y=-999)")))))