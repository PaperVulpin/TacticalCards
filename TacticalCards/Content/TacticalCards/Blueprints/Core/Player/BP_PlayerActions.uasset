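; Player input hub for the tactical card game, turning mouse and keyboard input into grid and unit actions in overworld and combat.
; Each tick it traces the hovered tile and unit, while selection updates tile states and unit highlights.
; Left and right clicks run swappable spawned action actors, re-fired on tile change while held.
; Combat events swap those actions and manage combat UI; number keys pick abilities and Space ends turns.
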(event Custom|Event_ExecuteActionWhenHoveredTileChanged
  (bind _selectedaction_rightclick (Variables|Actions|GetSelectedAction_RightClick))
  (bind _hoveredtile (Variables|Default|GetHoveredTile))
  (bind _selectedaction_leftclick (Variables|Actions|GetSelectedAction_LeftClick))
  (Utilities|FlowControl|Sequence
    (:then_0
      (Utilities|IsValid _selectedaction_leftclick
        (:Is%20Valid
          (Default|ExecuteHoveredAction _selectedaction_leftclick (Variables|Default|GetHoveredTile))
          (if (Variables|Actions|GetIsLeftClickDown)
            (Default|ExecuteAction (Variables|Actions|GetSelectedAction_LeftClick) _hoveredtile)))))
    (:then_1
      (Utilities|IsValid _selectedaction_rightclick
        (:Is%20Valid
          (Default|ExecuteHoveredAction _selectedaction_rightclick (Variables|Default|GetHoveredTile))
          (if (Variables|Actions|GetIsRightClickDown)
            (Default|ExecuteAction (Variables|Actions|GetSelectedAction_RightClick) _hoveredtile)))))))

(event Custom|Event_SimulateLeftClickFromExternalSource
  (bind _selectedaction_leftclick (Variables|Actions|GetSelectedAction_LeftClick))
  (Utilities|FlowControl|Sequence
    (:then_0
      (HoveredandSelected|UpdateHoveredTileandUnit)
      (Variables|Actions|SetIsLeftClickDown true)
      (Utilities|IsValid _selectedaction_leftclick
        (:Is%20Valid
          (Default|ExecuteAction _selectedaction_leftclick (Variables|Default|GetHoveredTile)))))
    (:then_1
      (Variables|Actions|SetIsLeftClickDown false))))

(event EventBeginPlay
  (bind _combatsystem (Variables|References|GetCombatSystem))
  (bind _overworldunitgroupsmanager (Variables|References|GetOverworldUnitGroupsManager))
  (Variables|References|SetGrid (Variables|/Game/TacticalCards/Blueprints/Core/Combat/BP_CombatSystem.BP_CombatSystem_C|GetGrid (Variables|References|GetCombatSystem)))
  (EventDispatchers|BindEventtoOnGridGenerated (Variables|References|GetGrid) (EventDispatchers|CreateEvent :!event OnGridGenerated))
  (EventDispatchers|BindEventtoOnTileDataUpdated (Variables|References|GetGrid) (EventDispatchers|CreateEvent :!event OnTileDataUpdated))
  (EventDispatchers|BindEventtoOnUnitGridIndexChanged _combatsystem (EventDispatchers|CreateEvent :!event OnUnitGridIndexChanged))
  (EventDispatchers|BindEventtoOnCombatStarted _combatsystem (EventDispatchers|CreateEvent :!event OnCombatStarted))
  (EventDispatchers|BindEventtoOnCombatEnded _combatsystem (EventDispatchers|CreateEvent :!event OnCombatEnded))
  (EventDispatchers|BindEventtoOnUnitTurnStarted _combatsystem (EventDispatchers|CreateEvent :!event OnUnitTurnStarted))
  (EventDispatchers|BindEventtoOnUnitTurnEnded _combatsystem (EventDispatchers|CreateEvent :!event OnUnitTurnEnded))
  (EventDispatchers|BindEventtoOnCombatFinishing _combatsystem (EventDispatchers|CreateEvent :!event OnCombatFinishing))
  (Input|EnableInput (Game|GetPlayerController 0))
  (Utilities|IsValid _overworldunitgroupsmanager
    (:Is%20Valid
      (Default|SetCombatSystem _overworldunitgroupsmanager (Variables|References|GetCombatSystem))
      (if (Variables|Default|GetAutoSelectOverworldMovementActions)
        (Actions|SetSelectedActions "/Game/TacticalCards/Blueprints/Core/Player/Actions/Overworld/BP_Action_SelectUnitInOverworld.BP_Action_SelectUnitInOverworld_C" "/Game/TacticalCards/Blueprints/Core/Player/Actions/Overworld/BP_Action_MoveUnitInOverworld.BP_Action_MoveUnitInOverworld_C")))))

(event EventTick
  (params (DeltaSeconds :type Float%20%28single-precision%29))
  (HoveredandSelected|UpdateHoveredTileandUnit))

(event Input|MouseEvents|LeftMouseButton
  (params (Key :type Key%20Structure))
  (bind _selectedaction_leftclick (Variables|Actions|GetSelectedAction_LeftClick))
  (:Pressed
    (HoveredandSelected|UpdateHoveredTileandUnit)
    (Variables|Actions|SetIsLeftClickDown true)
    (Utilities|IsValid _selectedaction_leftclick
      (:Is%20Valid
        (Default|ExecuteAction _selectedaction_leftclick (Variables|Default|GetHoveredTile)))))
  (:Released
    (Variables|Actions|SetIsLeftClickDown false)))

(event Input|MouseEvents|RightMouseButton
  (params (Key :type Key%20Structure))
  (bind _selectedaction_rightclick (Variables|Actions|GetSelectedAction_RightClick))
  (:Pressed
    (HoveredandSelected|UpdateHoveredTileandUnit)
    (Variables|Actions|SetIsRightClickDown true)
    (Utilities|IsValid _selectedaction_rightclick
      (:Is%20Valid
        (Default|ExecuteAction _selectedaction_rightclick (Variables|Default|GetHoveredTile)))))
  (:Released
    (Variables|Actions|SetIsRightClickDown false)))

(event Input|KeyboardEvents|AnyKey
  (params (Key :type Key%20Structure))
  (bind _returnvalue (Class|KismetInputLibrary|KeyGetDisplayName Key true))
  (bind _combatsystem (Variables|References|GetCombatSystem))
  (bind _returnvalue_2 (Utilities|String|ToString(Text) _returnvalue))
  (:Pressed
    (if (Math|Boolean|ANDBoolean (Variables|/Game/TacticalCards/Blueprints/Core/Combat/BP_CombatSystem.BP_CombatSystem_C|GetIsInCombat _combatsystem) (not (Variables|/Game/TacticalCards/Blueprints/Core/Combat/BP_CombatSystem.BP_CombatSystem_C|GetIsFinishingCombat _combatsystem)) (== (Variables|/Game/TacticalCards/Blueprints/Core/Combat/BP_CombatSystem.BP_CombatSystem_C|GetCurrentUnit _combatsystem) (Variables|Default|GetSelectedUnit)))
      (if (Class|KismetStringLibrary|IsNumeric _returnvalue_2)
        (Default|SetSelectedAbilityfromIndex (Variables|/Game/TacticalCards/Blueprints/Core/Combat/Widgets/WBP_Combat.WBP_Combat_C|GetButtonList_Abilities (Variables|Default|GetW_Combat)) (Math|Conversions|ToInteger(Byte) _returnvalue_2))
        (elif (Utilities|Enum|Equal(Enum) _returnvalue_2 "Space Bar")
          (Default|NextUnit (Variables|References|GetCombatSystem)))))))

(fn ConstructionScript)

(fn UpdateHoveredTileandUnit
  (bind _grid (Variables|References|GetGrid))
  (bind _hoveredunitoverride (Variables|Default|GetHoveredUnitOverride))
  (Utilities|FlowControl|Sequence
    (:then_0
      (Utilities|IsValid _hoveredunitoverride
        (:Is%20Valid
          (LocalVariables|SetU _hoveredunitoverride))
        (:Is%20Not%20Valid
          (bind _unit (HoveredandSelected|GetUnitUnderCursor))
          (bind _output_get (LocalVariables|SetU _unit))))
      (if (!= _output_get (Variables|Default|GetHoveredUnit))
        (Utilities|FlowControl|Sequence
          (:then_0
            (Utilities|IsValid (Variables|Default|GetHoveredUnit)
              (:Is%20Valid
                (Default|SetIsHovered (Variables|Default|GetHoveredUnit) false))))
          (:then_1
            (Variables|Default|SetHoveredUnit _output_get)
            (Utilities|IsValid _output_get
              (:Is%20Valid
                (Default|SetIsHovered _output_get true)))))))
    (:then_1
      (Utilities|IsValid (Variables|Default|GetHoveredUnit)
        (:Is%20Valid
          (LocalVariables|SetNewIndex (Variables|/Game/TacticalCards/Blueprints/Core/Units/BP_Unit.BP_Unit_C|GetIndex (Variables|Default|GetHoveredUnit))))
        (:Is%20Not%20Valid
          (bind _index (Default|GetTileIndexUnderCursor _grid 0 (CallFunction|CanHoverGround) (CallFunction|CanHoverEmptySpace)))
          (bind _output_get_2 (LocalVariables|SetNewIndex _index))))
      (if (!= _output_get_2 (Variables|Default|GetHoveredTile))
        (Default|RemoveStatefromTile _grid (Variables|Default|GetHoveredTile) "NewEnumerator1")
        (bind _output_get_3 (Variables|Default|SetHoveredTile _output_get_2))
        (Default|AddStatetoTile _grid _output_get_3 "NewEnumerator1")
        (CallFunction|EventExecuteActionwhenHoveredTileChanged)
        (Default|CallOnHoveredTileChanged (Variables|Default|GetHoveredTile))))))

(fn SetSelectedActions
  (params (LeftAction :type BP%20Action%20Class%20Reference) (RightAction :type BP%20Action%20Class%20Reference))
  (Utilities|FlowControl|Sequence
    (:then_0
      (Utilities|IsValid (Variables|Actions|GetSelectedAction_LeftClick)
        (:Is%20Valid
          (Actor|DestroyActor (Variables|Actions|GetSelectedAction_LeftClick))
          (Variables|Actions|SetSelectedAction_LeftClick 0))
        (:Is%20Not%20Valid
          _))
      (if (Utilities|IsValidClass LeftAction)
        (bind _returnvalue (Game|SpawnActorfromClass LeftAction (Math|Transform|MakeTransform "0, 0, 0" "0, 0, 0" "1.000000,1.000000,1.000000") "AlwaysSpawn" "MultiplyWithRoot" 0 self 0))
        (Variables|Actions|SetSelectedAction_LeftClick _returnvalue)))
    (:then_1
      (Utilities|IsValid (Variables|Actions|GetSelectedAction_RightClick)
        (:Is%20Valid
          (Actor|DestroyActor (Variables|Actions|GetSelectedAction_RightClick))
          (Variables|Actions|SetSelectedAction_RightClick 0))
        (:Is%20Not%20Valid
          _))
      (if (Utilities|IsValidClass RightAction)
        (bind _returnvalue_2 (Game|SpawnActorfromClass RightAction (Math|Transform|MakeTransform "0, 0, 0" "0, 0, 0" "1.000000,1.000000,1.000000") "AlwaysSpawn" "MultiplyWithRoot" 0 self 0))
        (Variables|Actions|SetSelectedAction_RightClick _returnvalue_2)))
    (:then_2
      (Default|CallOnSelectedActionsChanged (Variables|Actions|GetSelectedAction_LeftClick) (Variables|Actions|GetSelectedAction_RightClick)))))

(fn GetUnitUnderCursor
  (params (PlayerIndex :type Integer))
  (bind _returnvalue (Game|GetPlayerController PlayerIndex))
  (bind (_hitresult _returnvalue_2) (Game|Player|GetHitResultUnderCursorbyChannel _returnvalue "TraceTypeQuery5" true))
  (if _returnvalue_2
    (return (.AsBP%20Unit (Utilities|Casting|CastToBP_Unit (.HitActor (Collision|BreakHitResult _hitresult)))))
    (else
      (bind _index (Default|GetTileIndexUnderCursor (Variables|References|GetGrid) PlayerIndex (CallFunction|CanHoverGround) (CallFunction|CanHoverEmptySpace)))
      (return (Utilities|Struct|BreakS_TileData (.Value (Utilities|Map|Find (Variables|/Game/TacticalCards/Blueprints/Core/Grid/BP_Grid.BP_Grid_C|GetGridTiles (Variables|References|GetGrid)) _index)))))))

(fn SetSelectedTileandUnit
  (params (Index :type Int%20Point%20Structure) (Unit :type BP%20Unit%20Object%20Reference) (Force :type Boolean))
  (bind _grid (Variables|References|GetGrid))
  (bind _output_get (LocalVariables|SetDesiredIndex Index))
  (Utilities|IsValid Unit
    (:Is%20Valid
      (LocalVariables|SetDesiredIndex (Variables|/Game/TacticalCards/Blueprints/Core/Units/BP_Unit.BP_Unit_C|GetIndex Unit)))
    (:Is%20Not%20Valid
      _))
  (Utilities|FlowControl|Sequence
    (:then_0
      (if (or (!= _output_get (Variables|Default|GetSelectedTile)) Force) ; Different Tile?
        (Default|RemoveStatefromTile _grid (Variables|Default|GetSelectedTile) "NewEnumerator2")
        (bind _output_get_2 (Variables|Default|SetSelectedTile _output_get))
        (Default|AddStatetoTile _grid _output_get_2 "NewEnumerator2")
        (else
          (Default|RemoveStatefromTile _grid (Variables|Default|GetSelectedTile) "NewEnumerator2")
          (Variables|Default|SetSelectedTile (Utilities|Struct|MakeIntPoint -999 -999))))
      (Default|CallOnSelectedTileChanged (Variables|Default|GetSelectedTile)))
    (:then_1
      (LocalVariables|SetNewUnit (select (Utilities|IsValid Unit) Unit (Utilities|Struct|BreakS_TileData (.Value (Utilities|Map|Find (Variables|/Game/TacticalCards/Blueprints/Core/Grid/BP_Grid.BP_Grid_C|GetGridTiles (Variables|References|GetGrid)) (Variables|Default|GetSelectedTile))))))
      (if (or Force (!= (Variables|Default|GetSelectedUnit) (LocalVariables|GetNewUnit)))
        (Utilities|FlowControl|Sequence
          (:then_0
            (Utilities|IsValid (Variables|Default|GetSelectedUnit)
              (:Is%20Valid
                (Default|SetIsSelected (Variables|Default|GetSelectedUnit) false))))
          (:then_1
            (bind _output_get_3 (Variables|Default|SetSelectedUnit (LocalVariables|GetNewUnit)))
            (Utilities|IsValid _output_get_3
              (:Is%20Valid
                (Default|SetIsSelected _output_get_3 true)))))))))

(fn OnGridGenerated
  (if (Default|IsIndexValid (Variables|References|GetGrid) (Variables|Default|GetSelectedTile))
    (HoveredandSelected|SetSelectedTileandUnit (Variables|Default|GetSelectedTile) 0 true)
    (else
      (HoveredandSelected|SetSelectedTileandUnit (Utilities|Struct|MakeIntPoint -999 -999) 0 false))))

(fn OnTileDataUpdated
  (params (Index :type Int%20Point%20Structure))
  (if (Class|KismetMathLibrary|EqualIntPointIntPoint Index (Variables|Default|GetSelectedTile))
    (Grid|OnGridGenerated)))

(fn OnUnitGridIndexChanged
  (params (Unit :type BP%20Unit%20Object%20Reference))
  (if (== Unit (Variables|Default|GetSelectedUnit))
    (HoveredandSelected|SetSelectedTileandUnit (Variables|/Game/TacticalCards/Blueprints/Core/Units/BP_Unit.BP_Unit_C|GetIndex Unit) 0 false)))

(fn OnCombatStarted
  (Actions|SetSelectedActions)
  (HoveredandSelected|SetSelectedTileandUnit (Utilities|Struct|MakeIntPoint -999 -999) 0 false)
  (bind _returnvalue (UserInterface|CreateWidget "/Game/TacticalCards/Blueprints/Core/Combat/Widgets/WBP_Combat.WBP_Combat_C" 0 self))
  (bind _output_get (Variables|Default|SetW_Combat _returnvalue))
  (UserInterface|Viewport|AddtoPlayerScreen _output_get)
  (EventDispatchers|BindEventtoOnSelectedAbilityButtonChanged (Variables|/Game/TacticalCards/Blueprints/Core/Combat/Widgets/WBP_Combat.WBP_Combat_C|GetButtonList_Abilities (Variables|Default|GetW_Combat)) (EventDispatchers|CreateEvent :!event OnSelectedAbilityChanged)))

(fn OnCombatEnded
  (Widget|RemovefromParent (Variables|Default|GetW_CombatEndScreen))
  (Variables|Default|SetW_CombatEndScreen 0)
  (if (Variables|Default|GetAutoSelectOverworldMovementActions)
    (Actions|SetSelectedActions "/Game/TacticalCards/Blueprints/Core/Player/Actions/Overworld/BP_Action_SelectUnitInOverworld.BP_Action_SelectUnitInOverworld_C" "/Game/TacticalCards/Blueprints/Core/Player/Actions/Overworld/BP_Action_MoveUnitInOverworld.BP_Action_MoveUnitInOverworld_C")
    (else
      (Actions|SetSelectedActions))))

(fn OnUnitTurnStarted
  (params (Unit :type BP%20Unit%20Object%20Reference))
  (Utilities|IsValid (Variables|/Game/TacticalCards/Blueprints/Core/Units/BP_Unit.BP_Unit_C|GetAI Unit)
    (:Is%20Valid
      (if (!= (Utilities|GetClass (Variables|Actions|GetSelectedAction_LeftClick)) "/Game/TacticalCards/Blueprints/Core/Player/Actions/Combat/BP_Action_Combat_WaitForTurn.BP_Action_Combat_WaitForTurn_C")
        (Actions|SetSelectedActions "/Game/TacticalCards/Blueprints/Core/Player/Actions/Combat/BP_Action_Combat_WaitForTurn.BP_Action_Combat_WaitForTurn_C")))
    (:Is%20Not%20Valid
      (HoveredandSelected|SetSelectedTileandUnit (Variables|/Game/TacticalCards/Blueprints/Core/Units/BP_Unit.BP_Unit_C|GetIndex Unit) 0 false)
      (Actions|SetSelectedActions "/Game/TacticalCards/Blueprints/Core/Player/Actions/Combat/BP_Action_Combat_Move.BP_Action_Combat_Move_C")
      (Default|LinkUnittoAbilitiesList (Variables|/Game/TacticalCards/Blueprints/Core/Combat/Widgets/WBP_Combat.WBP_Combat_C|GetButtonList_Abilities (Variables|Default|GetW_Combat)) (Variables|Default|GetSelectedUnit)))))

(fn OnUnitTurnEnded
  (params (Unit :type BP%20Unit%20Object%20Reference))
  (HoveredandSelected|SetSelectedTileandUnit (Utilities|Struct|MakeIntPoint -999 -999) 0 false)
  (Default|LinkUnittoAbilitiesList (Variables|/Game/TacticalCards/Blueprints/Core/Combat/Widgets/WBP_Combat.WBP_Combat_C|GetButtonList_Abilities (Variables|Default|GetW_Combat))))

(fn OnSelectedAbilityChanged
  (params (Button :type WBP%20Button%20Ability%20Object%20Reference))
  (Utilities|IsValid Button
    (:Is%20Valid
      (Actions|SetSelectedActions "/Game/TacticalCards/Blueprints/Core/Player/Actions/Combat/BP_Action_Combat_CastAbility.BP_Action_Combat_CastAbility_C") ; Set mouse action to cast
      (bind _asbp_action_combat_cast_ability (Utilities|Casting|CastToBP_Action_Combat_CastAbility (Variables|Actions|GetSelectedAction_LeftClick)))
      (Default|SetAbility _asbp_action_combat_cast_ability (Variables|/Game/TacticalCards/Blueprints/Core/Combat/Abilities/Widgets/WBP_Button_Ability.WBP_Button_Ability_C|GetAbility Button)))
    (:Is%20Not%20Valid
      (if (!= (Utilities|GetClass (Variables|Actions|GetSelectedAction_LeftClick)) "/Game/TacticalCards/Blueprints/Core/Player/Actions/Combat/BP_Action_Combat_Move.BP_Action_Combat_Move_C")
        (Actions|SetSelectedActions "/Game/TacticalCards/Blueprints/Core/Player/Actions/Combat/BP_Action_Combat_Move.BP_Action_Combat_Move_C") ; Set mouse action to move
      ))))

(fn OnCombatFinishing
  (Actions|SetSelectedActions)
  (HoveredandSelected|SetSelectedTileandUnit (Utilities|Struct|MakeIntPoint -999 -999) 0 false)
  (Widget|RemovefromParent (Variables|Default|GetW_Combat))
  (Variables|Default|SetW_Combat 0)
  (bind _returnvalue (UserInterface|CreateWidget "/Game/TacticalCards/Blueprints/Core/Combat/Widgets/WBP_CombatEndScreen.WBP_CombatEndScreen_C" 0 self (Variables|/Game/TacticalCards/Blueprints/Core/Combat/BP_CombatSystem.BP_CombatSystem_C|GetTeamIndexThatWonLastCombat (Variables|References|GetCombatSystem))))
  (bind _output_get (Variables|Default|SetW_CombatEndScreen _returnvalue))
  (UserInterface|Viewport|AddtoPlayerScreen _output_get))

(fn SetHoveredUnitOverride
  (params (Unit :type BP%20Unit%20Object%20Reference))
  (Variables|Default|SetHoveredUnitOverride Unit)
  (HoveredandSelected|UpdateHoveredTileandUnit))

(fn CanHoverGround
  (bind _selectedaction_leftclick (Variables|Actions|GetSelectedAction_LeftClick))
  (bind _selectedaction_rightclick (Variables|Actions|GetSelectedAction_RightClick))
  (bind _returnvalue (Utilities|GetClass _selectedaction_rightclick))
  (bind _returnvalue_2 (Utilities|GetClass _selectedaction_leftclick))
  (bind _array (Utilities|Array|MakeArray _returnvalue_2 _returnvalue))
  (return (or (Utilities|Array|ContainsItem _array "/Game/TacticalCards/Blueprints/Core/Player/Actions/Overworld/BP_Action_AddRemoveUnitFromOverworld.BP_Action_AddRemoveUnitFromOverworld_C") (Utilities|Array|ContainsItem _array "/Game/TacticalCards/Blueprints/Core/Player/Actions/Overworld/BP_Action_MoveUnitInOverworld.BP_Action_MoveUnitInOverworld_C"))))

(fn CanHoverEmptySpace
  (return (Utilities|Array|ContainsItem (Utilities|Array|MakeArray (Utilities|GetClass (Variables|Actions|GetSelectedAction_LeftClick)) (Utilities|GetClass (Variables|Actions|GetSelectedAction_RightClick))) "/Game/TacticalCards/Blueprints/Core/Player/Actions/Grid/BP_Action_AddTile.BP_Action_AddTile_C")))