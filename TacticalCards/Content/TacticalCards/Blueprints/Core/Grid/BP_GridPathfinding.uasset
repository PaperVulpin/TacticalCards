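; BP_GridPathfinding runs A* pathfinding on the tactical grid, returning a path to a target or all tiles reachable within a cost limit.
; Neighbor and heuristic functions support square, hexagon and triangle grids, filtering tiles by type, occupancy and height.
; A cost-sorted open list favors straight steps over diagonals on ties.
; Searches run instantly or stepped through a delay gate, firing callbacks on data changes and completion.
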(event Custom|FindPathWithDelay
  (Utilities|FlowControl|Sequence
    (:then_0
      (goto _label_3 Open))
    (:then_1
      (Variables|Default|SetLoopStartTime (Math|DateTime|Now) :!label _label)
      (if (> (Utilities|Array|Length (Variables|Default|GetDiscoveredTileIndexes)) 0) :!label _label_2
        (bind _foundtargettile (CallFunction|AnalyzeNextDiscoveredTiled))
        (if _foundtargettile
          (bind _path (Utilities|GeneratePath))
          (Default|CallOnPathfindingCompleted _path)
          (else
            (if (> (Variables|Default|GetMaxMsPerFrame) 0.0) ; Do we have a limit?
              (if (< (Class|KismetMathLibrary|GetTotalMilliseconds (- (Math|DateTime|Now) (Variables|Default|GetLoopStartTime))) (Variables|Default|GetMaxMsPerFrame)) ; Still have time left?
                (goto _label_2)
                (else
                  _)))
            (if (not (> (Variables|Default|GetMaxMsPerFrame) 0.0))
              (Utilities|FlowControl|RetriggerableDelay (Variables|Default|GetDelayBetweenIterations))
              (Utilities|FlowControl|Gate true :!label _label_3
                (:Exit
                  (goto _label))))))
        (else
          (Default|CallOnPathfindingCompleted (select (Variables|Default|GetReturnReachableTiles) (Variables|Default|GetAnalyzedTileIndexes) (Utilities|Array|MakeArray))))))))

(event Custom|CloseDelayGate
  (Utilities|FlowControl|Gate true) ; enters at Close
)

(fn ConstructionScript)

(fn GetValidTileNeighbors
  (params (Index :type Int%20Point%20Structure) (IncludeDiagonals :type Boolean) (ValidTypes :type Array%20of%20E_TileTypes%20Enums :default "NewEnumerator0"))
  (bind _grid (Variables|Default|GetGrid))
  (bind _gridtiles (Variables|/Game/TacticalCards/Blueprints/Core/Grid/BP_Grid.BP_Grid_C|GetGridTiles _grid))
  (bind _output_get (LocalVariables|SetInputData (.Value (Utilities|Map|Find _gridtiles Index))))
  (bind _neighbors (Neighbors|GetNeighborIndexes Index IncludeDiagonals))
  (for _array_element _neighbors
    (bind _output_get_2 (LocalVariables|SetData (.Value (Utilities|Map|Find _gridtiles _array_element))))
    (if (Utilities|Array|ContainsItem ValidTypes (.type _output_get_2))
      (if (not (Utilities|IsValid (.unitontile _output_get_2)))
        (if (<= (Math|Float|Absolute(Float) (- (.Z (Class|KismetMathLibrary|BreakVector3f (.location (.transform _output_get_2)))) (.Z (Class|KismetMathLibrary|BreakVector3f (.location (.Transform (Utilities|Struct|BreakS_TileData _output_get))))))) (+ (.z (Variables|/Game/TacticalCards/Blueprints/Core/Grid/BP_Grid.BP_Grid_C|GetGridTileSize _grid)) 15.0))
          (Utilities|Array|Add (LocalVariables|GetReturn) (Utilities|Struct|MakeS_PathfindingData (.index _output_get_2) (CallFunction|GetTileTypeCost (.type _output_get_2)) 999999 999999 Index))))))
  (return (LocalVariables|GetReturn)))

(fn GetNeighborsIndexesforSquare
  (params (Index :type Int%20Point%20Structure) (IncludeDiagonals :type Boolean))
  (bind _intpoint (Utilities|Struct|MakeIntPoint 1 0))
  (bind _intpoint_2 (Utilities|Struct|MakeIntPoint 0 1))
  (bind _intpoint_3 (Utilities|Struct|MakeIntPoint -1 0))
  (bind _intpoint_4 (Utilities|Struct|MakeIntPoint 0 -1))
  (bind _returnvalue (+ Index _intpoint))
  (bind _returnvalue_2 (+ Index _intpoint_2))
  (bind _returnvalue_3 (+ Index _intpoint_3))
  (bind _returnvalue_4 (+ Index _intpoint_4))
  (bind _array (Utilities|Array|MakeArray _returnvalue _returnvalue_2 _returnvalue_3 _returnvalue_4))
  (if IncludeDiagonals
    (bind _output_get (LocalVariables|SetReturn _array))
    (Utilities|Array|AppendArray _output_get (Utilities|Array|MakeArray (+ Index (Utilities|Struct|MakeIntPoint 1 1)) (+ Index (Utilities|Struct|MakeIntPoint -1 1)) (+ Index (Utilities|Struct|MakeIntPoint -1 -1)) (+ Index (Utilities|Struct|MakeIntPoint 1 -1))))
    (return (LocalVariables|GetReturn))
    (else
      (return _array))))

(fn GetNeighborsIndexesforHexagon
  (params (Index :type Int%20Point%20Structure))
  (return (Utilities|Array|MakeArray (+ Index (Utilities|Struct|MakeIntPoint 1 1)) (+ Index (Utilities|Struct|MakeIntPoint 0 2)) (+ Index (Utilities|Struct|MakeIntPoint -1 1)) (+ Index (Utilities|Struct|MakeIntPoint -1 -1)) (+ Index (Utilities|Struct|MakeIntPoint 0 -2)) (+ Index (Utilities|Struct|MakeIntPoint 1 -1)))))

(fn GetNeighborsIndexesforTriangle
  (params (Index :type Int%20Point%20Structure) (IncludeDiagonals :type Boolean))
  (bind _output_get (LocalVariables|SetReturn (Utilities|Array|MakeArray (+ Index (Utilities|Struct|MakeIntPoint 0 -1)) (+ Index (Utilities|Struct|MakeIntPoint 0 1)))))
  (if (CallFunction|IsTriangleTileFacingUp Index)
    (Utilities|Array|Add _output_get (+ Index (Utilities|Struct|MakeIntPoint -1 0)))
    (else
      (Utilities|Array|Add _output_get (+ Index (Utilities|Struct|MakeIntPoint 1 0)))))
  (if (Variables|Default|GetIncludeDiagonals)
    (if (CallFunction|IsTriangleTileFacingUp Index)
      (Utilities|Array|AppendArray (LocalVariables|GetReturn) (Utilities|Array|MakeArray (+ Index (Utilities|Struct|MakeIntPoint 1 0)) (+ Index (Utilities|Struct|MakeIntPoint -1 2)) (+ Index (Utilities|Struct|MakeIntPoint -1 -2))))
      (else
        (Utilities|Array|AppendArray (LocalVariables|GetReturn) (Utilities|Array|MakeArray (+ Index (Utilities|Struct|MakeIntPoint -1 0)) (+ Index (Utilities|Struct|MakeIntPoint 1 2)) (+ Index (Utilities|Struct|MakeIntPoint 1 -2))))))
    (return (LocalVariables|GetReturn))
    (else
      (return _output_get))))

(fn GetNeighborIndexes
  (params (Index :type Int%20Point%20Structure) (IncludeDiagonals :type Boolean))
  (switch Utilities|FlowControl|Switch|SwitchonE_GridShape (Variables|/Game/TacticalCards/Blueprints/Core/Grid/BP_Grid.BP_Grid_C|GetGridShape (Variables|Default|GetGrid))
    (:NewEnumerator0
      (return (Neighbors|GetNeighborsIndexesforSquare Index IncludeDiagonals)))
    (:NewEnumerator1
      (return (Neighbors|GetNeighborsIndexesforTriangle Index IncludeDiagonals)))
    (:NewEnumerator2
      (return (Neighbors|GetNeighborsIndexesforHexagon Index)))))

(fn FindPath
  (params (Start :type Int%20Point%20Structure) (Target :type Int%20Point%20Structure) (Diagonals :type Boolean) (ValidTilesTypes :type Array%20of%20E_TileTypes%20Enums :default "NewEnumerator0") (Delay :type Float%20%28double-precision%29) (MaxMs :type Float%20%28double-precision%29) (ReturnReachables :type Boolean) (PathLength :type Integer))
  (bind _array (Utilities|Array|MakeArray))
  (Variables|Default|SetStartIndex Start)
  (Variables|Default|SetTargetIndex Target)
  (Variables|Default|SetIncludeDiagonals Diagonals)
  (Variables|Default|SetValidTilesTypes ValidTilesTypes)
  (Variables|Default|SetDelayBetweenIterations Delay)
  (Variables|Default|SetMaxMsPerFrame MaxMs)
  (Variables|Default|SetReturnReachableTiles ReturnReachables)
  (Variables|Default|SetMaxPathLength PathLength)
  (CallFunction|CloseDelayGate)
  (Utilities|ClearGeneratedData)
  (bind _isvalid (Utilities|IsInputDataValid))
  (if _isvalid
    (Utilities|DiscoverTile (Utilities|Struct|MakeS_PathfindingData (Variables|Default|GetStartIndex) 1 0 (Utilities|GetMinimumCostBetweenTwoTiles Start Target Diagonals) "(X=-999,Y=-999)"))
    (if (<= (Variables|Default|GetDelayBetweenIterations) 0.0)
      (while (> (Utilities|Array|Length (Variables|Default|GetDiscoveredTileIndexes)) 0)
        (bind _foundtargettile (CallFunction|AnalyzeNextDiscoveredTiled))
        (if _foundtargettile
          (bind _path (Utilities|GeneratePath))
          (Default|CallOnPathfindingCompleted _path)
          (return _path)))
      (Default|CallOnPathfindingCompleted (select (Variables|Default|GetReturnReachableTiles) (Variables|Default|GetAnalyzedTileIndexes) (Utilities|Array|MakeArray)))
      (return (select (Variables|Default|GetReturnReachableTiles) (Variables|Default|GetAnalyzedTileIndexes) (Utilities|Array|MakeArray)))
      (else
        (CallFunction|FindPathwithDelay)
        (return (Utilities|Array|MakeArray))))
    (else
      (Default|CallOnPathfindingCompleted _array)
      (return _array))))

(fn IsInputDataValid
  (bind _grid (Variables|Default|GetGrid))
  (bind _startindex (Variables|Default|GetStartIndex))
  (bind _targetindex (Variables|Default|GetTargetIndex))
  (bind _gridtiles (Variables|/Game/TacticalCards/Blueprints/Core/Grid/BP_Grid.BP_Grid_C|GetGridTiles _grid))
  (bind _value (Utilities|Map|Find _gridtiles _targetindex))
  (bind (_type _unitontile) (Utilities|Struct|BreakS_TileData _value))
  (if (!= _startindex _targetindex)
    (if (Default|IsTileWalkable (Variables|Default|GetGrid) _startindex)
      (if (not (Variables|Default|GetReturnReachableTiles))
        (if (Default|IsTileWalkable (Variables|Default|GetGrid) _targetindex)
          (if (<= (Utilities|GetMinimumCostBetweenTwoTiles (Variables|Default|GetStartIndex) _targetindex (Variables|Default|GetIncludeDiagonals)) (Variables|Default|GetMaxPathLength))
            (if (Utilities|Array|ContainsItem (Variables|Default|GetValidTilesTypes) _type)
              (if (not (Utilities|IsValid _unitontile))
                (return true)
                (else
                  _)))
            (return false)
            (else
              _)))
        (else
          (return true)))))
  (return false))

(fn DiscoverTile
  (params (TilePathData :type S%20Pathfinding%20Data%20Structure))
  (bind _index (Utilities|Struct|BreakS_PathfindingData TilePathData))
  (Utilities|Map|Add (Variables|Default|GetPathfindingData) _index TilePathData)
  (Utilities|InsertTileinDiscoveredArray TilePathData)
  (Default|CallOnPathfindingDataUpdated _index))

(fn GetMinimumCostBetweenTwoTiles
  (params (Index1 :type Int%20Point%20Structure) (Index2 :type Int%20Point%20Structure) (Diagonals :type Boolean))
  (bind (_x _y) (Utilities|Struct|BreakIntPoint Index1))
  (bind _x_2 (Utilities|Struct|BreakIntPoint Index2))
  (bind _returnvalue (- Index1 Index2))
  (bind _returnvalue_2 (- Index1 Index2))
  (bind _returnvalue_3 (- Index1 Index2))
  (bind _returnvalue_4 (Math|Integer|Absolute(Integer) (.x _returnvalue_2)))
  (bind _returnvalue_5 (Math|Integer|Absolute(Integer) (.y _returnvalue_2)))
  (bind _isfacingup (CallFunction|IsTriangleTileFacingUp (Utilities|Struct|MakeIntPoint _x _y)))
  (bind _returnvalue_6 (Math|Integer|Absolute(Integer) (.x _returnvalue)))
  (bind _returnvalue_7 (< _x_2 _x))
  (bind _returnvalue_8 (+ _returnvalue_4 _returnvalue_5))
  (bind _returnvalue_9 (select _returnvalue_7 -1 1))
  (switch Utilities|FlowControl|Switch|SwitchonE_GridShape (Variables|/Game/TacticalCards/Blueprints/Core/Grid/BP_Grid.BP_Grid_C|GetGridShape (Variables|Default|GetGrid))
    (:NewEnumerator0
      (if Diagonals
        (return (Math|Integer|Max(Integer) _returnvalue_4 _returnvalue_5))
        (else
          (return _returnvalue_8))))
    (:NewEnumerator1
      (if Diagonals
        (return (/ _returnvalue_8 2))
        (else
          (LocalVariables|SetX (Math|Integer|Absolute(Integer) (.x _returnvalue_3)))
          (LocalVariables|SetY (Math|Integer|Absolute(Integer) (.y _returnvalue_3)))
          (if (select _isfacingup (select _returnvalue_7 (<= (- (LocalVariables|GetX) 1) (LocalVariables|GetY)) (<= (LocalVariables|GetX) (LocalVariables|GetY))) (select _returnvalue_7 (<= (LocalVariables|GetX) (LocalVariables|GetY)) (<= (- (LocalVariables|GetX) 1) (LocalVariables|GetY)))) ; Is part of the normal zone?
            (return (+ (LocalVariables|GetX) (LocalVariables|GetY)))
            (elif (CallFunction|IsTriangleTileFacingUp (Utilities|Struct|MakeIntPoint (LocalVariables|GetX) (LocalVariables|GetY))) ; Is tile facing up?
              (return (* (LocalVariables|GetX) 2))
              (else
                (return (+ (* (LocalVariables|GetX) 2) (select _isfacingup _returnvalue_9 (* _returnvalue_9 -1))))))))))
    (:NewEnumerator2
      (return (+ _returnvalue_6 (Math|Integer|Max(Integer) (/ (- (Math|Integer|Absolute(Integer) (.y _returnvalue)) _returnvalue_6) 2)))))))

(fn AnalyzeNextDiscoveredTiled
  (bind _tilepathdata (Utilities|PullCheapestTileOutOfDiscoverdList))
  (bind _output_get (Variables|Default|SetCurrentDiscoveredTile _tilepathdata))
  (Default|CallOnPathfindingDataUpdated (.Index (Utilities|Struct|BreakS_PathfindingData _output_get)))
  (bind _neighbors (Neighbors|GetValidTileNeighbors (.Index (Utilities|Struct|BreakS_PathfindingData _output_get)) (Variables|Default|GetIncludeDiagonals) (Variables|Default|GetValidTilesTypes)))
  (bind _output_get_2 (Variables|Default|SetCurrentNeighbors _neighbors))
  (while (> (Utilities|Array|Length _output_get_2) 0)
    (bind _istargettile (CallFunction|DiscoverNextNeighbor))
    (if _istargettile
      (return true) ; This neighbor is the target.
    ))
  (return false) ; None of the neighbors were the target tile.
)

(fn GeneratePath
  (bind _invertedpath (LocalVariables|GetInvertedPath))
  (bind _return (LocalVariables|GetReturn))
  (bind _output_get (LocalVariables|SetCurrent (Variables|Default|GetTargetIndex)))
  (while (!= _output_get (Variables|Default|GetStartIndex))
    (Utilities|Array|Add _invertedpath _output_get)
    (LocalVariables|SetCurrent (Utilities|Struct|BreakS_PathfindingData (.Value (Utilities|Map|Find (Variables|Default|GetPathfindingData) _output_get)))))
  (bind _arrayelement (Utilities|Array|ReverseforEachLoop _invertedpath)
    (:LoopBody
      (Utilities|Array|Add _return _arrayelement))
    (:Completed
      (return _return))))

(fn PullCheapestTileOutOfDiscoverdList
  (bind _discoveredtileindexes (Variables|Default|GetDiscoveredTileIndexes))
  (bind _output_get (LocalVariables|SetTileIndex (Utilities|Array|Get(acopy) _discoveredtileindexes)))
  (Utilities|Array|RemoveIndex (Variables|Default|GetDiscoveredTileSortingCosts))
  (Utilities|Array|RemoveIndex _discoveredtileindexes)
  (Utilities|Array|Add (Variables|Default|GetAnalyzedTileIndexes) _output_get)
  (return (.Value (Utilities|Map|Find (Variables|Default|GetPathfindingData) _output_get))))

(fn DiscoverNextNeighbor
  (bind _currentneighbors (Variables|Default|GetCurrentNeighbors))
  (bind _output_get (Variables|Default|SetCurrentNeighbor (Utilities|Array|Get(acopy) _currentneighbors)))
  (Utilities|Array|RemoveIndex _currentneighbors)
  (if (not (Utilities|Array|ContainsItem (Variables|Default|GetAnalyzedTileIndexes) (.Index (Utilities|Struct|BreakS_PathfindingData _output_get)))) ; Not already analyzed
    (bind _output_get_2 (LocalVariables|SetCostFromStart (+ (Utilities|Struct|BreakS_PathfindingData (Variables|Default|GetCurrentDiscoveredTile)) (.CostToEnterTile (Utilities|Struct|BreakS_PathfindingData (Variables|Default|GetCurrentNeighbor))))))
    (if (<= _output_get_2 (Variables|Default|GetMaxPathLength))
      (bind _output_get_3 (LocalVariables|SetIndexInDiscovered (Utilities|Array|FindItem (Variables|Default|GetDiscoveredTileIndexes) (.Index (Utilities|Struct|BreakS_PathfindingData (Variables|Default|GetCurrentNeighbor))))))
      (if (== _output_get_3 -1) ; New Neighbor?
        _
        (else
          (bind _output_get_4 (Variables|Default|SetCurrentNeighbor (.Value (Utilities|Map|Find (Variables|Default|GetPathfindingData) (.Index (Utilities|Struct|BreakS_PathfindingData (Variables|Default|GetCurrentNeighbor)))))))
          (if (< (LocalVariables|GetCostFromStart) (Utilities|Struct|BreakS_PathfindingData _output_get_4)) ; Found better path to neighbor?
            (Utilities|Array|RemoveIndex (Variables|Default|GetDiscoveredTileIndexes) (LocalVariables|GetIndexInDiscovered))
            (Utilities|Array|RemoveIndex (Variables|Default|GetDiscoveredTileSortingCosts) (LocalVariables|GetIndexInDiscovered))
            (else
              (return false)))))
      (Utilities|DiscoverTile (Utilities|Struct|MakeS_PathfindingData (.Index (Utilities|Struct|BreakS_PathfindingData (Variables|Default|GetCurrentNeighbor))) (.CostToEnterTile (Utilities|Struct|BreakS_PathfindingData (Variables|Default|GetCurrentNeighbor))) (LocalVariables|GetCostFromStart) (Utilities|GetMinimumCostBetweenTwoTiles (.Index (Utilities|Struct|BreakS_PathfindingData (Variables|Default|GetCurrentNeighbor))) (Variables|Default|GetTargetIndex) (Variables|Default|GetIncludeDiagonals)) (Utilities|Struct|BreakS_PathfindingData (Variables|Default|GetCurrentDiscoveredTile))))
      (if (Class|KismetMathLibrary|EqualIntPointIntPoint (Utilities|Struct|BreakS_PathfindingData (Variables|Default|GetCurrentNeighbor)) (Variables|Default|GetTargetIndex))
        (return true)
        (else
          (return false)))
      (else
        (return false)))
    (else
      (return false))))

(fn InsertTileinDiscoveredArray
  (params (TileData :type S%20Pathfinding%20Data%20Structure))
  (bind _discoveredtilesortingcosts (Variables|Default|GetDiscoveredTileSortingCosts))
  (bind _discoveredtileindexes (Variables|Default|GetDiscoveredTileIndexes))
  (bind _output_get (LocalVariables|SetSortingCost (CallFunction|GetTileSortingCost TileData)))
  (if (== (Utilities|Array|Length _discoveredtilesortingcosts) 0)
    (Utilities|Array|Add _discoveredtilesortingcosts _output_get :!label _label)
    (Utilities|Array|Add _discoveredtileindexes (Utilities|Struct|BreakS_PathfindingData TileData))
    (elif (>= _output_get (Utilities|Array|Get(acopy) _discoveredtilesortingcosts (Utilities|Array|LastIndex _discoveredtilesortingcosts)))
      (goto _label)
      (else
        (bind (_array_element _array_index) (Utilities|Array|ForEachLoopwithBreak _discoveredtilesortingcosts :!label _label_2)
          (:LoopBody
            (if (>= _array_element _output_get)
              (Utilities|Array|Insert _discoveredtilesortingcosts _output_get _array_index)
              (Utilities|Array|Insert _discoveredtileindexes (Utilities|Struct|BreakS_PathfindingData TileData) _array_index)
              (goto _label_2 Break))))))))

(fn ClearGeneratedData
  (Utilities|Map|Clear (Variables|Default|GetPathfindingData))
  (Utilities|Array|Clear (Variables|Default|GetDiscoveredTileSortingCosts))
  (Utilities|Array|Clear (Variables|Default|GetDiscoveredTileIndexes))
  (Utilities|Array|Clear (Variables|Default|GetAnalyzedTileIndexes))
  (Default|CallOnPathfindingDataCleared))

(fn IsDiagonal
  (params (Index1 :type Int%20Point%20Structure) (Index2 :type Int%20Point%20Structure))
  (bind _neighbors (Neighbors|GetNeighborIndexes Index1 false))
  (return (not (Utilities|Array|ContainsItem _neighbors Index2))))

(fn GetTileSortingCost
  (params (TileData :type S%20Pathfinding%20Data%20Structure%20%28by%20ref%29))
  (bind (_index _costfromstart _minimuncosttotarget _previousindex) (Utilities|Struct|BreakS_PathfindingData TileData))
  (return (+ (* (+ _costfromstart _minimuncosttotarget) 2) (CallFunction|IsDiagonal _index _previousindex))))

(fn GetPathCost
  (params (Path :type Array%20of%20Int%20Point%20Structures))
  (LocalVariables|SetRet 0)
  (for _array_element Path
    (LocalVariables|SetRet (+ (LocalVariables|GetRet) (CallFunction|GetTileTypeCost (Utilities|Struct|BreakS_TileData (.Value (Utilities|Map|Find (Variables|/Game/TacticalCards/Blueprints/Core/Grid/BP_Grid.BP_Grid_C|GetGridTiles (Variables|Default|GetGrid)) _array_element)))))))
  (return (LocalVariables|GetRet)))