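; BP_GridVisual renders the tactical grid's tiles through two child BP_GridMeshInst instanced-mesh actors: a flat overlay offset from the ground and a tactical 3D view.
; Tile updates re-add instances by type; tactical tiles stretch vertically from the lowest tile height.
; Toggling tactical mode hides "NotTactical"-tagged actors, switches collision, and lazily regenerates tactical instances flagged stale while hidden or after the lowest height changes.
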(event EventBeginPlay
  (Actor|Tick|SetActorTickEnabled false))

(event Collision|EventActorBeginOverlap
  (params (OtherActor :type Actor%20Object%20Reference)))

(event EventTick
  (params (DeltaSeconds :type Float%20%28single-precision%29)))

(fn ConstructionScript)

(fn InitializeGridVisual
  (params (Grid :type BP%20Grid%20Object%20Reference))
  (Variables|Default|SetGrid Grid)
  (bind _output_get (Variables|Default|SetGridMeshInst (.AsBP%20Grid%20Mesh%20Inst (Utilities|Casting|CastToBP_GridMeshInst (Variables|/Script/Engine.ChildActorComponent|GetChildActor (Variables|Default|GetChildActor_GridMeshInst))))))
  (Variables|Default|SetGridMeshInst_Tactical (.AsBP%20Grid%20Mesh%20Inst (Utilities|Casting|CastToBP_GridMeshInst (Variables|/Script/Engine.ChildActorComponent|GetChildActor (Variables|Default|GetChildActor_GridMeshInst_Tactical)))))
  (Default|InitializeGridMeshInst _output_get (.FlatMesh (Utilities|Struct|BreakS_GridShapeData (Default|GetCurrentShapeData (Variables|Default|GetGrid)))) (.FlatMaterial (Utilities|Struct|BreakS_GridShapeData (Default|GetCurrentShapeData (Variables|Default|GetGrid)))) false "QueryOnly")
  (Default|InitializeGridMeshInst (Variables|Default|GetGridMeshInst_Tactical) (.Mesh (Utilities|Struct|BreakS_GridShapeData (Default|GetCurrentShapeData (Variables|Default|GetGrid)))) (.MeshMaterial (Utilities|Struct|BreakS_GridShapeData (Default|GetCurrentShapeData (Variables|Default|GetGrid)))) true "QueryOnly")
  (Transformation|SetActorLocation "0, 0, 0" false false) ; Center grid in world
  (CallFunction|SetOffsetfromGround (Variables|Default|GetOffsetFromGround))
  (CallFunction|SetGridLowesttoZ 999999.0)
  (CallFunction|SetIsTactical (Variables|Default|GetIsTactical)))

(fn SetOffsetfromGround
  (params (Offset :type Float%20%28double-precision%29))
  (Variables|Default|SetOffsetFromGround Offset)
  (Transformation|SetRelativeLocation (Variables|Default|GetChildActor_GridMeshInst) (Math|Vector|MakeVector 0.0 0.0 (Variables|Default|GetOffsetFromGround)) false false))

(fn DestroyGridVisual
  (bind _gridmeshinst_tactical (Variables|Default|GetGridMeshInst_Tactical))
  (bind _gridmeshinst (Variables|Default|GetGridMeshInst))
  (Utilities|FlowControl|Sequence
    (:then_0
      (Utilities|IsValid _gridmeshinst
        (:Is%20Valid
          (Default|ClearInstances _gridmeshinst))))
    (:then_1
      (Utilities|IsValid _gridmeshinst_tactical
        (:Is%20Valid
          (Default|ClearInstances _gridmeshinst_tactical))))
    (:then_2
      (CallFunction|SetGridLowesttoZ 999999.0))))

(fn UpdateTileVisual
  (params (Data :type S%20Tile%20Data%20Structure))
  (bind _gridmeshinst (Variables|Default|GetGridMeshInst))
  (Utilities|FlowControl|Sequence
    (:then_0
      (Default|RemoveInstance _gridmeshinst (.index Data))
      (if (CallFunction|IsTileTypeWalkable (.type Data))
        (Default|AddInstance _gridmeshinst (.index Data) (.transform Data) (.states Data) (.type Data))))
    (:then_1
      (CallFunction|UpdateTileVisualTactical Data))))

(fn UpdateTileVisualTactical
  (params (Data :type S%20Tile%20Data%20Structure))
  (bind _gridmeshinst_tactical (Variables|Default|GetGridMeshInst_Tactical))
  (bind _grid (Variables|Default|GetGrid))
  (bind (_location _rotation _scale) (Math|Transform|BreakTransform (.transform Data)))
  (bind _location_2 (Math|Transform|BreakTransform (.transform Data)))
  (bind _returnvalue (Default|GetCurrentShapeData _grid))
  (bind _meshsize (Utilities|Struct|BreakS_GridShapeData _returnvalue))
  (bind _z (Class|KismetMathLibrary|BreakVector3f _meshsize))
  (Utilities|FlowControl|Sequence
    (:then_0
      (if (< (.z _location_2) (Variables|Default|GetGridLowestZ))
        (CallFunction|SetGridLowesttoZ (.z _location_2))))
    (:then_1
      (if (Variables|Default|GetIsTactical)
        (Default|RemoveInstance _gridmeshinst_tactical (.index Data))
        (if (Utilities|Enum|NotEqual(Enum) (.type Data) "NewEnumerator0")
          (Default|AddInstance _gridmeshinst_tactical (.index Data) (Math|Transform|MakeTransform _location _rotation (Math|Vector|MakeVector (.x _scale) (.y _scale) (/ (+ (- (.Z (Class|KismetMathLibrary|BreakVector3f _location)) (Variables|Default|GetGridLowestZ)) _z) _z))) (.states Data) (.type Data)))
        (else
          (Variables|Default|SetNeedToReGenerateTacticalOnNextEnable true))))))

(fn SetGridLowesttoZ
  (params (GridLowestZ :type Float%20%28double-precision%29))
  (Variables|Default|SetGridLowestZ GridLowestZ)
  (Variables|Default|SetNeedToReGenerateTacticalOnNextEnable true))

(fn SetIsTactical
  (params (Tactical :type Boolean))
  (bind _grid (Variables|Default|GetGrid))
  (bind _gridmeshinst_tactical (Variables|Default|GetGridMeshInst_Tactical))
  (bind _output_get (Variables|Default|SetIsTactical Tactical))
  (Development|SetHiddeninGame (Variables|Default|GetChildActor_GridMeshInst_Tactical) (not _output_get) false)
  (bind _outactors (Actor|GetAllActorswithTag "NotTactical"))
  (for _array_element _outactors
    (Rendering|SetActorHiddenInGame _array_element (Variables|Default|GetIsTactical)))
  (Utilities|FlowControl|Sequence
    (:then_0
      (if (and (Variables|Default|GetIsTactical) (Variables|Default|GetNeedToReGenerateTacticalOnNextEnable))
        (Variables|Default|SetNeedToReGenerateTacticalOnNextEnable false)
        (Utilities|IsValid _grid
          (:Is%20Valid
            (bind _values (Utilities|Map|Values (Variables|/Game/TacticalCards/Blueprints/Core/Grid/BP_Grid.BP_Grid_C|GetGridTiles _grid)))
            (for _array_element_2 _values
              (CallFunction|UpdateTileVisual _array_element_2))))))
    (:then_1
      (Utilities|IsValid _gridmeshinst_tactical
        (:Is%20Valid
          (Collision|SetCollisionEnabled (Variables|/Game/TacticalCards/Blueprints/Core/Grid/Utilities/BP_GridMeshInst.BP_GridMeshInst_C|GetInstancedStaticMesh _gridmeshinst_tactical) (select (Variables|Default|GetIsTactical) "QueryOnly" "NoCollision")))))))