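; Manager for overworld unit groups that syncs hover and movement across members and turns group meetings into combat.
; Encounter groups wander and cluster around the mover's target, while other groups follow in a chain, unbinding events during propagation to avoid recursion.
; Reaching an encounter saves positions, disables bystanders and quick-starts grid combat with AI-controlled encounter units.
; Afterwards it destroys losing non-player units, heals the others, restores positions and resumes wandering.
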(event EventBeginPlay)

(event Collision|EventActorBeginOverlap
  (params (OtherActor :type Actor%20Object%20Reference)))

(event EventTick
  (params (DeltaSeconds :type Float%20%28single-precision%29)))

(fn ConstructionScript)

(fn AddUnittoGroup
  (params (Unit :type BP%20Unit%20Object%20Reference) (GroupID :type Integer))
  (if (!= (Variables|/Game/TacticalCards/Blueprints/Core/Units/BP_Unit.BP_Unit_C|GetOverworldGroupID Unit) GroupID)
    (Add/Remove|RemoveUnitfromCurrentGroup Unit)
    (if (!= GroupID -999)
      (bind _output_get (LocalVariables|SetGroup (.Value (Utilities|Map|Find (Variables|Default|GetUnitGroups) GroupID))))
      (Utilities|Array|Add (Utilities|Struct|BreakS_OverworldUnitGroup _output_get) Unit)
      (Utilities|Struct|SetmembersinS_OverworldUnitGroup (LocalVariables|GetGroup) GroupID)
      (Utilities|Map|Add (Variables|Default|GetUnitGroups) GroupID (LocalVariables|GetGroup))
      (Variables|/Game/TacticalCards/Blueprints/Core/Units/BP_Unit.BP_Unit_C|SetOverworldGroupID Unit GroupID)
      (Game|BindEventtoOnDestroyed Unit (EventDispatchers|CreateEvent :!event OnUnitDestroyed))
      (EventDispatchers|BindEventtoOnUnitHoveredChanged Unit (EventDispatchers|CreateEvent :!event OnUnitHoveredChanged))
      (EventDispatchers|BindEventtoOnUnitStartedWalkinginOverworld Unit (EventDispatchers|CreateEvent :!event OnUnitStartedWalkinginOverworld))
      (EventDispatchers|BindEventtoOnUnitReachedinOverworld Unit (EventDispatchers|CreateEvent :!event OnUnitReachedUnitinOverworld)))))

(fn RemoveUnitfromCurrentGroup
  (params (Unit :type BP%20Unit%20Object%20Reference))
  (if (!= -999 (Variables|/Game/TacticalCards/Blueprints/Core/Units/BP_Unit.BP_Unit_C|GetOverworldGroupID Unit))
    (bind _output_get (LocalVariables|SetGroup (.Value (Utilities|Map|Find (Variables|Default|GetUnitGroups) (Variables|/Game/TacticalCards/Blueprints/Core/Units/BP_Unit.BP_Unit_C|GetOverworldGroupID Unit)))))
    (Utilities|Array|RemoveItem (Utilities|Struct|BreakS_OverworldUnitGroup _output_get) Unit)
    (if (> (Utilities|Array|Length (Utilities|Struct|BreakS_OverworldUnitGroup _output_get)) 0)
      (Utilities|Map|Add (Variables|Default|GetUnitGroups) (Variables|/Game/TacticalCards/Blueprints/Core/Units/BP_Unit.BP_Unit_C|GetOverworldGroupID Unit) (LocalVariables|GetGroup))
      (else
        (Utilities|Map|Remove (Variables|Default|GetUnitGroups) (Variables|/Game/TacticalCards/Blueprints/Core/Units/BP_Unit.BP_Unit_C|GetOverworldGroupID Unit))))
    (Variables|/Game/TacticalCards/Blueprints/Core/Units/BP_Unit.BP_Unit_C|SetOverworldGroupID Unit -999)
    (EventDispatchers|UnbindEventfromOnUnitHoveredChanged Unit (EventDispatchers|CreateEvent :!event OnUnitHoveredChanged))
    (EventDispatchers|UnbindEventfromOnUnitStartedWalkinginOverworld Unit (EventDispatchers|CreateEvent :!event OnUnitStartedWalkinginOverworld))
    (EventDispatchers|UnbindEventfromOnUnitReachedinOverworld Unit (EventDispatchers|CreateEvent :!event OnUnitReachedUnitinOverworld))))

(fn OnUnitDestroyed
  (params (DestroyedActor :type Actor%20Object%20Reference))
  (bind _asbp_unit (Utilities|Casting|CastToBP_Unit DestroyedActor))
  (Add/Remove|RemoveUnitfromCurrentGroup _asbp_unit))

(fn OnUnitHoveredChanged
  (params (Unit :type BP%20Unit%20Object%20Reference))
  (bind _overworldgroupid (Variables|/Game/TacticalCards/Blueprints/Core/Units/BP_Unit.BP_Unit_C|GetOverworldGroupID Unit))
  (bind _unitgroups (Variables|Default|GetUnitGroups))
  (bind (_value _returnvalue) (Utilities|Map|Find _unitgroups _overworldgroupid))
  (if (not (Variables|/Game/TacticalCards/Blueprints/Core/Combat/BP_CombatSystem.BP_CombatSystem_C|GetIsInCombat (Variables|Default|GetCombatSystem)))
    (if _returnvalue
      (bind _output_get (LocalVariables|SetGroup _value))
      (for _array_element (.Units (Utilities|Struct|BreakS_OverworldUnitGroup _output_get))
        (bind _output_get_2 (LocalVariables|SetU _array_element))
        (if (!= _output_get_2 Unit)
          (EventDispatchers|UnbindEventfromOnUnitHoveredChanged (LocalVariables|GetU) (EventDispatchers|CreateEvent :!event OnUnitHoveredChanged))
          (Default|SetIsHovered (LocalVariables|GetU) (Variables|/Game/TacticalCards/Blueprints/Core/Units/BP_Unit.BP_Unit_C|GetIsHovered Unit))
          (EventDispatchers|BindEventtoOnUnitHoveredChanged (LocalVariables|GetU) (EventDispatchers|CreateEvent :!event OnUnitHoveredChanged)))))))

(fn OnUnitStartedWalkinginOverworld
  (params (Unit :type BP%20Unit%20Object%20Reference))
  (if (Utilities|Struct|BreakS_OverworldUnitGroup (.Value (Utilities|Map|Find (Variables|Default|GetUnitGroups) (Variables|/Game/TacticalCards/Blueprints/Core/Units/BP_Unit.BP_Unit_C|GetOverworldGroupID Unit))))
    (for _array_element (Utilities|Struct|BreakS_OverworldUnitGroup (.Value (Utilities|Map|Find (Variables|Default|GetUnitGroups) (Variables|/Game/TacticalCards/Blueprints/Core/Units/BP_Unit.BP_Unit_C|GetOverworldGroupID Unit))))
      (bind _output_get (LocalVariables|SetU _array_element))
      (if (!= _output_get Unit)
        (EventDispatchers|UnbindEventfromOnUnitStartedWalkinginOverworld (LocalVariables|GetU) (EventDispatchers|CreateEvent :!event OnUnitStartedWalkinginOverworld))
        (bind _randomlocation (Default|GetRandomReachableLocationinRadius (LocalVariables|GetU) (Variables|/Game/TacticalCards/Blueprints/Core/Units/BP_Unit.BP_Unit_C|GetTargetLocationInOverworld Unit) "(X=25.000000,Y=100.000000)"))
        (Default|EventMoveUnitinOverworld (LocalVariables|GetU) _randomlocation 0 false)
        (EventDispatchers|BindEventtoOnUnitStartedWalkinginOverworld (LocalVariables|GetU) (EventDispatchers|CreateEvent :!event OnUnitStartedWalkinginOverworld))))
    (else
      (LocalVariables|SetPreviousUnitInChain Unit)
      (for _array_element_2 (Utilities|Struct|BreakS_OverworldUnitGroup (.Value (Utilities|Map|Find (Variables|Default|GetUnitGroups) (Variables|/Game/TacticalCards/Blueprints/Core/Units/BP_Unit.BP_Unit_C|GetOverworldGroupID Unit))))
        (bind _output_get_2 (LocalVariables|SetU _array_element_2))
        (if (!= _output_get_2 Unit)
          (EventDispatchers|UnbindEventfromOnUnitStartedWalkinginOverworld (LocalVariables|GetU) (EventDispatchers|CreateEvent :!event OnUnitStartedWalkinginOverworld))
          (Default|EventMoveUnitinOverworld (LocalVariables|GetU) "0, 0, 0" (LocalVariables|GetPreviousUnitInChain) false)
          (LocalVariables|SetPreviousUnitInChain (LocalVariables|GetU))
          (EventDispatchers|BindEventtoOnUnitStartedWalkinginOverworld (LocalVariables|GetU) (EventDispatchers|CreateEvent :!event OnUnitStartedWalkinginOverworld)))))))

(fn SetGroupIsEncounter
  (params (IsEncounter :type Boolean) (GroupID :type Integer))
  (bind _unitgroups (Variables|Default|GetUnitGroups))
  (bind (_value _returnvalue) (Utilities|Map|Find _unitgroups GroupID))
  (if _returnvalue
    (bind _output_get (LocalVariables|SetGroup _value))
    (if (!= (Utilities|Struct|BreakS_OverworldUnitGroup _output_get) IsEncounter)
      (Utilities|Struct|SetmembersinS_OverworldUnitGroup (LocalVariables|GetGroup) IsEncounter)
      (Utilities|Map|Add (Variables|Default|GetUnitGroups) GroupID (LocalVariables|GetGroup))
      (for _array_element (.Units (Utilities|Struct|BreakS_OverworldUnitGroup (LocalVariables|GetGroup)))
        (Default|EventStopMovingUnitinOverworld _array_element))
      (if (.IsEncounter (Utilities|Struct|BreakS_OverworldUnitGroup (LocalVariables|GetGroup)))
        (Default|EventMoveUnitinOverworld (Utilities|Array|Get(acopy) (.Units (Utilities|Struct|BreakS_OverworldUnitGroup (LocalVariables|GetGroup)))) "0, 0, 0" 0 true)))))

(fn SetCombatSystem
  (params (CombatSystem :type BP%20Combat%20System%20Object%20Reference))
  (bind _output_get (Variables|Default|SetCombatSystem CombatSystem))
  (EventDispatchers|BindEventtoOnCombatEnded _output_get (EventDispatchers|CreateEvent :!event OnCombatEnded)))

(fn OnUnitReachedUnitinOverworld
  (params (Unit :type BP%20Unit%20Object%20Reference))
  (bind _unitgroups (Variables|Default|GetUnitGroups))
  (LocalVariables|SetGroup1 (.Value (Utilities|Map|Find _unitgroups (Variables|/Game/TacticalCards/Blueprints/Core/Units/BP_Unit.BP_Unit_C|GetOverworldGroupID Unit))))
  (LocalVariables|SetGroup2 (.Value (Utilities|Map|Find _unitgroups (Variables|/Game/TacticalCards/Blueprints/Core/Units/BP_Unit.BP_Unit_C|GetOverworldGroupID (Variables|/Game/TacticalCards/Blueprints/Core/Units/BP_Unit.BP_Unit_C|GetUnitToFollowInOverworld Unit)))))
  (if (Math|Boolean|ANDBoolean (!= (.GroupID (Utilities|Struct|BreakS_OverworldUnitGroup (LocalVariables|GetGroup1))) (.GroupID (Utilities|Struct|BreakS_OverworldUnitGroup (LocalVariables|GetGroup2)))) (not (.IsEncounter (Utilities|Struct|BreakS_OverworldUnitGroup (LocalVariables|GetGroup1)))) (.IsEncounter (Utilities|Struct|BreakS_OverworldUnitGroup (LocalVariables|GetGroup2))))
    (CallFunction|TriggerEncounter (Utilities|Array|MakeArray (LocalVariables|GetGroup1) (LocalVariables|GetGroup2)))))

(fn TriggerEncounter
  (params (Groups :type Array%20of%20S%20Overworld%20Unit%20Group%20Structures))
  (if (not (Variables|/Game/TacticalCards/Blueprints/Core/Combat/BP_CombatSystem.BP_CombatSystem_C|GetIsInCombat (Variables|Default|GetCombatSystem)))
    (Utilities|FlowControl|Sequence
      (:then_0
        (Utilities|Map|Clear (Variables|Default|GetUnitPositionsWhenCombatStarted))
        (bind _values (Utilities|Map|Values (Variables|Default|GetUnitGroups)))
        (for _array_element _values
          (for _array_element_2 (Utilities|Struct|BreakS_OverworldUnitGroup _array_element)
            (Utilities|Map|Add (Variables|Default|GetUnitPositionsWhenCombatStarted) _array_element_2 (Transformation|GetActorLocation _array_element_2))
            (if (not (Utilities|Array|ContainsItem Groups _array_element))
              (Default|DisableUnit _array_element_2) ; Disable units that are not in combat.
            )))
        (LocalVariables|SetGridData (Utilities|Struct|MakeS_QuickCombat_Grid true (Transformation|GetActorLocation (Utilities|Array|Get(acopy) (Utilities|Struct|BreakS_OverworldUnitGroup (Utilities|Array|Get(acopy) Groups)))) "100.000000,100.000000,5.000000" (Utilities|Struct|MakeIntPoint (Math|Random|RandomIntegerinRange 10 20) (Math|Random|RandomIntegerinRange 10 20)) "NewEnumerator2" true))
        (for _array_element_3 Groups
          (Utilities|Array|Add (LocalVariables|GetUnitTeams) (Utilities|Struct|MakeS_UnitArray (.Units (Utilities|Struct|BreakS_OverworldUnitGroup _array_element_3))))
          (if (.IsEncounter (Utilities|Struct|BreakS_OverworldUnitGroup _array_element_3))
            (Utilities|Array|AppendArray (LocalVariables|GetControlledByAI) (.Units (Utilities|Struct|BreakS_OverworldUnitGroup _array_element_3)))))
        (Default|QuickStartCombat (Variables|Default|GetCombatSystem) (LocalVariables|GetGridData) (Utilities|Struct|MakeS_QuickCombat_UnitTeams (LocalVariables|GetUnitTeams) (LocalVariables|GetControlledByAI) (Utilities|Map|MakeMap)) self)))))

(fn OnCombatEnded
  (bind _combatsystem (Variables|Default|GetCombatSystem))
  (bind _teamindexthatwonlastcombat (Variables|/Game/TacticalCards/Blueprints/Core/Combat/BP_CombatSystem.BP_CombatSystem_C|GetTeamIndexThatWonLastCombat _combatsystem))
  (if (== (Variables|/Game/TacticalCards/Blueprints/Core/Combat/BP_CombatSystem.BP_CombatSystem_C|GetObjectThatStartedCombat (Variables|Default|GetCombatSystem)) self)
    (bind _keys (Utilities|Map|Keys (Variables|/Game/TacticalCards/Blueprints/Core/Combat/BP_CombatSystem.BP_CombatSystem_C|GetUnitTeams (Variables|Default|GetCombatSystem))))
    (for _array_element _keys
      (LocalVariables|SetTeamIndex _array_element)
      (bind _output_get (LocalVariables|SetUnitsInTeam (Utilities|Struct|BreakS_UnitArray (.Value (Utilities|Map|Find (Variables|/Game/TacticalCards/Blueprints/Core/Combat/BP_CombatSystem.BP_CombatSystem_C|GetUnitTeams (Variables|Default|GetCombatSystem)) (LocalVariables|GetTeamIndex))))))
      (for _array_element_2 _output_get
        (bind _output_get_2 (LocalVariables|SetUnit _array_element_2))
        (Default|RemoveUnitfromCombat (Variables|Default|GetCombatSystem) _output_get_2)
        (if (Math|Boolean|ORBoolean (== (LocalVariables|GetTeamIndex) 0) (== (LocalVariables|GetTeamIndex) _teamindexthatwonlastcombat) (== _teamindexthatwonlastcombat -1))
          (Default|ResetHP (LocalVariables|GetUnit))
          (else
            (Actor|DestroyActor (LocalVariables|GetUnit))))))
    (bind _keys_2 (Utilities|Map|Keys (Variables|Default|GetUnitPositionsWhenCombatStarted)))
    (for _array_element_3 _keys_2
      (bind _output_get_3 (LocalVariables|SetUnit _array_element_3))
      (Utilities|IsValid _output_get_3
        (:Is%20Valid
          (Transformation|SetActorLocation (LocalVariables|GetUnit) (.Value (Utilities|Map|Find (Variables|Default|GetUnitPositionsWhenCombatStarted) (LocalVariables|GetUnit))) false false)
          (Default|EnableUnit (LocalVariables|GetUnit) "NewEnumerator1"))))
    (Utilities|Map|Clear (Variables|Default|GetUnitPositionsWhenCombatStarted))
    (bind _values (Utilities|Map|Values (Variables|Default|GetUnitGroups)))
    (for _array_element_4 _values
      (if (.IsEncounter (Utilities|Struct|BreakS_OverworldUnitGroup _array_element_4))
        (Default|EventMoveUnitinOverworld (Utilities|Array|Get(acopy) (.Units (Utilities|Struct|BreakS_OverworldUnitGroup _array_element_4))) "0, 0, 0" 0 true)))
    (Default|DestroyGrid (Variables|/Game/TacticalCards/Blueprints/Core/Combat/BP_CombatSystem.BP_CombatSystem_C|GetGrid (Variables|Default|GetCombatSystem)))))