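; Ranger variant of the unit AI in a tactical card game, choosing its movement logic from turn parity and whether it has dealt damage.
; It counts turns per combat and flags any cast ability with a negative minimum HP modifier as damage for that turn.
; One movement mode applies on even turns without damage, another otherwise, with parent logic handling the rest.
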(event EventBeginPlay
  (|CallParentFunction) ; This node is disabled and will not be called.\nDrag off pins to build functionality.
)

(event Collision|EventActorBeginOverlap
  (params (OtherActor :type Actor%20Object%20Reference)))

(event EventTick
  (params (DeltaSeconds :type Float%20%28single-precision%29)))

(event EventCastAbility
  (bind _abilitydata (CallFunction|GetAbilityDatafromAbility (Utilities|Struct|BreakS_UnitAIAbilityCastingData (Variables|Default|GetAIAbilityCasting))))
  (Variables|Default|SetDamagedAnUnitThisTurn (or (< (Utilities|Struct|BreakIntPoint (Utilities|Struct|BreakS_AbilityData_Impact (Utilities|Struct|BreakS_AbilityData _abilitydata))) 0) (Variables|Default|GetDamagedAnUnitThisTurn)))
  (|CallParentFunction))

(fn ConstructionScript
  (|CallParentFunction))

(fn AIPlayTurn
  (Math|Integer|IncrementInt (Variables|Default|GetTurnCount)
    (:%20%20
      (Variables|Default|SetDamagedAnUnitThisTurn false)
      (|CallParentFunction))))

(fn GetUnitMovementLogic
  (return (select (and (CallFunction|IsIntegerEven (Variables|Default|GetTurnCount)) (not (Variables|Default|GetDamagedAnUnitThisTurn))) "NewEnumerator0" "NewEnumerator2")))

(fn AICombatStarted
  (Variables|Default|SetTurnCount 0)
  (|CallParentFunction))

(fn AICombatEnded
  (Variables|Default|SetTurnCount 0)
  (|CallParentFunction))