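; Chicken unit AI for turn-based tactical combat, extending a parent unit AI through overrides.
; It holds one ability out of the normal pool and self-casts it as a fallback when no valid ability was chosen and the unit can cast it.
; Movement logic switches to an alternate mode on even turns without a damaging cast, using a per-combat turn counter and a flag set by negative HP impact.
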(event EventBeginPlay
  (|CallParentFunction) ; This node is disabled and will not be called.\nDrag off pins to build functionality.
)

(event Collision|EventActorBeginOverlap
  (params (OtherActor :type Actor%20Object%20Reference)))

(event EventTick
  (params (DeltaSeconds :type Float%20%28single-precision%29)))

(event EventCastAbility
  (bind _abilitydata (CallFunction|GetAbilityDatafromAbility (Utilities|Struct|BreakS_UnitAIAbilityCastingData (Variables|Default|GetAIAbilityCasting))))
  (Variables|Default|SetDamagedAnUnitThisTurn (or (< (Utilities|Struct|BreakIntPoint (Utilities|Struct|BreakS_AbilityData_Impact (Utilities|Struct|BreakS_AbilityData _abilitydata))) 0) (Variables|Default|GetDamagedAnUnitThisTurn)))
  (|CallParentFunction))

(event EventDecideWhichAbilitytoCastDone
  (bind _unit (Variables|Default|GetUnit))
  (bind _index (Variables|/Game/TacticalCards/Blueprints/Core/Units/BP_Unit.BP_Unit_C|GetIndex _unit))
  (Utilities|FlowControl|Sequence
    (:then_0
      (if (not (Utilities|Struct|BreakS_UnitAIAbilityCastingData (Variables|Default|GetAIAbilityCasting)))
        (bind _abilitydata (CallFunction|GetAbilityDatafromAbility "NewEnumerator10"))
        (bind _cancast (Default|CanCastAbility _unit _abilitydata))
        (if _cancast
          (Variables|Default|SetAIAbilityCasting (Utilities|Struct|MakeS_UnitAIAbilityCastingData true "NewEnumerator10" _index _index)))))
    (:then_1
      (|CallParentFunction))))

(fn ConstructionScript
  (|CallParentFunction))

(fn AIPlayTurn
  (Math|Integer|IncrementInt (Variables|Default|GetTurnCount)
    (:%20%20
      (Variables|Default|SetDamagedAnUnitThisTurn false)
      (|CallParentFunction))))

(fn GetUnitMovementLogic
  (return (select (and (CallFunction|IsIntegerEven (Variables|Default|GetTurnCount)) (not (Variables|Default|GetDamagedAnUnitThisTurn))) "NewEnumerator0" "NewEnumerator2")))

(fn AICombatStarted
  (Variables|Default|SetTurnCount 0)
  (|CallParentFunction))

(fn AICombatEnded
  (Variables|Default|SetTurnCount 0)
  (|CallParentFunction))

(fn GetAvailableAbilities
  (bind _output_get (LocalVariables|SetRet (|CallParentFunction)))
  (Utilities|Array|RemoveItem _output_get "NewEnumerator10")
  (return (LocalVariables|GetRet)))